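; Edible object actor that spawns with random HP, which also sets its mesh scale, and is destroyed when HP runs out.
; Tick switches custom-channel and camera collision between blocking and passable based on Canoverlap.
; While overlapped, a looping timer drains its HP, sends negative damage to the other actor and pulls the gravity-free mesh toward it.
; Incoming damage also lowers HP, and ending overlap stops the drain and restores gravity.
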(event Custom|damagetarget
  ;[1 1 1] OverlapEvents
  (Utilities|FlowControl|Sequence
    (:then_0
      (bind _output_get (Variables|Default|SetHP (- (Variables|Default|GetHP) 1)))
      (if (<= _output_get 0)
        (Actor|DestroyActor)))
    (:then_1
      (Game|Damage|ApplyDamage (stale Collision|EventActorBeginOverlap OtherActor) -1.0 0 0))
    (:then_2
      (Components|MoveComponentTo (Variables|Default|GetStaticMesh) (Math|Interpolation|VInterpTo (Transformation|GetActorLocation) (Transformation|GetActorLocation (stale Collision|EventActorBeginOverlap OtherActor)) 1.0 1.0) "0, 0, 0" false false 0.2 false))))

(event EventBeginPlay
  ;[1 1 1] Event Beginplay
  (bind _output_get (Variables|Default|SetHP (Math|Random|RandomIntegerinRange 10 30)))
  (Transformation|SetWorldScale3D (Variables|Default|GetStaticMesh) (Math|Conversions|ToVector(Float) (/ (Math|Conversions|ToFloat(Integer) _output_get) 3e+01))))

(event Collision|EventActorEndOverlap
  (params (OtherActor :type Actor%20Object%20Reference))
  ;[1 1 1] OverlapEvents
  (Utilities|Time|ClearandInvalidateTimerbyHandle (stale Collision|EventActorBeginOverlap _returnvalue))
  (Utilities|FlowControl|Sequence
    (:then_0
      (Components|MoveComponentTo (Variables|Default|GetStaticMesh) (Math|Interpolation|VInterpTo (Transformation|GetActorLocation) (Transformation|GetActorLocation (stale Collision|EventActorBeginOverlap OtherActor)) 1.0 1.0) "0, 0, 0" false false 0.2 false) ; enters at Stop
    )
    (:then_1
      (Physics|SetEnableGravity (Variables|Default|GetStaticMesh) true))))

(event Game|Damage|EventAnyDamage
  (params (Damage :type Float%20%28single-precision%29) (DamageType :type Damage%20Type%20Object%20Reference) (InstigatedBy :type Controller%20Object%20Reference) (DamageCauser :type Actor%20Object%20Reference))
  ;[1 1 1] Damage Event
  (bind _output_get (Variables|Default|SetHP (- (Variables|Default|GetHP) (Math|Float|Truncate Damage))))
  (Development|PrintString (Utilities|String|ToString(Integer) _output_get))
  (if (<= _output_get 0)
    (Utilities|FlowControl|Sequence
      (:then_0
        (Actor|DestroyActor))
      (:then_1
        (Development|PrintString "dead")))))

(event Collision|EventActorBeginOverlap
  (params (OtherActor :type Actor%20Object%20Reference))
  ;[1 1 1] OverlapEvents
  (bind _returnvalue (Utilities|Time|SetTimerbyEvent (delegate Custom|damagetarget) 0.3 true))
  (Physics|SetEnableGravity (Variables|Default|GetStaticMesh) false))

(event EventTick
  (params (DeltaSeconds :type Float%20%28single-precision%29))
  ;[1 1 1] Everytick Events
  (if (Variables|Default|Getcanoverlap)
    (Collision|SetCollisionResponsetoChannel (Variables|Default|GetStaticMesh) "ECC_GameTraceChannel1" "ECR_Overlap")
    (Collision|SetCollisionResponsetoChannel (Variables|Default|GetStaticMesh) "ECC_Camera" "ECR_Ignore")
    (else
      (Collision|SetCollisionResponsetoChannel (Variables|Default|GetStaticMesh) "ECC_GameTraceChannel1" "ECR_Block")
      (Collision|SetCollisionResponsetoChannel (Variables|Default|GetStaticMesh) "ECC_Camera" "ECR_Block"))))

(fn ConstructionScript)