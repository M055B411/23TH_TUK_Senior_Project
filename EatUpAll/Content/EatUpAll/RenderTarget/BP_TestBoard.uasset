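; Test paint board Blueprint that stamps marks into the CRT_PaintBoard render target at supplied 2D locations.
; On BeginPlay it creates a dynamic instance of M_PaintboardMaker and clears the target to black.
; DrawOnShuttle sets the material's DrawLocation, draws it to the target and prints a debug message.
; DrawSize sets the brush material's Size parameter for subsequent draws.
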(event Custom|DrawOnShuttle
  (params (LocationToDraw :type Vector%202D%20Structure))
  (bind _paintboardmarker (Variables|Default|GetPaintboardMarker))
  (Rendering|Material|SetVectorParameterValue _paintboardmarker "DrawLocation" (Math|Conversions|ToLinearColor(Vector) (Math|Conversions|ToVector(Vector2D) LocationToDraw 0.1)) :!class /Script/Engine.MaterialInstanceDynamic)
  (Rendering|DrawMaterialtoRenderTarget "/Game/EatUpAll/RenderTarget/CRT_PaintBoard.CRT_PaintBoard" _paintboardmarker)
  (Development|PrintString "painting"))

(event Custom|DrawSize
  (params (Draw%20size :type Float%20%28double-precision%29))
  (Rendering|Material|SetScalarParameterValue (Variables|Default|GetPaintboardMarker) "Size" Draw%20size :!class /Script/Engine.MaterialInstanceDynamic))

(event EventBeginPlay
  (bind _returnvalue (Rendering|Material|CreateDynamicMaterialInstance "/Game/EatUpAll/RenderTarget/M_PaintboardMaker.M_PaintboardMaker" "None" "None" :!class /Script/Engine.KismetMaterialLibrary))
  (Variables|Default|SetPaintboardMarker _returnvalue)
  (Rendering|ClearRenderTarget2D "/Game/EatUpAll/RenderTarget/CRT_PaintBoard.CRT_PaintBoard"))

(fn ConstructionScript)