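; BP_HeatMap is an actor that paints the player's path as heat splats into a render target.
; Each tick it traces vertically from player 0 to its mesh's height and, on a blocking hit against itself, converts the point to local UV space.
; It draws M_HeatSplat there through a dynamic material instance.
; The MPC_Heat parameter collection receives the capture size at BeginPlay and the actor location after each draw.
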(event Custom|DrawToRenderTarget
  (params (Location :type Vector) (Strength :type Float%20%28double-precision%29) (Size :type Float%20%28double-precision%29))
  (bind _mid_heatsplat (Variables|Default|GetMID_Heatsplat))
  (bind _staticmesh (Variables|Default|GetStaticMesh))
  (bind _resolution (Variables|Default|GetResolution))
  (bind _returnvalue (Transformation|GetWorldTransform _staticmesh))
  (bind _returnvalue_2 (Math|Transform|InvertTransform _returnvalue))
  (bind _returnvalue_3 (Math|Transform|TransformLocation _returnvalue_2 Location))
  (bind _returnvalue_4 (/ _returnvalue_3 _resolution))
  (bind (_x _y _z) (Math|Vector|BreakVector _returnvalue_4))
  (bind _returnvalue_5 (/ _x 2.0))
  (bind _returnvalue_6 (/ _y 2.0))
  (bind _returnvalue_7 (* _returnvalue_5 -1.0))
  (bind _returnvalue_8 (+ _returnvalue_6 0.5))
  (bind _returnvalue_9 (+ _returnvalue_7 0.5))
  (bind _returnvalue_10 (Math|Vector|MakeVector _returnvalue_8 _returnvalue_9 _z))
  (Rendering|Material|SetScalarParameterValue _mid_heatsplat "Strength" Strength :!class /Script/Engine.MaterialInstanceDynamic)
  (Rendering|Material|SetScalarParameterValue _mid_heatsplat "Size" Size :!class /Script/Engine.MaterialInstanceDynamic)
  (Rendering|Material|SetVectorParameterValue _mid_heatsplat "Position" (Math|Conversions|ToLinearColor(Vector) _returnvalue_10) :!class /Script/Engine.MaterialInstanceDynamic)
  (Rendering|DrawMaterialtoRenderTarget (Variables|Default|GetRenderTargetRuntime) _mid_heatsplat)
  (CallFunction|CaptureLocation)
  (Development|PrintString (Utilities|String|ToString(Vector) _returnvalue_10)))

(event EventTick
  (params (DeltaSeconds :type Float%20%28single-precision%29))
  (bind _playerref (Variables|Default|GetPlayerRef))
  (bind _returnvalue (Transformation|GetActorLocation _playerref))
  (bind (_x _y) (Math|Vector|BreakVector _returnvalue))
  (Utilities|IsValid _playerref
    (:Is%20Valid
      (bind _outhits (Class|KismetSystemLibrary|LineTraceMultiforObjects _returnvalue (Math|Vector|MakeVector _x _y (* (.z (Transformation|GetWorldLocation (Variables|Default|GetStaticMesh))) 1.0)) (Utilities|Array|MakeArray "ObjectTypeQuery1" "ObjectTypeQuery2") false 0 "ForOneFrame" false))
      (for _array_element _outhits
        (if (and (.bBlockingHit (Collision|BreakHitResult _array_element)) (== (.HitActor (Collision|BreakHitResult _array_element)) self))
          (CallFunction|DrawtoRenderTarget (.Location (Collision|BreakHitResult _array_element)) 1.0 0.06))))))

(event EventBeginPlay
  ;[1 1 1] you need every player search in multiplay
  (Variables|Default|SetPlayerRef (Game|GetPlayerCharacter 0))
  (Rendering|Material|SetScalarParameterValue "/Game/EatUpAll/SceneCapture/PaintTest2/MPC_Heat.MPC_Heat" "CaptureSize" (Variables|Default|GetResolution) :!class /Script/Engine.KismetMaterialLibrary)
  (Rendering|ClearRenderTarget2D (Variables|Default|GetRenderTargetRuntime)))

(fn ConstructionScript
  (bind _returnvalue (Rendering|Material|CreateDynamicMaterialInstance "/Game/EatUpAll/SceneCapture/PaintTest2/M_HeatSplat.M_HeatSplat" "None" "None" :!class /Script/Engine.KismetMaterialLibrary))
  (Variables|Default|SetMID_Heatsplat _returnvalue))

(fn CaptureLocation
  (Rendering|Material|SetVectorParameterValue "/Game/EatUpAll/SceneCapture/PaintTest2/MPC_Heat.MPC_Heat" "CaptureLocation" (Math|Conversions|ToLinearColor(Vector) (Transformation|GetActorLocation)) :!class /Script/Engine.KismetMaterialLibrary))