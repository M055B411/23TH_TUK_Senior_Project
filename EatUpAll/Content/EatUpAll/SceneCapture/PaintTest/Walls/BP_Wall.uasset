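; BP_Wall is a wall actor that shows a render target texture on its Plane mesh, part of a scene capture paint test.
; On BeginPlay it creates a dynamic material instance for each of the plane's material slots and stores them in an array.
; SetValues then passes the RT variable into the "RT" texture parameter of every stored instance.
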(event Custom|SetValues
  (for _array_element (Variables|Default|GetDynamicMaterials)
    (Rendering|Material|SetTextureParameterValue _array_element "RT" (Variables|Default|GetRT))))

(event EventBeginPlay
  (bind _plane (Variables|Default|GetPlane))
  (for (_array_element _array_index) (Rendering|Material|GetMaterials _plane)
    (bind _returnvalue (Rendering|Material|CreateDynamicMaterialInstance _plane _array_index _array_element "None" :!class /Script/Engine.PrimitiveComponent))
    (Utilities|Array|SetArrayElem (Variables|Default|GetDynamicMaterials) _array_index _returnvalue true))
  (CallFunction|SetValues))

(fn ConstructionScript)