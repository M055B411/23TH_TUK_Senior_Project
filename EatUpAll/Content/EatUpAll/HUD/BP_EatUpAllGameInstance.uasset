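; Game instance for EatUpAll that handles character selection and shows the selection and countdown widgets.
; Select events spawn Hunter 1, Hunter 2 or Slime at their spawn transforms and possess them with player controller 0.
; Only Hunter 1 routes through Server and Multi-named events and equips a vacuum gun if missing.
; The selection screen enables the cursor and UI-only input, while DestroyTravelTimer is an empty stub.
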(event Custom|View%20TravelTimer
  (bind _returnvalue (UserInterface|CreateWidget "/Game/EatUpAll/HUD/WBP_CountTimer.WBP_CountTimer_C"))
  (UserInterface|Viewport|AddtoViewport _returnvalue 0))

(event Custom|SlimeSelect
  (bind _returnvalue (Game|SpawnActorfromClass "/Game/EatUpAll/Blueprints/Slime/BP_SlimeCharacter_Child.BP_SlimeCharacter_Child_C" (Variables|Default|GetSlime%20Spawn%20Transform) "Undefined" "MultiplyWithRoot" 0 0))
  (Pawn|Possess (Game|GetPlayerController 0) _returnvalue))

(event Custom|Hunter2%20Select
  (bind _returnvalue (Game|SpawnActorfromClass "/Game/EatUpAll/Blueprints/Player/BP_HunterPlayer.BP_HunterPlayer_C" (Variables|Default|GetHunter2%20Spawn%20Transform) "Undefined" "MultiplyWithRoot" 0 0))
  (Pawn|Possess (Game|GetPlayerController 0) _returnvalue))

(event Custom|Hunter1Select%20Multi
  (bind _returnvalue (Game|GetPlayerCharacter 0))
  (bind _returnvalue_2 (Game|SpawnActorfromClass "/Game/EatUpAll/Blueprints/Player/BP_HunterPlayer.BP_HunterPlayer_C" (Variables|Default|GetHunter1%20Spawn%20Transform) "Undefined" "MultiplyWithRoot" 0 0))
  (Pawn|Possess (Game|GetPlayerController 0) _returnvalue_2)
  (Development|PrintString (Utilities|GetDisplayName _returnvalue))
  (bind _asbp_hunter_player (Utilities|Casting|CastToBP_HunterPlayer _returnvalue))
  (Utilities|IsValid (Variables|/Script/EatUpAll.VacuumPlayer|GetVacuumGun _asbp_hunter_player)
    (:Is%20Not%20Valid
      (Class|VacuumPlayer|EquipVacuumGun _asbp_hunter_player))))

(event Custom|Hunter1%20Select%20Server
  (CallFunction|Hunter1SelectMulti))

(event Custom|View%20SelectCharacter
  (bind _returnvalue (Game|GetPlayerController 0))
  (bind _returnvalue_2 (UserInterface|CreateWidget "/Game/EatUpAll/HUD/WBP_SelectCharacter.WBP_SelectCharacter_C"))
  (UserInterface|Viewport|AddtoViewport _returnvalue_2 0)
  (Variables|/Script/Engine.PlayerController|SetbShowMouseCursor _returnvalue true)
  (Input|SetInputModeUIOnly _returnvalue 0 "DoNotLock" false))

(event Custom|Destroy%20TravelTimer)