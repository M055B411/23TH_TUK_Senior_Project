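; Actor that tracks whether each of the three playable characters, Hunter 1, Hunter 2 and Slime, has been selected.
; Per-character server-named events call client-named counterparts that set the matching selected flag.
; Each Set Spawned function returns its flag if already true, otherwise derives it from IsSpawned on the first actor found of that character's class, defaulting to false when none exists.
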(event Custom|Set%20Hunter1%20Selected%20on%20Server
  (CallFunction|SetHunter1SelectedonClient))

(event Custom|Set%20Hunter1%20Selected%20on%20Client
  (Variables|Default|SetbIsHunter1Selected true))

(event Custom|Set%20Slime%20Selected%20on%20Client
  (Variables|Default|SetbIsSlimeSelected true))

(event Custom|Set%20Slime%20Selected%20on%20Server
  (CallFunction|SetSlimeSelectedonClient))

(event Custom|Set%20Hunter2%20Selected%20on%20Server
  (CallFunction|SetHunter2SelectedonClient))

(event Custom|Set%20Hunter2%20Selected%20on%20Client
  (Variables|Default|SetbIsHunter2Selected true))

(event EventBeginPlay)

(event Collision|EventActorBeginOverlap
  (params (OtherActor :type Actor%20Object%20Reference)))

(event EventTick
  (params (DeltaSeconds :type Float%20%28single-precision%29)))

(fn ConstructionScript)

(fn SetHunter1Spawned
  (if (Variables|Default|GetbIsHunter1Selected)
    _
    (else
      (bind _outactors (Actor|GetAllActorsOfClass "/Game/EatUpAll/Blueprints/Player/BP_HunterPlayer.BP_HunterPlayer_C"))
      (if (Utilities|Array|IsValidIndex _outactors)
        (if (Variables|/Game/EatUpAll/Blueprints/Player/BP_VacuumPlayer.BP_VacuumPlayer_C|GetbIsSpawned (Utilities|Array|Get(acopy) _outactors))
          (bind _output_get (Variables|Default|SetbIsHunter1Selected true))
          (else
            (bind _output_get_2 (Variables|Default|SetbIsHunter1Selected false :!label _label))
            (return _output_get_2)))
        (else
          (goto _label)))))
  (return _output_get))

(fn SetHunter2Spawned
  (if (Variables|Default|GetbIsHunter2Selected)
    _
    (else
      (bind _outactors (Actor|GetAllActorsOfClass "/Game/EatUpAll/Blueprints/Player/BP_Hunter2Player.BP_Hunter2Player_C"))
      (if (Utilities|Array|IsValidIndex _outactors)
        (if (Variables|/Game/EatUpAll/Blueprints/Player/BP_VacuumPlayer.BP_VacuumPlayer_C|GetbIsSpawned (Utilities|Array|Get(acopy) _outactors))
          (bind _output_get (Variables|Default|SetbIsHunter2Selected true))
          (else
            (bind _output_get_2 (Variables|Default|SetbIsHunter2Selected false :!label _label))
            (return _output_get_2)))
        (else
          (goto _label)))))
  (return _output_get))

(fn SetSlimeSpawned
  (if (Variables|Default|GetbIsSlimeSelected)
    _
    (else
      (bind _outactors (Actor|GetAllActorsOfClass "/Game/EatUpAll/Blueprints/Slime/BP_SlimeCharForNewMove_Done.BP_SlimeCharForNewMove_Done_C"))
      (if (Utilities|Array|IsValidIndex _outactors)
        (if (Variables|/Game/EatUpAll/Blueprints/Slime/BP_SlimeCharForNewMove_Done.BP_SlimeCharForNewMove_Done_C|GetbIsSpawned (Utilities|Array|Get(acopy) _outactors))
          (bind _output_get (Variables|Default|SetbIsSlimeSelected true))
          (else
            (bind _output_get_2 (Variables|Default|SetbIsSlimeSelected false :!label _label))
            (return _output_get_2)))
        (else
          (goto _label)))))
  (return _output_get))