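; Player controller for EatUpAll that handles character selection (Hunter 1, Hunter 2 or Slime), spawning and match phase hand-off.
; BeginPlay shows select and ready-count widgets; server-named spawn events replace and possess the pawn, while client-named events add the play HUD.
; Each spawn updates the GameInstance player count, and a count of three makes the GameMode start the ready phase.
; Phase events relay state changes; Tab reopens selection, and 0 is a debug Phase 2 trigger.
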(event Custom|Slime%20Spawn%20on%20Server
  (bind _returnvalue (Game|GetGameInstance))
  (bind _asbp_eat_up_all_game_instance (Utilities|Casting|CastToBP_EatUpAllGameInstance _returnvalue))
  ;[1 1 1] Slime Spawn on Map
  ; When Slime Character Select in Select Widget
  (Utilities|IsValid (Variables|Default|GetCurrent%20Chracter)
    (:Is%20Valid
      (Actor|DestroyActor (Variables|Default|GetCurrent%20Chracter)))
    (:Is%20Not%20Valid
      _))
  (Utilities|FlowControl|Delay 0.2)
  (bind _returnvalue_2 (Game|SpawnActorfromClass "/Game/EatUpAll/Blueprints/Slime/BP_SlimeCharForNewMove_Done.BP_SlimeCharForNewMove_Done_C" (Variables|Default|GetSlime%20Spawn%20ini%20Transform) "AdjustIfPossibleButAlwaysSpawn" "MultiplyWithRoot" 0 0))
  (Variables|Default|SetCurrent%20Chracter _returnvalue_2)
  (CallFunction|SlimeSpawnonClient)
  (Pawn|Possess _returnvalue_2)
  (Default|SelectedPCcount _asbp_eat_up_all_game_instance)
  (if (== (Variables|/Game/EatUpAll/HUD/BP_EatUpAllGameInstance.BP_EatUpAllGameInstance_C|GetInt_PCcount _asbp_eat_up_all_game_instance) 3)
    (bind _asbp_eat_up_all_game_mode (Utilities|Casting|CastToBP_EatUpAll_GameMode (Game|GetGameMode)))
    (Default|StartPhaseReady _asbp_eat_up_all_game_mode)))

(event Custom|Start%20GameResult
  (Default|CallEventGameResult))

(event Custom|Start%20PhaseReady
  (Variables|Default|SetbIsPhaseReady true)
  (Default|CallEvnetPhaseReady))

(event Custom|Slime%20Spawn%20on%20Client
  ;[1 1 1] Slime Spawn on Map
  ; When Slime Character Select in Select Widget
  (if (Pawn|IsLocalPlayerController)
    (bind _returnvalue (UserInterface|CreateWidget "/Game/EatUpAll/HUD/WBP_PlayCommon.WBP_PlayCommon_C"))
    (bind _output_get (Variables|Default|SetWBP_PlayCommon _returnvalue))
    (UserInterface|Viewport|AddtoPlayerScreen _output_get)
    (Variables|/Game/EatUpAll/HUD/WBP_PlayCommon.WBP_PlayCommon_C|SetbIsSlime (Variables|Default|GetWBP_PlayCommon) true)))

(event Custom|Hunter1%20Spawn%20on%20Server
  (bind _returnvalue (Game|GetGameInstance))
  (bind _asbp_eat_up_all_game_instance (Utilities|Casting|CastToBP_EatUpAllGameInstance _returnvalue))
  ;[1 1 1] Hunter1 Spawn on Map
  ; When Hunter1 Character Select in Select Widget
  (Utilities|IsValid (Variables|Default|GetCurrent%20Chracter)
    (:Is%20Valid
      (Actor|DestroyActor (Variables|Default|GetCurrent%20Chracter)))
    (:Is%20Not%20Valid
      _))
  (Utilities|FlowControl|Delay 0.2)
  (bind _returnvalue_2 (Game|SpawnActorfromClass "/Game/EatUpAll/Blueprints/Player/BP_HunterPlayer.BP_HunterPlayer_C" (Variables|Default|GetHunter1%20Spawn%20ini%20Transform) "AdjustIfPossibleButAlwaysSpawn" "MultiplyWithRoot" 0 0))
  (Variables|Default|SetCurrent%20Chracter _returnvalue_2)
  (CallFunction|HunterSpawnonClient)
  (Pawn|Possess _returnvalue_2)
  (Default|SelectedPCcount _asbp_eat_up_all_game_instance)
  (if (== (Variables|/Game/EatUpAll/HUD/BP_EatUpAllGameInstance.BP_EatUpAllGameInstance_C|GetInt_PCcount _asbp_eat_up_all_game_instance) 3)
    (bind _asbp_eat_up_all_game_mode (Utilities|Casting|CastToBP_EatUpAll_GameMode (Game|GetGameMode)))
    (Default|StartPhaseReady _asbp_eat_up_all_game_mode)))

(event Custom|IntPCcount%20initalize
  (bind _result (Math|Integer|DecrementInt (Variables|/Game/EatUpAll/HUD/BP_EatUpAllGameInstance.BP_EatUpAllGameInstance_C|GetInt_PCcount (.AsBP%20Eat%20Up%20All%20Game%20Instance (Utilities|Casting|CastToBP_EatUpAllGameInstance (Game|GetGameInstance)))))
    (:%20%20
      (Variables|Default|SetInt_PCcount _result))))

(event Custom|Hunter%20Spawn%20on%20Client
  ;[1 1 1] Hunter1 Spawn on Map
  ; When Hunter1 Character Select in Select Widget
  (if (Pawn|IsLocalPlayerController)
    (bind _returnvalue (UserInterface|CreateWidget "/Game/EatUpAll/HUD/WBP_PlayCommon.WBP_PlayCommon_C"))
    (bind _output_get (Variables|Default|SetWBP_PlayCommon _returnvalue))
    (UserInterface|Viewport|AddtoPlayerScreen _output_get)))

(event Custom|Start%20PhasePlay2
  (Variables|Default|SetbIsPhasePlay2 true)
  (Default|CallEventPhase2))

(event Custom|Start%20PhasePlay1
  (bind _wbp_ready (Variables|Default|GetWBP_Ready))
  (Variables|Default|SetbIsPhasePlay1 true)
  (Utilities|IsValid _wbp_ready
    (:Is%20Valid
      (Widget|RemovefromParent _wbp_ready)
      (Default|CallEventPhase1))))

(event Custom|Hunter2%20Spawn%20on%20Server
  (bind _returnvalue (Game|GetGameInstance))
  (bind _asbp_eat_up_all_game_instance (Utilities|Casting|CastToBP_EatUpAllGameInstance _returnvalue))
  ;[1 1 1] Hunter2 Spawn on Map
  ; When Hunter2 Character Select in Select Widget
  (Utilities|IsValid (Variables|Default|GetCurrent%20Chracter)
    (:Is%20Valid
      (Actor|DestroyActor (Variables|Default|GetCurrent%20Chracter)))
    (:Is%20Not%20Valid
      _))
  (Utilities|FlowControl|Delay 0.2)
  (bind _returnvalue_2 (Game|SpawnActorfromClass "/Game/EatUpAll/Blueprints/Player/BP_Hunter2Player.BP_Hunter2Player_C" (Variables|Default|GetHunter2%20Spawn%20ini%20Transform) "AdjustIfPossibleButAlwaysSpawn" "MultiplyWithRoot" 0 0))
  (Variables|Default|SetCurrent%20Chracter _returnvalue_2)
  (CallFunction|HunterSpawnonClient)
  (Pawn|Possess _returnvalue_2)
  (Default|SelectedPCcount _asbp_eat_up_all_game_instance)
  (if (== (Variables|/Game/EatUpAll/HUD/BP_EatUpAllGameInstance.BP_EatUpAllGameInstance_C|GetInt_PCcount _asbp_eat_up_all_game_instance) 3)
    (bind _asbp_eat_up_all_game_mode (Utilities|Casting|CastToBP_EatUpAll_GameMode (Game|GetGameMode)))
    (Default|StartPhaseReady _asbp_eat_up_all_game_mode)))

(event EventBeginPlay
  (bind _returnvalue (Game|GetPlayerController 0))
  (Utilities|FlowControl|Delay 1.0)
  (if (Pawn|IsLocalPlayerController)
    (bind _returnvalue_2 (UserInterface|CreateWidget "/Game/EatUpAll/HUD/WBP_SelectCharacter.WBP_SelectCharacter_C"))
    (UserInterface|Viewport|AddtoViewport _returnvalue_2 0)
    (Variables|/Script/Engine.PlayerController|SetbShowMouseCursor _returnvalue true)
    (Input|SetInputModeUIOnly _returnvalue 0 "DoNotLock" false)
    (bind _returnvalue_3 (UserInterface|CreateWidget "/Game/EatUpAll/HUD/WBP_ReadyCount.WBP_ReadyCount_C"))
    (bind _output_get (Variables|Default|SetWBP_Ready _returnvalue_3))
    (UserInterface|Viewport|AddtoPlayerScreen _output_get)))

(event Input|KeyboardEvents|Tab
  (params (Key :type Key%20Structure))
  (bind _returnvalue (Game|GetPlayerController 0))
  (:Pressed
    (CallFunction|IntPCcountInitalize)
    (if (Pawn|IsLocalPlayerController)
      (bind _returnvalue_2 (UserInterface|CreateWidget "/Game/EatUpAll/HUD/WBP_SelectCharacter.WBP_SelectCharacter_C"))
      (UserInterface|Viewport|AddtoViewport _returnvalue_2 0)
      (Variables|/Script/Engine.PlayerController|SetbShowMouseCursor _returnvalue true)
      (Input|SetInputModeUIOnly _returnvalue 0 "DoNotLock" false)
      (bind _returnvalue_3 (UserInterface|CreateWidget "/Game/EatUpAll/HUD/WBP_ReadyCount.WBP_ReadyCount_C"))
      (bind _output_get (Variables|Default|SetWBP_Ready _returnvalue_3))
      (UserInterface|Viewport|AddtoPlayerScreen _output_get))))

(event Input|KeyboardEvents|0
  (params (Key :type Key%20Structure))
  (bind _returnvalue (Game|GetGameMode))
  (:Pressed
    (Utilities|IsValid _returnvalue
      (:Is%20Valid
        (Development|PrintString "Hello")
        (bind _asbp_eat_up_all_game_mode (Utilities|Casting|CastToBP_EatUpAll_GameMode _returnvalue))
        (Default|StartPhase2 _asbp_eat_up_all_game_mode)))))

(fn ConstructionScript)