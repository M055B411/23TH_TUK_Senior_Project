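; Player controller that handles character selection, spawning and match phase relays for a Hunters-versus-Slime game.
; BeginPlay opens the selection widget for the local player.
; Server spawn events replace the current pawn with Hunter1, Hunter2 or Slime, possess it and trigger client HUD creation, flagging Slime.
; Each spawn updates the GameInstance selection count, calling GameMode's ready phase at the player limit; other events relay phases and win/draw results.
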(event Custom|Slime%20Spawn%20on%20Server
  (bind _returnvalue (Game|GetGameInstance))
  (bind _asbp_eat_up_all_game_instance (Utilities|Casting|CastToBP_EatUpAllGameInstance _returnvalue))
  ;[1 1 1] Slime Spawn on Map
  ; When Slime Character Select in Select Widget
  (Utilities|IsValid (Variables|Default|GetCurrent%20Chracter)
    (:Is%20Valid
      (Actor|DestroyActor (Variables|Default|GetCurrent%20Chracter)))
    (:Is%20Not%20Valid
      _))
  (Utilities|FlowControl|Delay 0.2)
  (bind _returnvalue_2 (Game|SpawnActorfromClass "/Game/EatUpAll/Blueprints/Slime/BP_SlimeCharForNewMove_Single.BP_SlimeCharForNewMove_Single_C" (Variables|Default|GetSlime%20Spawn%20ini%20Transform) "AdjustIfPossibleButAlwaysSpawn" "MultiplyWithRoot" 0 0))
  (Variables|Default|SetCurrent%20Chracter _returnvalue_2)
  (CallFunction|SlimeSpawnonClient)
  (Pawn|Possess _returnvalue_2)
  (Default|SelectedPCcount _asbp_eat_up_all_game_instance)
  (if (== (Variables|/Game/EatUpAll/HUD/BP_EatUpAllGameInstance.BP_EatUpAllGameInstance_C|GetSelect%20PC%20Count _asbp_eat_up_all_game_instance) (Variables|/Game/EatUpAll/HUD/BP_EatUpAllGameInstance.BP_EatUpAllGameInstance_C|GetPlay%20PC%20Num%20Ilmit _asbp_eat_up_all_game_instance))
    (bind _asbp_eat_up_all_game_mode (Utilities|Casting|CastToBP_EatUpAll_GameMode (Game|GetGameMode)))
    (Default|CallPhaseReady _asbp_eat_up_all_game_mode)))

(event Custom|Start%20DrawResult
  (Default|CallDrawResult))

(event Custom|Start%20SlimeWinResult
  (Default|CallSlimeWinResult))

(event Custom|Start%20PhasePlay1
  (Default|CallPhase1))

(event Custom|Start%20PhasePlay2
  (Default|CallPhase2))

(event Custom|Start%20PhaseReady
  (if (Pawn|IsLocalPlayerController)
    (Default|CallPhaseReady)))

(event Custom|Slime%20Spawn%20on%20Client
  ;[1 1 1] Slime Spawn on Map
  ; When Slime Character Select in Select Widget
  (if (Pawn|IsLocalPlayerController)
    (bind _returnvalue (UserInterface|CreateWidget "/Game/EatUpAll/HUD/WBP_PlayCommon.WBP_PlayCommon_C"))
    (bind _output_get (Variables|Default|SetWBP_PlayCommon _returnvalue))
    (UserInterface|Viewport|AddtoPlayerScreen _output_get)
    (Variables|/Game/EatUpAll/HUD/WBP_PlayCommon.WBP_PlayCommon_C|SetbIsSlime (Variables|Default|GetWBP_PlayCommon) true)))

(event Custom|Hunter1%20Spawn%20on%20Server
  (bind _returnvalue (Game|GetGameInstance))
  (bind _asbp_eat_up_all_game_instance (Utilities|Casting|CastToBP_EatUpAllGameInstance _returnvalue))
  ;[1 1 1] Hunter1 Spawn on Map
  ; When Hunter1 Character Select in Select Widget
  (Utilities|IsValid (Variables|Default|GetCurrent%20Chracter)
    (:Is%20Valid
      (Actor|DestroyActor (Variables|Default|GetCurrent%20Chracter)))
    (:Is%20Not%20Valid
      _))
  (Utilities|FlowControl|Delay 0.2)
  (bind _returnvalue_2 (Game|SpawnActorfromClass "/Game/EatUpAll/Blueprints/Player/BP_HunterPlayer.BP_HunterPlayer_C" (Variables|Default|GetHunter1%20Spawn%20ini%20Transform) "AdjustIfPossibleButAlwaysSpawn" "MultiplyWithRoot" 0 0))
  (Variables|Default|SetCurrent%20Chracter _returnvalue_2)
  (CallFunction|HunterSpawnonClient)
  (Pawn|Possess _returnvalue_2)
  (Default|SelectedPCcount _asbp_eat_up_all_game_instance)
  (if (== (Variables|/Game/EatUpAll/HUD/BP_EatUpAllGameInstance.BP_EatUpAllGameInstance_C|GetSelect%20PC%20Count _asbp_eat_up_all_game_instance) (Variables|/Game/EatUpAll/HUD/BP_EatUpAllGameInstance.BP_EatUpAllGameInstance_C|GetPlay%20PC%20Num%20Ilmit _asbp_eat_up_all_game_instance))
    (bind _asbp_eat_up_all_game_mode (Utilities|Casting|CastToBP_EatUpAll_GameMode (Game|GetGameMode)))
    (Default|CallPhaseReady _asbp_eat_up_all_game_mode)))

(event Custom|Start%20HunterWinResult
  (Default|CallHunterWinResult))

(event Custom|Hunter%20Spawn%20on%20Client
  ;[1 1 1] Hunter1 Spawn on Map
  ; When Hunter1 Character Select in Select Widget
  (if (Pawn|IsLocalPlayerController)
    (bind _returnvalue (UserInterface|CreateWidget "/Game/EatUpAll/HUD/WBP_PlayCommon.WBP_PlayCommon_C"))
    (bind _output_get (Variables|Default|SetWBP_PlayCommon _returnvalue))
    (UserInterface|Viewport|AddtoPlayerScreen _output_get)))

(event Custom|Start%20PhasePlay1'5
  (Default|CallPhase1'5))

(event Custom|Start%20PhasePlay0
  (if (Pawn|IsLocalPlayerController)
    (Default|CallPhase0)))

(event Custom|Hunter2%20Spawn%20on%20Server
  (bind _returnvalue (Game|GetGameInstance))
  (bind _asbp_eat_up_all_game_instance (Utilities|Casting|CastToBP_EatUpAllGameInstance _returnvalue))
  ;[1 1 1] Hunter2 Spawn on Map
  ; When Hunter2 Character Select in Select Widget
  (Utilities|IsValid (Variables|Default|GetCurrent%20Chracter)
    (:Is%20Valid
      (Actor|DestroyActor (Variables|Default|GetCurrent%20Chracter)))
    (:Is%20Not%20Valid
      _))
  (Utilities|FlowControl|Delay 0.2)
  (bind _returnvalue_2 (Game|SpawnActorfromClass "/Game/EatUpAll/Blueprints/Player/BP_Hunter2Player.BP_Hunter2Player_C" (Variables|Default|GetHunter2%20Spawn%20ini%20Transform) "AdjustIfPossibleButAlwaysSpawn" "MultiplyWithRoot" 0 0))
  (Variables|Default|SetCurrent%20Chracter _returnvalue_2)
  (CallFunction|HunterSpawnonClient)
  (Pawn|Possess _returnvalue_2)
  (Default|SelectedPCcount _asbp_eat_up_all_game_instance)
  (if (== (Variables|/Game/EatUpAll/HUD/BP_EatUpAllGameInstance.BP_EatUpAllGameInstance_C|GetSelect%20PC%20Count _asbp_eat_up_all_game_instance) (Variables|/Game/EatUpAll/HUD/BP_EatUpAllGameInstance.BP_EatUpAllGameInstance_C|GetPlay%20PC%20Num%20Ilmit _asbp_eat_up_all_game_instance))
    (bind _asbp_eat_up_all_game_mode (Utilities|Casting|CastToBP_EatUpAll_GameMode (Game|GetGameMode)))
    (Default|CallPhaseReady _asbp_eat_up_all_game_mode)))

(event EventBeginPlay
  (bind _returnvalue (Game|GetPlayerController 0))
  (if (Pawn|IsLocalPlayerController)
    (bind _returnvalue_2 (UserInterface|CreateWidget "/Game/EatUpAll/HUD/WBP_SelectCharacter.WBP_SelectCharacter_C"))
    (UserInterface|Viewport|AddtoViewport _returnvalue_2 0)
    (Variables|/Script/Engine.PlayerController|SetbShowMouseCursor _returnvalue true)
    (Input|SetInputModeUIOnly _returnvalue 0 "DoNotLock" false)))

(event Input|KeyboardEvents|Tab
  (params (Key :type Key%20Structure :default "None")))

(fn ConstructionScript)