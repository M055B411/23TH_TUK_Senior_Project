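; Child vacuum player character that erases and paints on surfaces from the first-person camera and interacts with nearby actors.
; Left mouse enables erasing and calls SuckTriggered, while right mouse enables painting.
; Each tick, LineTraceRT multi-traces forward and messages hit actors with the collision UV for whichever mode is held.
; Entering an interact zone stores the actor and shows a prompt widget, and the Interact input messages that actor.
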(event EventEndedInteractZone
  (params (InteractableActor :type Actor%20Object%20Reference))
  (if (== InteractableActor (Variables|Default|GetInteractableActor))
    (Variables|Default|SetInteractableActor 0)
    (Utilities|IsValid (Variables|Default|GetInteractWidget)
      (:Is%20Valid
        (Widget|RemovefromParent (Variables|Default|GetInteractWidget))))))

(event EventEnterInteractZone
  (params (InteractableActor :type Actor%20Object%20Reference))
  (Variables|Default|SetInteractableActor InteractableActor)
  (bind _returnvalue (UserInterface|CreateWidget "/Game/Example01/Widgets/UMG_Interact.UMG_Interact_C" (Game|GetPlayerController 0)))
  (bind _output_get (Variables|Default|SetInteractWidget _returnvalue))
  (UserInterface|Viewport|AddtoViewport _output_get 0))

(event EventTick
  (params (DeltaSeconds :type Float%20%28single-precision%29))
  (CallFunction|LineTraceRT))

(event EventBeginPlay
  (|CallParentFunction) ; This node is disabled and will not be called.\nDrag off pins to build functionality.
)

(event Collision|EventActorBeginOverlap
  (params (OtherActor :type Actor%20Object%20Reference))
  (|CallParentFunction OtherActor) ; This node is disabled and will not be called.\nDrag off pins to build functionality.
)

(event Input|ActionEvents|InputActionInteract
  (params (Key :type Key%20Structure :default "None"))
  (:Pressed
    (Utilities|IsValid (Variables|Default|GetInteractableActor)
      (:Is%20Valid
        (Class|BPIInteract|Interact(Message) (Variables|Default|GetInteractableActor) self)))))

(event Input|MouseEvents|LeftMouseButton
  (params (Key :type Key%20Structure :default "None"))
  (:Pressed
    (Variables|Default|SetCheckRT_Erase true)
    (Default|CallSuckTriggered))
  (:Released
    (Variables|Default|SetCheckRT_Erase false)))

(event Input|MouseEvents|RightMouseButton
  (params (Key :type Key%20Structure :default "None"))
  (:Pressed
    (Variables|Default|SetCheckRT_Paint true))
  (:Released
    (Variables|Default|SetCheckRT_Paint false)))

(fn ConstructionScript
  (|CallParentFunction))

(fn LineTraceRT
  (bind _firstpersoncameracomponent (Variables|Default|GetFirstPersonCameraComponent))
  (bind _firstpersoncameracomponent_2 (Variables|Default|GetFirstPersonCameraComponent))
  (bind _returnvalue (Transformation|GetWorldLocation _firstpersoncameracomponent_2))
  (bind _returnvalue_2 (Transformation|GetWorldLocation _firstpersoncameracomponent))
  (Utilities|FlowControl|Sequence
    (:then_0
      (if (Variables|Default|GetCheckRT_Erase)
        (bind _outhits (Class|KismetSystemLibrary|LineTraceMultiforObjects _returnvalue_2 (+ _returnvalue_2 (* (Math|Vector|GetForwardVector _firstpersoncameracomponent) 1e+03)) (Utilities|Array|MakeArray "ObjectTypeQuery1" "ObjectTypeQuery2") false 0 "ForOneFrame" false))
        (for _array_element _outhits
          (if (.bBlockingHit (Collision|BreakHitResult _array_element))
            (Class|BPIPaint|OnErase(Message) (.HitActor (Collision|BreakHitResult _array_element)) (.UV (Class|GameplayStatics|FindCollisionUV _array_element)))))))
    (:then_1
      (if (Variables|Default|GetCheckRT_Paint)
        (bind _outhits_2 (Class|KismetSystemLibrary|LineTraceMultiforObjects _returnvalue (+ _returnvalue (* (Math|Vector|GetForwardVector _firstpersoncameracomponent_2) 1e+03)) (Utilities|Array|MakeArray "ObjectTypeQuery1" "ObjectTypeQuery2") false 0 "ForOneFrame" false))
        (for _array_element_2 _outhits_2
          (if (.bBlockingHit (Collision|BreakHitResult _array_element_2))
            (Class|BPIPaint|OnPaint(Message) (.HitActor (Collision|BreakHitResult _array_element_2)) (.UV (Class|GameplayStatics|FindCollisionUV _array_element_2)))))))))