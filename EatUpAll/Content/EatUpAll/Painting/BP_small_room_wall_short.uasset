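; Short small-room wall Blueprint whose surface can be painted and erased at given UVs through render targets.
; The construction script builds splat and copy material instances; BeginPlay clears both targets and feeds the runtime one to the mesh's dynamic materials.
; OnPaint and OnErase draw a splat into the runtime target, then ping-pong through the persistent target to accumulate strokes.
; Render target creation nodes are disconnected, so both targets come from existing variable values.
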(event Custom|EraseToRenderTarget
  (params (Strength :type Float%20%28double-precision%29) (Size :type Float%20%28double-precision%29) (LocationToErase :type Vector%202D%20Structure) (TextureRenderTarget :type Texture%20Render%20Target%202D%20Object%20Reference) (TextureRenderTarget2 :type Texture%20Render%20Target%202D%20Object%20Reference))
  (bind _mid_erasesplat (Variables|Default|GetMID_Erasesplat))
  ;[0.3851 1 0.9801] Paint and Erase
  ;;[1 1 1] Draw RenderTarget
  (Rendering|Material|SetScalarParameterValue _mid_erasesplat "Strength" Strength :!class /Script/Engine.MaterialInstanceDynamic)
  (Rendering|Material|SetScalarParameterValue _mid_erasesplat "Size" Size :!class /Script/Engine.MaterialInstanceDynamic)
  (Rendering|Material|SetVectorParameterValue _mid_erasesplat "Position" (Math|Conversions|ToLinearColor(Vector) (Math|Conversions|ToVector(Vector2D) LocationToErase 0.1)) :!class /Script/Engine.MaterialInstanceDynamic)
  (Rendering|DrawMaterialtoRenderTarget TextureRenderTarget _mid_erasesplat)
  (Rendering|DrawMaterialtoRenderTarget TextureRenderTarget2 (Variables|Default|GetDrawToPersistantMaterial))
  (Rendering|DrawMaterialtoRenderTarget TextureRenderTarget (Variables|Default|GetDrawToRuntimeMaterial)))

(event Custom|SetValues
  ;[1 1 1] Inital Setting
  (for _array_element (Variables|Default|GetDynamicMaterials)
    (Rendering|Material|SetTextureParameterValue _array_element "RT_Runtime" (Variables|Default|GetRenderTargetRuntime))))

(event Custom|DrawToRenderTarget
  (params (Strength :type Float%20%28double-precision%29) (Size :type Float%20%28double-precision%29) (LocationToDraw :type Vector%202D%20Structure) (TextureRenderTarget :type Texture%20Render%20Target%202D%20Object%20Reference) (TextureRenderTarget2 :type Texture%20Render%20Target%202D%20Object%20Reference))
  (bind _mid_paintsplat (Variables|Default|GetMID_Paintsplat))
  ;[0.3851 1 0.9801] Paint and Erase
  ;;[1 1 1] Draw RenderTarget
  (Rendering|Material|SetScalarParameterValue _mid_paintsplat "Strength" Strength :!class /Script/Engine.MaterialInstanceDynamic)
  (Rendering|Material|SetScalarParameterValue _mid_paintsplat "Size" Size :!class /Script/Engine.MaterialInstanceDynamic)
  (Rendering|Material|SetVectorParameterValue _mid_paintsplat "Position" (Math|Conversions|ToLinearColor(Vector) (Math|Conversions|ToVector(Vector2D) LocationToDraw 0.1)) :!class /Script/Engine.MaterialInstanceDynamic)
  (Rendering|DrawMaterialtoRenderTarget TextureRenderTarget _mid_paintsplat)
  (Rendering|DrawMaterialtoRenderTarget TextureRenderTarget2 (Variables|Default|GetDrawToPersistantMaterial))
  (Rendering|DrawMaterialtoRenderTarget TextureRenderTarget (Variables|Default|GetDrawToRuntimeMaterial)))

(event EventOnPaint
  (params (UV :type Vector%202D%20Structure))
  ;[0.3851 1 0.9801] Paint and Erase
  ;;[1 1 1] Input for Paint
  (CallFunction|DrawtoRenderTarget (Variables|Default|GetStrength) (Variables|Default|GetSize) UV (Variables|Default|GetRenderTargetRuntime) (Variables|Default|GetRenderTargetPersistant)))

(event EventOnErase
  (params (UV :type Vector%202D%20Structure))
  ;[0.3851 1 0.9801] Paint and Erase
  ;;[1 1 1] Input for Erase
  (CallFunction|ErasetoRenderTarget (Variables|Default|GetStrength) (Variables|Default|GetSize) UV (Variables|Default|GetRenderTargetRuntime) (Variables|Default|GetRenderTargetPersistant)))

(event EventBeginPlay
  (bind _staticmesh (Variables|Default|GetStaticMesh))
  ;[1 1 1] Inital Setting
  (for (_array_element _array_index) (Rendering|Material|GetMaterials _staticmesh)
    (bind _returnvalue (Rendering|Material|CreateDynamicMaterialInstance _staticmesh _array_index _array_element "None" :!class /Script/Engine.PrimitiveComponent))
    (Utilities|Array|SetArrayElem (Variables|Default|GetDynamicMaterials) 0 _returnvalue true)
    (Rendering|Material|SetTextureParameterValue (Variables|Default|GetDrawToPersistantMaterial) "RT_Capture" (Variables|Default|GetRenderTargetRuntime))
    (Rendering|Material|SetTextureParameterValue (Variables|Default|GetDrawToRuntimeMaterial) "RT_Persistant" (Variables|Default|GetRenderTargetPersistant))
    (Rendering|ClearRenderTarget2D (Variables|Default|GetRenderTargetRuntime))
    (Rendering|ClearRenderTarget2D (Variables|Default|GetRenderTargetPersistant)))
  (CallFunction|SetValues))

(fn ConstructionScript
  (Utilities|FlowControl|Sequence
    (:then_0
      (bind _returnvalue (Rendering|Material|CreateDynamicMaterialInstance "/Game/EatUpAll/Painting/M_PaintSplat.M_PaintSplat" "None" "None" :!class /Script/Engine.KismetMaterialLibrary))
      (Variables|Default|SetMID_Paintsplat _returnvalue))
    (:then_1
      (bind _returnvalue_2 (Rendering|Material|CreateDynamicMaterialInstance "/Game/EatUpAll/Painting/M_EraseSplat.M_EraseSplat" "None" "None" :!class /Script/Engine.KismetMaterialLibrary))
      (Variables|Default|SetMID_Erasesplat _returnvalue_2))
    (:then_2
      (bind _returnvalue_3 (Rendering|Material|CreateDynamicMaterialInstance "/Game/EatUpAll/Painting/RT/M_DrawToPersistant.M_DrawToPersistant" "None" "None" :!class /Script/Engine.KismetMaterialLibrary))
      (Variables|Default|SetDrawToPersistantMaterial _returnvalue_3))
    (:then_3
      (bind _returnvalue_4 (Rendering|Material|CreateDynamicMaterialInstance "/Game/EatUpAll/Painting/RT/M_DrawToRuntime.M_DrawToRuntime" "None" "None" :!class /Script/Engine.KismetMaterialLibrary))
      (Variables|Default|SetDrawToRuntimeMaterial _returnvalue_4))))