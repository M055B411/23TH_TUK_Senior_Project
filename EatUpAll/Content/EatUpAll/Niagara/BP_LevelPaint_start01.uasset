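; Short-lived level paint actor that turns Niagara particle data into paint, then deactivates its effect and destroys itself after ten seconds.
; While its paint check is on, each exported particle is forwarded through a server event to a multicast-named event, apparently replicating the paint to clients.
; That final event calls Paint four times per particle, each along a different diagonal direction.
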(event Custom|Destroy%20Self
  (Components|Activation|SetActive (Variables|Default|GetNiagara) false false)
  (Variables|Default|SetPaintCheck false)
  (Actor|DestroyActor))

(event EventBeginPlay
  (|CallParentFunction)
  (Utilities|Time|SetTimerbyEvent (delegate Custom|Destroy%20Self) 1e+01))

(event Collision|EventActorBeginOverlap
  (params (OtherActor :type Actor%20Object%20Reference)))

(event EventTick
  (params (DeltaSeconds :type Float%20%28single-precision%29)))

(event EventParticleData
  (params (Data :type Array%20of%20Basic%20Particle%20Data%20Structures) (NiagaraSystem :type Niagara%20System%20Object%20Reference) (SimulationPositionOffset :type Vector%20%28by%20ref%29 :default "0, 0, 0"))
  (if (Variables|Default|GetPaintCheck)
    (for _array_element Data
      (CallFunction|ReceiveParticleDataServer _array_element))))

(event EventParticleDataServer
  (params (Data :type Basic%20Particle%20Data%20Structure))
  (CallFunction|ReceiveParticleDataMulti Data))

(event EventParticleDataMulti
  (params (Data :type Basic%20Particle%20Data%20Structure))
  (CallFunction|Paint Data "-100.000000,100.000000,-100.000000")
  (CallFunction|Paint Data "-100.000000,-100.000000,100.000000")
  (CallFunction|Paint Data "100.000000,100.000000,-100.000000")
  (CallFunction|Paint Data "100.000000,-100.000000,100.000000"))

(fn ConstructionScript
  (|CallParentFunction))