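; BP_LevelPaint01 turns exported Niagara particle positions into paint hits on the actors beneath them.
; On BeginPlay it registers itself as the Niagara system's `User.BPCallback` to receive particle data.
; Each particle triggers a short downward object trace, drawn for debugging.
; Blocking hits pass their collision UV to the hit actor through `OnPaintMessage`, leaving the painting to that actor.
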(event EventBeginPlay
  (Niagara|SetNiagaraVariable(Object) (Variables|Default|GetNiagara) "User.BPCallback" self))

(event EventParticleData
  (params (Data :type Array%20of%20Basic%20Particle%20Data%20Structures) (NiagaraSystem :type Niagara%20System%20Object%20Reference) (SimulationPositionOffset :type Vector%20%28by%20ref%29 :default "0, 0, 0"))
  (for _array_element Data
    (bind _outhit (Collision|LineTraceForObjects (.Position (Utilities|Struct|BreakBasicParticleData _array_element)) (+ (.Position (Utilities|Struct|BreakBasicParticleData _array_element)) "0.000000,0.000000,-100.000000") (Utilities|Array|MakeArray "ObjectTypeQuery1" "ObjectTypeQuery2" "ObjectTypeQuery3") false 0 "ForOneFrame"))
    (for _array_element_2 (Utilities|Array|MakeArray _outhit)
      (if (.bBlockingHit (Collision|BreakHitResult _array_element_2))
        (Class|BPIPaint|OnPaint(Message) (.HitActor (Collision|BreakHitResult _array_element_2)) (.UV (Class|GameplayStatics|FindCollisionUV _array_element_2)))))))

(fn ConstructionScript)