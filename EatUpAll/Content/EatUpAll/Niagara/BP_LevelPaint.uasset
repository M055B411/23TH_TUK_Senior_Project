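; BP_LevelPaint is an actor that turns Niagara particle positions into paint on the level.
; The server activates the Niagara system with itself as export callback, then relays each exported particle through server and multicast events.
; Paint traces 100 units downward from each particle and sends the collision UV of blocking hits to the hit actors through OnPaintMessage.
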(event Custom|Receive%20ParticleData%20Server
  (params (Data :type Basic%20Particle%20Data%20Structure))
  (CallFunction|ReceiveParticleDataMulti Data))

(event Custom|Receive%20ParticleData%20Multi
  (params (Data :type Basic%20Particle%20Data%20Structure))
  (CallFunction|Paint Data "0.000000,0.000000,-100.000000"))

(event EventBeginPlay
  (if (Networking|IsServer)
    (Niagara|SetNiagaraVariable(Object) (Variables|Default|GetNiagara) "User.BPCallback" self)
    (Components|Activation|SetActive (Variables|Default|GetNiagara) true false)))

(event EventParticleData
  (params (Data :type Array%20of%20Basic%20Particle%20Data%20Structures) (NiagaraSystem :type Niagara%20System%20Object%20Reference) (SimulationPositionOffset :type Vector%20%28by%20ref%29 :default "0, 0, 0"))
  (for _array_element Data
    (CallFunction|ReceiveParticleDataServer _array_element)))

(fn ConstructionScript)

(fn Paint
  (params (BasicParticleData :type Basic%20Particle%20Data%20Structure) (PaintDirection :type Vector))
  (bind _position (Utilities|Struct|BreakBasicParticleData BasicParticleData))
  (bind _outhits (Class|KismetSystemLibrary|LineTraceMultiforObjects _position (+ _position PaintDirection) (Utilities|Array|MakeArray "ObjectTypeQuery1" "ObjectTypeQuery2" "ObjectTypeQuery3" "ObjectTypeQuery8" "ObjectTypeQuery10") false 0 "None" true))
  (for _array_element _outhits
    (if (.bBlockingHit (Collision|BreakHitResult _array_element))
      (Class|BPIPaint|OnPaint(Message) (.HitActor (Collision|BreakHitResult _array_element)) (.UV (Class|GameplayStatics|FindCollisionUV _array_element))))))