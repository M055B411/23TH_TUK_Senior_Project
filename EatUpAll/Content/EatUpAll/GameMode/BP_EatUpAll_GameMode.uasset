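; Game mode for EatUpAll that relays match phases and Slime, Hunter or draw results to every player controller.
; It adds controllers to an array and counts them on login and logout, printing debug messages.
; On BeginPlay it binds a handler to each phase and result event.
; Each handler loops over the array, casts to BP_PlayerContorller and calls the matching Start function.
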(event Custom|Enter%20PhaseReady
  (for _array_element (Variables|Default|GetPCs)
    (bind _asbp_player_contorller (Utilities|Casting|CastToBP_PlayerContorller _array_element))
    (Default|StartPhaseReady _asbp_player_contorller)))

(event Custom|Enter%20Phase0
  (for _array_element (Variables|Default|GetPCs)
    (bind _asbp_player_contorller (Utilities|Casting|CastToBP_PlayerContorller _array_element))
    (Default|StartPhasePlay0 _asbp_player_contorller)))

(event Custom|Enter%20Phase1'5
  (for _array_element (Variables|Default|GetPCs)
    (bind _asbp_player_contorller (Utilities|Casting|CastToBP_PlayerContorller _array_element))
    (Default|StartPhasePlay1'5 _asbp_player_contorller)))

(event Custom|Enter%20SlimeWinResult
  (for _array_element (Variables|Default|GetPCs)
    (bind _asbp_player_contorller (Utilities|Casting|CastToBP_PlayerContorller _array_element))
    (Default|StartSlimeWinResult _asbp_player_contorller)))

(event Custom|Enter%20Phase1
  (for _array_element (Variables|Default|GetPCs)
    (bind _asbp_player_contorller (Utilities|Casting|CastToBP_PlayerContorller _array_element))
    (Default|StartPhasePlay1 _asbp_player_contorller)))

(event Custom|Enter%20HunterWinResult
  (for _array_element (Variables|Default|GetPCs)
    (bind _asbp_player_contorller (Utilities|Casting|CastToBP_PlayerContorller _array_element))
    (Default|StartHunterWinResult _asbp_player_contorller)))

(event Custom|Enter%20Phase2
  (for _array_element (Variables|Default|GetPCs)
    (bind _asbp_player_contorller (Utilities|Casting|CastToBP_PlayerContorller _array_element))
    (Default|StartPhasePlay2 _asbp_player_contorller)))

(event Custom|Enter%20DrawResult
  (for _array_element (Variables|Default|GetPCs)
    (bind _asbp_player_contorller (Utilities|Casting|CastToBP_PlayerContorller _array_element))
    (Default|StartDrawResult _asbp_player_contorller)))

(event EventBeginPlay
  (EventDispatchers|BindEventtoPhaseReady (delegate Custom|Enter%20PhaseReady))
  (EventDispatchers|BindEventtoPhase0 (delegate Custom|Enter%20Phase0))
  (EventDispatchers|BindEventtoPhase1 (delegate Custom|Enter%20Phase1))
  (EventDispatchers|BindEventtoPhase1'5 (delegate Custom|Enter%20Phase1'5))
  (EventDispatchers|BindEventtoPhase2 (delegate Custom|Enter%20Phase2))
  (EventDispatchers|BindEventtoSlimeWinResult (delegate Custom|Enter%20SlimeWinResult))
  (EventDispatchers|BindEventtoHunterWinResult (delegate Custom|Enter%20HunterWinResult))
  (EventDispatchers|BindEventtoDrawResult (delegate Custom|Enter%20DrawResult)))

(event EventPostLogin
  (params (NewPlayer :type Player%20Controller%20Object%20Reference))
  (Utilities|Array|Add (Variables|Default|GetPCs) NewPlayer)
  (bind _result (Math|Integer|IncrementInt (Variables|Default|GetPC%20Num))
    (:%20%20
      (bind _output_get (Variables|Default|SetPC%20Num _result))
      (Development|PrintString "OnPostLogin - Add PC " false)
      (Development|PrintString (Utilities|String|Append "OnPostLogin PC Num - " (Utilities|String|ToString(Integer) _output_get)) false true "(R=1.000000,G=0.000000,B=0.687739,A=1.000000)"))))

(event EventOnLogout
  (params (ExitingController :type Controller%20Object%20Reference))
  (bind _asbp_player_contorller (Utilities|Casting|CastToBP_PlayerContorller ExitingController))
  (Utilities|Array|RemoveItem (Variables|Default|GetPCs) _asbp_player_contorller)
  (bind _result (Math|Integer|DecrementInt (Variables|Default|GetPC%20Num))
    (:%20%20
      (bind _output_get (Variables|Default|SetPC%20Num _result))
      (Development|PrintString "LogOut - Remove PC " false)
      (Development|PrintString (Utilities|String|Append "LoginOut PC Num - " (Utilities|String|ToString(Integer) _output_get)) false true "(R=1.000000,G=0.000000,B=0.687739,A=1.000000)"))))

(fn ConstructionScript)