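; Slime movement component that lets the locally controlled character crawl over arbitrary surfaces, moving relative to camera and control rotation.
; Each tick, line-trace grids toward acceleration (heavily weighted) and the current surface average hit normals into a stick direction, offsetting the actor along it.
; A distance sphere trace attaches to the hit component or starts falling; a radial sphere sweep re-snaps when ground traces miss.
; A pivot component smoothly follows the capsule's position and surface orientation.
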(event EventTick
  (params (DeltaSeconds :type Float%20%28single-precision%29))
  (if (Pawn|IsLocallyControlled (Variables|/Script/Engine.Actor|GetInstigator (Components|GetOwner)))
    (Utilities|Array|Clear (Variables|Default|GetNormals))
    (Utilities|FlowControl|Sequence
      (:then_0
        (bind _output_get (Variables|Default|SetMoving (or (!= (Variables|Default|GetForwardAxisValue) 0.0) (!= (Variables|Default|GetRight%20Axis%20Value) 0.0))))
        (if _output_get
          (CallFunction|GuidingTraces "None")))
      (:then_1
        (CallFunction|GroundTraces "None")
        (CallFunction|DistanceTrace "None")
        (CallFunction|PivotComponentLocomotion 0.1 0.08)))))

(event EventBeginPlay)

(event EventForwardInputMovement
  (params (AxisValue :type Float%20%28double-precision%29))
  (Variables|Default|SetForwardAxisValue AxisValue)
  (Movement|ForwardsMovement))

(event EventRightInputMovement
  (params (AxisValue :type Float%20%28double-precision%29))
  (Variables|Default|SetRight%20Axis%20Value AxisValue)
  (Movement|SidewaysMovement))

(event EventMainInitialization
  (params (Capsule_Component :type Capsule%20Component%20Object%20Reference) (Character_Movement :type Character%20Movement%20Component%20Object%20Reference) (Camera_Component :type Camera%20Component%20Object%20Reference) (Pivot_Component :type Scene%20Component%20Object%20Reference))
  (Variables|Default|SetCapsuleComponent Capsule_Component)
  (Variables|Default|SetCharacterMovement Character_Movement)
  (Variables|Default|SetFollow%20Camera Camera_Component)
  (Variables|Default|SetPivotComponent Pivot_Component)
  (Variables|/Script/Engine.CharacterMovementComponent|SetbOrientRotationToMovement (Variables|Default|GetCharacterMovement) false)
  (Variables|Default|SetInitial%20Offset (Math|Vector|GetForwardVector (Variables|Default|GetCapsuleComponent)))
  (Utilities|FlowControl|Delay 0.2)
  (Variables|Default|SetStartingDelay true))

(fn GridTrace
  (params (NumberOfRows :type Integer) (NumberOfColumns :type Integer) (Start :type Vector) (ForwardVector :type Vector) (RightVector :type Vector) (UpVector :type Vector) (Range :type Float%20%28double-precision%29) (DistanceBetweenX :type Float%20%28double-precision%29) (DistanceBetweenY :type Float%20%28double-precision%29) (DrawDebugType :type EDrawDebugTrace%20Enum :default "None") (TraceColor :type Linear%20Color%20Structure))
  (bind _normalsarray (LocalVariables|GetNormalsArray))
  (for _index (range 1 NumberOfRows)
    (for _index_2 (range 1 NumberOfColumns)
      (bind (_outhit _returnvalue) (Collision|LineTraceByChannel (+ (* RightVector (Math|Conversions|ToVector(Float) (* (Math|Conversions|ToFloat(Integer) (Utilities|Operators|Subtract _index_2 (/ NumberOfColumns 2) 1)) DistanceBetweenX))) (* UpVector (Math|Conversions|ToVector(Float) (* (Math|Conversions|ToFloat(Integer) (Utilities|Operators|Subtract _index (/ NumberOfRows 2) 1)) DistanceBetweenY))) Start) (+ (+ (* RightVector (Math|Conversions|ToVector(Float) (* (Math|Conversions|ToFloat(Integer) (Utilities|Operators|Subtract _index_2 (/ NumberOfColumns 2) 1)) DistanceBetweenX))) (* UpVector (Math|Conversions|ToVector(Float) (* (Math|Conversions|ToFloat(Integer) (Utilities|Operators|Subtract _index (/ NumberOfRows 2) 1)) DistanceBetweenY))) Start) (* (Math|Vector|GetUnitDirection(Vector) (+ (* RightVector (Math|Conversions|ToVector(Float) (* (Math|Conversions|ToFloat(Integer) (Utilities|Operators|Subtract _index_2 (/ NumberOfColumns 2) 1)) DistanceBetweenX))) (* UpVector (Math|Conversions|ToVector(Float) (* (Math|Conversions|ToFloat(Integer) (Utilities|Operators|Subtract _index (/ NumberOfRows 2) 1)) DistanceBetweenY))) Start) (+ Start (* UpVector (Math|Conversions|ToVector(Float) (* (Math|Conversions|ToFloat(Integer) (Utilities|Operators|Subtract _index (/ NumberOfRows 2) 1)) DistanceBetweenY))) (* RightVector (Math|Conversions|ToVector(Float) (* (Math|Conversions|ToFloat(Integer) (Utilities|Operators|Subtract _index_2 (/ NumberOfColumns 2) 1)) DistanceBetweenX))) ForwardVector)) (Math|Conversions|ToVector(Float) Range))) "TraceTypeQuery1" true (Variables|Default|GetActors%20to%20Ignore) DrawDebugType true TraceColor "(R=0.000000,G=0.112263,B=0.364583,A=1.000000)" 0.0))
      (if _returnvalue
        (if (not (Physics|IsSimulatingPhysics (.HitComponent (Collision|BreakHitResult _outhit)) "None"))
          (Utilities|Array|Add (LocalVariables|GetNormalsArray) (.Normal (Collision|BreakHitResult _outhit)))))))
  (return (> (Utilities|Array|Length _normalsarray) 0) (Math|Vector|GetVectorArrayAverage _normalsarray)))

(fn MultiGridTrace
  (params (Density :type Integer) (RangeMul :type Float%20%28double-precision%29) (GuideRotator :type Rotator) (Start :type Vector) (DrawDebugType :type EDrawDebugTrace%20Enum :default "None") (TraceColor :type Linear%20Color%20Structure) (DivideSize :type Float%20%28double-precision%29) (Spread :type Float%20%28double-precision%29))
  (bind _localnormals (LocalVariables|GetLocalNormals))
  (bind _capsulecomponent (Variables|Default|GetCapsuleComponent))
  (bind (_outradius _outhalfheight) (Components|Capsule|GetScaledCapsuleSize _capsulecomponent))
  (bind _output_get (LocalVariables|SetXindex Density))
  (LocalVariables|SetYindex _output_get)
  (LocalVariables|SetRange (* RangeMul (Components|Capsule|GetScaledCapsuleRadius (Variables|Default|GetCapsuleComponent))))
  (for _index (range 0 3)
    (bind (_hit__ _newparam) (Traces|GridTrace (LocalVariables|GetXindex) (LocalVariables|GetYindex) Start (+ (Math|Vector|GetForwardVector GuideRotator) (* (Math|Conversions|ToVector(Float) (* (Utilities|Select :Index _index :Option%200 1.0 :Option%201 -1.0 :Option%202 1.0 :Option%203 -1.0) Spread)) (Math|Vector|GetRightVector GuideRotator)) (* (Math|Conversions|ToVector(Float) (* Spread (Utilities|Select :Index _index :Option%200 1.0 :Option%201 1.0 :Option%202 -1.0 :Option%203 -1.0))) (Math|Vector|GetUpVector GuideRotator))) (Math|Vector|GetRightVector GuideRotator) (Math|Vector|GetUpVector GuideRotator) (LocalVariables|GetRange) (/ _outradius DivideSize) (/ _outhalfheight DivideSize) DrawDebugType TraceColor))
    (if _hit__
      (Utilities|Array|Add (LocalVariables|GetLocalNormals) _newparam)))
  (return (> (Utilities|Array|Length _localnormals) 0) (Math|Vector|GetVectorArrayAverage _localnormals)))

(fn SphereTrace
  (params (Start :type Vector) (Density :type Float%20%28double-precision%29) (Range :type Integer) (Radius :type Float%20%28double-precision%29) (DrawDebugType :type EDrawDebugTrace%20Enum :default "None"))
  (bind _returnvalue (* 36.0 Density))
  (bind _returnvalue_2 (* 36.0 Density))
  (bind _returnvalue_3 (- _returnvalue 0.0))
  (bind _returnvalue_4 (- _returnvalue_2 0.0))
  (bind _returnvalue_5 (Math|Float|Truncate _returnvalue_4))
  (bind _returnvalue_6 (Math|Float|Truncate _returnvalue_3))
  (for _index (range 0 _returnvalue_6)
    (LocalVariables|SetPitch (* (Math|Conversions|ToFloat(Integer) _index) (/ 3.6e+02 (Math|Conversions|ToFloat(Integer) _returnvalue_6))))
    (for _index_2 (range 0 _returnvalue_5)
      (LocalVariables|SetYaw (* (Math|Conversions|ToFloat(Integer) _index_2) (/ 3.6e+02 (Math|Conversions|ToFloat(Integer) _returnvalue_5))))
      (bind _outhit (Collision|SphereTraceByChannel Start (+ Start (* (Math|Vector|RotateVector "1.000000, 0, 0" (Math|Rotator|MakeRotator 0.0 (LocalVariables|GetPitch) (LocalVariables|GetYaw))) (Math|Conversions|ToFloat(Integer) Range))) Radius "TraceTypeQuery1" true 0 DrawDebugType true "(R=1.000000,G=0.000000,B=0.000000,A=1.000000)" "(R=0.000000,G=1.000000,B=0.000000,A=1.000000)" 0.0))
      (LocalVariables|SetLocTemp (.Location (Collision|BreakHitResult _outhit)))
      (LocalVariables|SetDisTemp (Math|Vector|Distance(Vector) (LocalVariables|GetLocTemp) Start))
      (if (< (LocalVariables|GetDisTemp) (LocalVariables|GetMin))
        (LocalVariables|SetMin (LocalVariables|GetDisTemp))
        (LocalVariables|SetMinLoc (LocalVariables|GetLocTemp)))))
  (return (LocalVariables|GetMin) (LocalVariables|GetMinLoc)))

(fn GuidingTraces
  (params (DrawDebugType :type EDrawDebugTrace%20Enum :default "None"))
  (bind _charactermovement (Variables|Default|GetCharacterMovement))
  (bind _capsulecomponent (Variables|Default|GetCapsuleComponent))
  (bind _returnvalue (Pawn|Components|CharacterMovement|GetCurrentAcceleration _charactermovement))
  (bind _returnvalue_2 (Transformation|GetWorldLocation _capsulecomponent))
  (bind (_hit_ _normal) (Traces|MultiGridTrace 3 1.0 (Math|Rotator|FindLookatRotation _returnvalue_2 (+ _returnvalue_2 (Math|Vector|SelectVector "0, 0, 0" (* (Math|Conversions|ToVector(Float) (Variables|/Script/Engine.CapsuleComponent|GetCapsuleRadius (Variables|Default|GetCapsuleComponent))) (Class|KismetMathLibrary|VectorNormalUnsafe _returnvalue)) (Math|Vector|Equal(Vector) _returnvalue "0, 0, 0" 0.0001)))) (Transformation|GetWorldLocation (Variables|Default|GetCapsuleComponent)) DrawDebugType "(R=0.599766,G=0.000000,B=0.713542,A=1.000000)" 4.0 0.15))
  (if _hit_
    (Utilities|Array|AppendArray (Variables|Default|GetNormals) (Utilities|Array|MakeArray _normal _normal _normal _normal _normal _normal _normal))))

(fn DistanceTrace
  (params (DrawDebugType :type EDrawDebugTrace%20Enum :default "None"))
  (bind _capsulecomponent (Variables|Default|GetCapsuleComponent))
  (bind _capsulecomponent_2 (Variables|Default|GetCapsuleComponent))
  (bind _returnvalue (Transformation|GetWorldLocation _capsulecomponent))
  (bind _outradius (Components|Capsule|GetScaledCapsuleSize _capsulecomponent_2))
  (if (not (Variables|Default|GetJumping))
    (bind (_outhit _returnvalue_2) (Collision|SphereTraceByChannel _returnvalue (+ _returnvalue (* (Math|Vector|GetForwardVector (Variables|Default|GetRotator)) (Math|Conversions|ToVector(Float) (* 3.0 _outradius)))) _outradius "TraceTypeQuery1" false (Variables|Default|GetActors%20to%20Ignore) DrawDebugType true "(R=0.232734,G=1.000000,B=0.000000,A=1.000000)" "(R=0.055704,G=0.250000,B=0.000000,A=1.000000)"))
    (Variables|Default|SetDistance (.Distance (Collision|BreakHitResult _outhit)))
    (Variables|Default|SetContactLocation (.ImpactPoint (Collision|BreakHitResult _outhit)))
    (Utilities|IsValid (Variables|Default|GetPivotComponent)
      (:Is%20Valid
        (if _returnvalue_2
          (Variables|Default|SetAttachedTo (.HitComponent (Collision|BreakHitResult _outhit)))
          (bind _returnvalue_3 (Transformation|AttachComponentToComponent (Components|GetOwner (Variables|Default|GetPivotComponent)) (Variables|Default|GetAttachedTo) "None" "KeepWorld" "KeepWorld" "KeepWorld" false))
          (Variables|Default|SetAttached _returnvalue_3)
          (else
            (bind _ascharacter (Utilities|Casting|CastToCharacter (Components|GetOwner)))
            (Pawn|Components|CharacterMovement|SetMovementMode (Variables|/Script/Engine.Character|GetCharacterMovement _ascharacter) "MOVE_Falling" 0)
            (Variables|Default|SetJumping true)))))))

(fn SidewaysMovement
  (bind _returnvalue (Components|GetOwner))
  (bind _instigator (Variables|/Script/Engine.Actor|GetInstigator _returnvalue))
  (bind _returnvalue_2 (Pawn|GetControlRotation _instigator :!class /Script/Engine.Pawn))
  (bind (_roll _pitch _yaw) (Math|Rotator|BreakRotator _returnvalue_2))
  (Class|BPISlime|AddMovement(Message) (Components|GetOwner) (Math|Vector|GetRightVector (Math|Rotator|MakeRotator _roll 0.0 _yaw)) (Variables|Default|GetRight%20Axis%20Value) false)
  (if (!= 0.0 (Variables|Default|GetRight%20Axis%20Value))
    (Variables|Default|SetInitialOffset "0, 0, 0")))

(fn ForwardsMovement
  (bind _returnvalue (Math|Conversions|ToVector(Float) 0.2))
  (bind _follow_camera (Variables|Default|GetFollow%20Camera))
  (bind _forwardaxisvalue (Variables|Default|GetForwardAxisValue))
  (bind _capsulecomponent (Variables|Default|GetCapsuleComponent))
  (bind _forwardaxisvalue_2 (Variables|Default|GetForwardAxisValue))
  (bind _follow_camera_2 (Variables|Default|GetFollow%20Camera))
  (bind _capsulecomponent_2 (Variables|Default|GetCapsuleComponent))
  (bind _capsulecomponent_3 (Variables|Default|GetCapsuleComponent))
  (bind _outradius (Components|Capsule|GetScaledCapsuleSize _capsulecomponent_2))
  (bind _returnvalue_2 (Math|Vector|GetForwardVector _follow_camera))
  (bind _returnvalue_3 (Transformation|GetWorldLocation _capsulecomponent))
  (bind _returnvalue_4 (Components|Capsule|GetScaledCapsuleRadius _capsulecomponent_3))
  (bind _returnvalue_5 (Math|Vector|GetUpVector _follow_camera_2))
  (bind _returnvalue_6 (* _returnvalue_2 _returnvalue))
  (bind _returnvalue_7 (* _returnvalue_4 _forwardaxisvalue 2.0))
  (bind _returnvalue_8 (Math|Conversions|ToVector(Float) _returnvalue_7))
  (bind _returnvalue_9 (+ _returnvalue_6 _returnvalue_5))
  (bind _returnvalue_10 (* _returnvalue_9 _returnvalue_8))
  (bind _returnvalue_11 (+ _returnvalue_10 _returnvalue_3))
  (bind (_outhit _returnvalue_12) (Collision|SphereTraceByChannel _returnvalue_11 (+ (Transformation|GetWorldLocation (Variables|Default|GetCapsuleComponent)) (* (Math|Conversions|ToVector(Float) (* _outradius 8.0)) (Math|Vector|GetUnitDirection(Vector) (+ (Transformation|GetWorldLocation (Variables|Default|GetFollow%20Camera)) (* (Math|Vector|GetUpVector (Variables|Default|GetFollow%20Camera)) (Math|Conversions|ToVector(Float) 0.5))) _returnvalue_11))) (* _outradius 0.2) "TraceTypeQuery1" false (Variables|Default|GetActors%20to%20Ignore) "None" true "(R=0.000000,G=1.000000,B=0.931906,A=1.000000)" "(R=0.000000,G=0.017203,B=1.000000,A=1.000000)" 0.5))
  (Variables|Default|SetForwardProxy (select (not _returnvalue_12) (.TraceEnd (Collision|BreakHitResult _outhit)) (.Location (Collision|BreakHitResult _outhit))))
  (Class|BPISlime|AddMovement(Message) (Components|GetOwner) (Math|Vector|GetUnitDirection(Vector) (Transformation|GetWorldLocation (Variables|Default|GetCapsuleComponent)) (Variables|Default|GetForwardProxy)) (Math|Float|SelectFloat _forwardaxisvalue_2 (Math|Float|Absolute(Float) _forwardaxisvalue_2) (< (Class|KismetMathLibrary|DegAcos (Math|Vector|DotProduct (Math|Vector|GetUpVector (Variables|Default|GetPivotComponent)) (Math|Vector|GetUpVector (Variables|Default|GetFollow%20Camera)))) 45.0)) false)
  (if (!= 0.0 (Variables|Default|GetForwardAxisValue))
    (Variables|Default|SetInitialOffset "0, 0, 0")))

(fn GroundTraces
  (params (DrawDebugType :type EDrawDebugTrace%20Enum :default "None"))
  (bind (_hit_ _normal) (Traces|MultiGridTrace 5 2.0 (Variables|Default|GetRotator) (Transformation|GetWorldLocation (Variables|Default|GetCapsuleComponent)) DrawDebugType "(R=0.000000,G=0.071185,B=0.479167,A=1.000000)" 4.0 0.35))
  (if _hit_
    (Utilities|Array|Add (Variables|Default|GetNormals) _normal)
    (Variables|Default|SetRotator (Math|Rotator|MakeRotfromX (* (Math|Vector|GetVectorArrayAverage (Variables|Default|GetNormals)) "-1.000000,-1.000000,-1.000000")))
    (Transformation|AddActorWorldOffset (Components|GetOwner) (* (Math|Vector|GetForwardVector (Variables|Default|GetRotator)) (+ -5.0 (Variables|Default|GetDistance))))
    (else
      (CallFunction|PositionFix))))

(fn PivotComponentLocomotion
  (params (MovementAlpha :type Float%20%28single-precision%29) (RotationAlpha :type Float%20%28single-precision%29))
  (bind _attachedto (Variables|Default|GetAttachedTo))
  (bind _attachedto_2 (Variables|Default|GetAttachedTo))
  (bind _output_get (LocalVariables|SetLoc (Math|Vector|Lerp(Vector) (Transformation|GetWorldLocation (Variables|Default|GetPivotComponent)) (Transformation|GetWorldLocation (Variables|Default|GetCapsuleComponent)) MovementAlpha)))
  (Transformation|SetWorldLocation (Variables|Default|GetPivotComponent) _output_get false false)
  (Utilities|IsValid (Variables|Default|GetAttachedTo)
    (:Is%20Valid
      (if (Math|Boolean|ORBoolean (!= (Variables|Default|GetForwardAxisValue) 0.0) (!= (Variables|Default|GetRight%20Axis%20Value) 0.0) (or (Utilities|Operators|NotEqual(!=) (Transformation|GetWorldLocation _attachedto) (Variables|Default|GetAttachedCompLoc) 0.0) (Utilities|Operators|NotEqual(!=) (Transformation|GetWorldRotation _attachedto) (Variables|Default|GetAttachedCompRpt) 0.0)))
        (LocalVariables|SetRot (Math|Rotator|Lerp(Rotator) (Transformation|GetWorldRotation (Variables|Default|GetPivotComponent)) (Math|Rotator|MakeRotfromXZ (Math|Vector|GetUnitDirection(Vector) (Transformation|GetWorldLocation (Variables|Default|GetPivotComponent)) (+ (Transformation|GetWorldLocation (Variables|Default|GetCapsuleComponent)) (Variables|Default|GetInitialOffset))) (Math|Vector|GetUnitDirection(Vector) (Variables|Default|GetContactLocation) (Transformation|GetWorldLocation (Variables|Default|GetCapsuleComponent)))) RotationAlpha true))
        (Transformation|SetWorldRotation (Variables|Default|GetPivotComponent) (LocalVariables|GetRot) false false)
        (Variables|Default|SetAttachedCompLoc (Transformation|GetWorldLocation _attachedto_2))
        (Variables|Default|SetAttachedCompRpt (Transformation|GetWorldRotation _attachedto_2))
        (return (LocalVariables|GetLoc) (LocalVariables|GetRot) true)
        (else
          _)))
    (:Is%20Not%20Valid
      _))
  (return (LocalVariables|GetLoc) (LocalVariables|GetRot) false))

(fn PositionFix
  (bind _capsulecomponent (Variables|Default|GetCapsuleComponent))
  (bind _capsulecomponent_2 (Variables|Default|GetCapsuleComponent))
  (bind _capsuleradius (Variables|/Script/Engine.CapsuleComponent|GetCapsuleRadius _capsulecomponent_2))
  (bind _capsuleradius_2 (Variables|/Script/Engine.CapsuleComponent|GetCapsuleRadius _capsulecomponent))
  (bind _minloc_ (Traces|SphereTrace (Transformation|GetWorldLocation _capsulecomponent) 0.2 (Math|Float|Truncate (* 3.0 _capsuleradius_2)) (* _capsuleradius_2 1.0) "None"))
  (if (and (Utilities|Operators|NotEqual(!=) :A _minloc_) (Variables|Default|GetStartingDelay))
    (Transformation|SetWorldLocation (Variables|Default|GetCapsuleComponent) _minloc_ false false)
    (bind _minloc__2 (Traces|SphereTrace (Transformation|GetWorldLocation _capsulecomponent_2) 0.4 (Math|Float|Truncate (* 3.0 _capsuleradius)) (* _capsuleradius 0.3) "ForDuration"))
    (Variables|Default|SetRotator (Math|Rotator|FindLookatRotation (Transformation|GetWorldLocation (Variables|Default|GetCapsuleComponent)) _minloc__2))))

(fn MovingTowardsNothingCheck
  (params (DrawDebugType :type EDrawDebugTrace%20Enum :default "None"))
  (bind _pivotcomponent (Variables|Default|GetPivotComponent))
  (bind _capsulecomponent (Variables|Default|GetCapsuleComponent))
  (bind _follow_camera (Variables|Default|GetFollow%20Camera))
  (bind _returnvalue (Math|Vector|GetUpVector _pivotcomponent))
  (bind _returnvalue_2 (Math|Vector|GetForwardVector _follow_camera))
  (bind _returnvalue_3 (Transformation|GetWorldLocation _pivotcomponent))
  (bind _capsuleradius (Variables|/Script/Engine.CapsuleComponent|GetCapsuleRadius _capsulecomponent))
  (bind _returnvalue_4 (* _capsuleradius 0.0))
  (bind _returnvalue_5 (* _capsuleradius 0.5))
  (bind _returnvalue_6 (Math|Conversions|ToVector(Float) _returnvalue_4))
  (bind _returnvalue_7 (Math|Conversions|ToVector(Float) _returnvalue_5))
  (bind _returnvalue_8 (* _returnvalue _returnvalue_6))
  (bind _returnvalue_9 (* _returnvalue_2 _returnvalue_7))
  (bind _returnvalue_10 (+ _returnvalue_3 _returnvalue_8 _returnvalue_9))
  (bind _returnvalue_11 (Collision|SphereTraceByChannel _returnvalue_10 _returnvalue_10 (* (Variables|/Script/Engine.CapsuleComponent|GetCapsuleRadius (Variables|Default|GetCapsuleComponent)) 1.4) "TraceTypeQuery1" false 0 DrawDebugType true "(R=0.873932,G=0.000000,B=1.000000,A=1.000000)"))
  (return _returnvalue_11))

(fn IgnoreTarget
  (params (Actors%20to%20Ignore :type Array%20of%20Actor%20Object%20References))
  (Variables|Default|SetActors%20to%20Ignore Actors%20to%20Ignore))