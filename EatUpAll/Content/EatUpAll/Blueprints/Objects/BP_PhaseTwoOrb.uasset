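; BP_PhaseTwoOrb is a destructible orb that moves the EatUpAll game into its second phase when its health runs out.
; AnyDamage subtracts from a clamped ObjectHP and, at zero, activates the Niagara effect, calls EnterGamePhase2 and sets Dead.
; EnterGamePhase2 casts the game mode to BP_EatUpAll_GameMode and calls its EnterPhase2.
; Dead is not checked here, so further damage at zero health repeats that sequence.
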(event Custom|Enter%20GamePhase2
  (bind _returnvalue (Game|GetGameMode))
  (Utilities|IsValid _returnvalue
    (:Is%20Valid
      (bind _asbp_eat_up_all_game_mode (Utilities|Casting|CastToBP_EatUpAll_GameMode _returnvalue))
      (Default|EnterPhase2 _asbp_eat_up_all_game_mode))))

(event EventBeginPlay
  (|CallParentFunction) ; This node is disabled and will not be called.\nDrag off pins to build functionality.
)

(event Collision|EventActorBeginOverlap
  (params (OtherActor :type Actor%20Object%20Reference))
  (|CallParentFunction OtherActor) ; This node is disabled and will not be called.\nDrag off pins to build functionality.
)

(event EventTick
  (params (DeltaSeconds :type Float%20%28single-precision%29))
  (|CallParentFunction DeltaSeconds) ; This node is disabled and will not be called.\nDrag off pins to build functionality.
)

(event Game|Damage|EventAnyDamage
  (params (Damage :type Float%20%28single-precision%29) (DamageType :type Damage%20Type%20Object%20Reference) (InstigatedBy :type Controller%20Object%20Reference) (DamageCauser :type Actor%20Object%20Reference))
  (bind _output_get (Variables|Default|SetObjectHP (Math|Float|Clamp(Float) (- (Variables|Default|GetObjectHP) Damage) 0.0 1e+01)))
  (if (== _output_get 0.0)
    (Components|Activation|SetActive (Variables|Default|GetNiagara) true false)
    (CallFunction|EnterGamePhase2)
    (Variables|Default|SetDead true)))

(fn ConstructionScript
  (|CallParentFunction))