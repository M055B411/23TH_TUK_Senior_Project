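; BP_screen is a physics mesh object that gets progressively consumed and destroys itself once its material progress maxes out.
; Received damage or paint raises progress, replicated into custom primitive data; the maximum activates Niagara and marks it dead.
; While overlapped, the server applies negative damage to the other actor and runs trace-based buoyancy, pulling the mesh toward the slime's Core socket, scaled by slime HP from the game instance.
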(event Custom|CheckDead
  (if (>= (Variables|Default|GetMaterialProgress) (Variables|Default|GetProgressMax))
    (Components|Activation|SetActive (Variables|Default|GetNiagara) true false)
    (Variables|Default|SetDead true)))

(event Custom|Set%20Material%20Progress%20on%20Client
  (params (Progress :type Float%20%28double-precision%29))
  (CallFunction|SetMaterialProgress Progress)
  (CallFunction|CheckDead))

(event Custom|Set%20Material%20Progress%20on%20Server
  (params (Progress :type Float%20%28double-precision%29))
  (CallFunction|SetMaterialProgressonClient Progress))

(event Custom|Set%20SlimeHP
  (params (MainSlimeHP :type Float%20%28double-precision%29))
  (Variables|Default|SetSlimeHP MainSlimeHP))

(event Collision|EventActorBeginOverlap
  (params (OtherActor :type Actor%20Object%20Reference))
  (CallFunction|OverlapEventBegin OtherActor))

(event Collision|EventActorEndOverlap
  (params (OtherActor :type Actor%20Object%20Reference))
  (CallFunction|ClearOverlapEvent))

(event EventOnPaint
  (params (UV :type Vector%202D%20Structure))
  (Utilities|FlowControl|Delay 0.2)
  (CallFunction|MaterialProgressUp)
  (CallFunction|CheckDead))

(event EventTick
  (params (DeltaSeconds :type Float%20%28single-precision%29))
  (Networking|SwitchHasAuthority
    (:Authority
      (if (Variables|Default|GetDead)
        (Actor|DestroyActor)
        (elif (Variables|Default|GetisOverlapping)
          (Game|Damage|ApplyDamage (Variables|Default|GetOther%20Actor) (* 0.009 -1.0) 0 self)
          (CallFunction|Buoyancy (Variables|Character|GetMesh) 1e+02 "ObjectTypeQuery7"))))))

(event EventBeginPlay
  (Rendering|Material|SetCustomPrimitiveDataFloat (Variables|Character|GetMesh) (+ (Variables|Default|GetMaterialPrimitiveDataIndex) 1) (Variables|Default|GetProgressMax))
  (bind _asbp_eat_up_all_game_instance (Utilities|Casting|CastToBP_EatUpAllGameInstance (Game|GetGameInstance)))
  (EventDispatchers|BindEventtoChangeSlimeHP _asbp_eat_up_all_game_instance (delegate Custom|Set%20SlimeHP)))

(event Game|Damage|EventAnyDamage
  (params (Damage :type Float%20%28single-precision%29) (DamageType :type Damage%20Type%20Object%20Reference) (InstigatedBy :type Controller%20Object%20Reference) (DamageCauser :type Actor%20Object%20Reference))
  (Networking|SwitchHasAuthority
    (:Authority
      (bind _output_get (Variables|Default|SetMaterialProgress (+ (Variables|Default|GetMaterialProgress) (* Damage 0.1))))
      (CallFunction|SetMaterialProgressonServer _output_get))))

(event EventDestroyed
  (bind _asbp_eat_up_all_game_instance (Utilities|Casting|CastToBP_EatUpAllGameInstance (Game|GetGameInstance)))
  (EventDispatchers|UnbindEventfromChangeSlimeHP _asbp_eat_up_all_game_instance (delegate Custom|Set%20SlimeHP)))

(event EventOnErase
  (params (UV :type Vector%202D%20Structure) (Hunter :type Character%20Object%20Reference))
  (Utilities|FlowControl|Delay 0.2)
  (CallFunction|MaterialProgressDown))

(fn ConstructionScript)

(fn Buoyancy
  (params (Float :type Primitive%20Component%20Object%20Reference) (FloatHeight :type Float%20%28double-precision%29) (ObjectType :type EObjectTypeQuery%20Enum :default "ObjectTypeQuery1"))
  (bind _returnvalue (Transformation|GetWorldLocation Float))
  (bind _returnvalue_2 (Transformation|GetWorldScale Float))
  (bind (_outhit _returnvalue_3) (Collision|LineTraceForObjects _returnvalue (- _returnvalue (Math|Vector|MakeVector 0.0 0.0 (+ (/ (+ (.x _returnvalue_2) (.y _returnvalue_2) (.z _returnvalue_2)) 3.0) FloatHeight))) (Utilities|Array|MakeArray ObjectType) false 0 "None" true "(R=1.000000,G=0.000000,B=0.000000,A=1.000000)" "(R=0.000000,G=1.000000,B=0.000000,A=1.000000)" 0.0))
  (if _returnvalue_3
    (bind _asbp_slime_char_for_new_move_single (Utilities|Casting|CastToBP_SlimeCharForNewMove_Single (.HitActor (Collision|BreakHitResult _outhit))))
    (Physics|AddForce Float (+ (* (Math|Vector|Normalize (- (Transformation|GetSocketLocation (Variables|/Game/EatUpAll/Blueprints/Slime/BP_SlimeCharForNewMove_Single.BP_SlimeCharForNewMove_Single_C|GetBody _asbp_slime_char_for_new_move_single) "Core") (Transformation|GetWorldLocation Float))) (* (Math|Float|MapRangeClamped (Variables|Default|GetSlimeHP) 0.0 1e+02 1.0 1e+01) 7e+03)) (* (.ImpactNormal (Collision|BreakHitResult _outhit)) (Math|Float|Lerp (* (Physics|GetMass Float) 5e+01) 0.05 (/ (Math|Vector|VectorLength (- (.Location (Collision|BreakHitResult _outhit)) (Transformation|GetWorldLocation Float))) FloatHeight)))) "None" false)
    (Class|PrimitiveComponent|SetAngularDamping Float 1e+01)
    (Class|PrimitiveComponent|SetLinearDamping Float 5.0)))

(fn OverlapEventBegin
  (params (Other%20Actor :type Actor%20Object%20Reference))
  (Variables|Default|SetisOverlapping true)
  (Variables|Default|SetOther%20Actor Other%20Actor))

(fn ClearOverlapEvent
  (Variables|Default|SetisOverlapping false)
  (Variables|Default|SetOther%20Actor 0))

(fn MaterialProgressUp
  (if (< (Variables|Default|GetMaterialProgress) (Variables|Default|GetProgressMax))
    (Variables|Default|SetMaterialProgress (+ (Variables|Default|GetMaterialProgress) 0.1))))

(fn MaterialProgressDown
  (if (> (Variables|Default|GetMaterialProgress) 0.0)
    (Variables|Default|SetMaterialProgress (- (Variables|Default|GetMaterialProgress) 0.14))))

(fn SetMaterialProgress
  (params (MaterialProgress :type Float%20%28double-precision%29))
  (bind _output_get (Variables|Default|SetMaterialProgress MaterialProgress))
  (Rendering|Material|SetCustomPrimitiveDataFloat (Variables|Character|GetMesh) (Variables|Default|GetMaterialPrimitiveDataIndex) _output_get))