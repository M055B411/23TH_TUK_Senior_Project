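; BP_BigroomALT is a map-paint mesh Blueprint that can create its own render targets, deferring BeginPlay and construction to its parent.
; ServerRT calls MultiRT, which creates two 1024-square float targets: a two-channel RenderTargetRuntime and a single-channel RenderTargetPersistant.
; The only ServerRT call here is disconnected, so this graph never triggers that setup itself.
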(event Custom|Server%20RT
  (CallFunction|MultiRT))

(event Custom|Multi%20RT
  (Utilities|FlowControl|Sequence
    (:then_0
      (bind _returnvalue (Rendering|CreateRenderTarget2D 1024 1024 "RTF_RG16f"))
      (Variables|Default|SetRenderTargetRuntime _returnvalue))
    (:then_1
      (bind _returnvalue_2 (Rendering|CreateRenderTarget2D 1024 1024 "RTF_R16f"))
      (Variables|Default|SetRenderTargetPersistant _returnvalue_2))))

(event EventBeginPlay
  (|CallParentFunction))

(fn ConstructionScript
  (|CallParentFunction))