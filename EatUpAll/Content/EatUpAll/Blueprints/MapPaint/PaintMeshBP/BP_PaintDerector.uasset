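; BP_PaintDerector is a paint-system relay that passes the slime character's size changes to the game instance.
; On BeginPlay it finds BP_SlimeCharForNewMove_Single and binds to its size-to-paint event.
; Each update prints the value, stores it as PaintSlimeSize on BP_EatUpAllGameInstance and calls CallChangeSlimeSize with it.
; An unconnected branch that would call CallSlimeSizeToChild on BP_RootPaint never runs.
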(event Custom|Set%20SlimeSize
  (params (SlimeSize :type Float%20%28double-precision%29))
  (bind _returnvalue (Game|GetGameInstance))
  (bind _asbp_eat_up_all_game_instance (Utilities|Casting|CastToBP_EatUpAllGameInstance _returnvalue))
  (Development|PrintString (Utilities|String|Append "Slime Size Mul : " (Utilities|String|ToString(Float) SlimeSize)) true true "(R=1.000000,G=0.000000,B=0.978704,A=1.000000)" 5.0)
  (bind _output_get (Variables|/Game/EatUpAll/HUD/BP_EatUpAllGameInstance.BP_EatUpAllGameInstance_C|SetPaint%20SlimeSize _asbp_eat_up_all_game_instance SlimeSize))
  (Default|CallChangeSlimeSize _asbp_eat_up_all_game_instance _output_get))

(event EventBeginPlay
  (bind _returnvalue (Actor|GetActorOfClass "/Game/EatUpAll/Blueprints/Slime/BP_SlimeCharForNewMove_Single.BP_SlimeCharForNewMove_Single_C"))
  (EventDispatchers|BindEventtoSlimeSizetoPaint _returnvalue (delegate Custom|Set%20SlimeSize)))

(fn ConstructionScript)