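; BP_2FloorDoor is an automatic double sliding door that opens when anything overlaps its trigger box and closes on end overlap.
; Open and close events use MoveComponentTo to slide the left and right panels apart along X or back to center.
; Each overlap event also plays an open or close sound at the box and switches DoorFrame collision to ignore or block all channels.
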(event OnComponentBeginOverlap(Box)
  (params (OverlappedComponent :type Primitive%20Component%20Object%20Reference) (OtherActor :type Actor%20Object%20Reference) (OtherComp :type Primitive%20Component%20Object%20Reference) (OtherBodyIndex :type Integer) (bFromSweep :type Boolean) (SweepResult :type Hit%20Result%20Structure%20%28by%20ref%29))
  (CallFunction|OpenLDoor)
  (CallFunction|OpenRdoor)
  (Audio|PlaySoundatLocation "/Game/EatUpAll/SoundEffects/Ambient/open_door_01.open_door_01" (Transformation|GetWorldLocation (Variables|Default|GetBox)) "0, 0, 0" 1.0 1.0 0.0 "/Game/EatUpAll/SoundEffects/SlimeSoundAttenuation.SlimeSoundAttenuation" 0 0 0)
  (Collision|SetCollisionResponsetoAllChannels (Variables|Default|GetDoorFrame) "ECR_Ignore"))

(event OnComponentEndOverlap(Box)
  (params (OverlappedComponent :type Primitive%20Component%20Object%20Reference) (OtherActor :type Actor%20Object%20Reference) (OtherComp :type Primitive%20Component%20Object%20Reference) (OtherBodyIndex :type Integer))
  (CallFunction|CloseRDoor)
  (CallFunction|CloseLDoor)
  (Audio|PlaySoundatLocation "/Game/EatUpAll/SoundEffects/Ambient/close_door_01.close_door_01" (Transformation|GetWorldLocation (Variables|Default|GetBox)) "0, 0, 0" 1.0 1.0 0.0 "/Game/EatUpAll/SoundEffects/SlimeSoundAttenuation.SlimeSoundAttenuation" 0 0 0)
  (Collision|SetCollisionResponsetoAllChannels (Variables|Default|GetDoorFrame) "ECR_Block"))

(event Custom|Close%20RDoor
  (Components|MoveComponentTo 0 "0.000000,-205.000000,0.000000" "0, 0, 0" false false 0.2 false))

(event Custom|Open%20LDoor
  (Components|MoveComponentTo 0 "100.000000,-205.000000,0.000000" "0, 0, 0" false false 0.2 false))

(event Custom|Open%20Rdoor
  (Components|MoveComponentTo 0 "-100.000000,-205.000000,0.000000" "0, 0, 0" false false 0.2 false))

(event Custom|Close%20LDoor
  (Components|MoveComponentTo 0 "0.000000,-205.000000,0.000000" "0, 0, 0" false false 0.2 false))

(event EventBeginPlay)

(event Collision|EventActorBeginOverlap
  (params (OtherActor :type Actor%20Object%20Reference)))

(event EventTick
  (params (DeltaSeconds :type Float%20%28single-precision%29)))

(fn ConstructionScript)