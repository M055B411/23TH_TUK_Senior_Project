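; Airlock door prop with two sliding doors, A and B, where opening one closes the other.
; DoorAction toggles them on BeginPlay and on interaction, which LockBox overlap enables for BP_VacuumPlayer, moving panels, playing sounds and switching Pawn collision.
; Sensors at each door toggle a no-pass mark for slime characters and are meant to highlight lock consoles for the vacuum player (hunter).
; The construction script positions frames and lock from variables.
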(event OnComponentBeginOverlap(SlimeSenserA)
  (params (OverlappedComponent :type Primitive%20Component%20Object%20Reference) (OtherActor :type Actor%20Object%20Reference) (OtherComp :type Primitive%20Component%20Object%20Reference) (OtherBodyIndex :type Integer) (bFromSweep :type Boolean) (SweepResult :type Hit%20Result%20Structure%20%28by%20ref%29))
  (bind _locka (Variables|Default|GetLockA))
  ;[1 1 1] Say Slime Cannot Pass + notify lock Console to Hunter
  (Utilities|FlowControl|Sequence
    (:then_0
      (Utilities|Casting|CastToBP_SlimeCharForNewMove_Single OtherActor)
      (Rendering|SetVisibility (Variables|Default|GetExhibitMarkA) true false)
      (Utilities|Casting|CastToBP_VacuumPlayer OtherActor)
      (Utilities|IsValid _locka
        (:Is%20Valid
          (Default|Highlighton _locka))))))

(event OnComponentEndOverlap(SlimeSenserA)
  (params (OverlappedComponent :type Primitive%20Component%20Object%20Reference) (OtherActor :type Actor%20Object%20Reference) (OtherComp :type Primitive%20Component%20Object%20Reference) (OtherBodyIndex :type Integer))
  (bind _locka (Variables|Default|GetLockA))
  ;[1 1 1] Say Slime Cannot Pass + notify lock Console to Hunter
  (Utilities|FlowControl|Sequence
    (:then_0
      (Utilities|Casting|CastToBP_SlimeCharForNewMove_Single OtherActor)
      (Rendering|SetVisibility (Variables|Default|GetExhibitMarkA) false false))
    (:then_1
      (Utilities|Casting|CastToBP_VacuumPlayer OtherActor)
      (Utilities|IsValid _locka
        (:Is%20Valid
          (Default|HighlightOff _locka))))))

(event OnComponentBeginOverlap(SlimeSenserB)
  (params (OverlappedComponent :type Primitive%20Component%20Object%20Reference) (OtherActor :type Actor%20Object%20Reference) (OtherComp :type Primitive%20Component%20Object%20Reference) (OtherBodyIndex :type Integer) (bFromSweep :type Boolean) (SweepResult :type Hit%20Result%20Structure%20%28by%20ref%29))
  (bind _lockb (Variables|Default|GetLockB))
  ;[1 1 1] Say Slime Cannot Pass + notify lock Console to Hunter
  (Utilities|FlowControl|Sequence
    (:then_0
      (Utilities|Casting|CastToBP_SlimeCharForNewMove_Single OtherActor)
      (Rendering|SetVisibility (Variables|Default|GetExhibitMarkB) true false)
      (Utilities|Casting|CastToBP_VacuumPlayer OtherActor)
      (Utilities|IsValid _lockb
        (:Is%20Valid
          (Default|Highlighton _lockb))))))

(event OnComponentEndOverlap(SlimeSenserB)
  (params (OverlappedComponent :type Primitive%20Component%20Object%20Reference) (OtherActor :type Actor%20Object%20Reference) (OtherComp :type Primitive%20Component%20Object%20Reference) (OtherBodyIndex :type Integer))
  (bind _lockb (Variables|Default|GetLockB))
  ;[1 1 1] Say Slime Cannot Pass + notify lock Console to Hunter
  (Utilities|FlowControl|Sequence
    (:then_0
      (Utilities|Casting|CastToBP_SlimeCharForNewMove_Single OtherActor)
      (Rendering|SetVisibility (Variables|Default|GetExhibitMarkB) false false)
      (Utilities|Casting|CastToBP_VacuumPlayer OtherActor)
      (Utilities|IsValid _lockb
        (:Is%20Valid
          (Default|HighlightOff _lockb))))))

(event OnComponentBeginOverlap(LockBox)
  (params (OverlappedComponent :type Primitive%20Component%20Object%20Reference) (OtherActor :type Actor%20Object%20Reference) (OtherComp :type Primitive%20Component%20Object%20Reference) (OtherBodyIndex :type Integer) (bFromSweep :type Boolean) (SweepResult :type Hit%20Result%20Structure%20%28by%20ref%29))
  (bind _asbp_vacuum_player (Utilities|Casting|CastToBP_VacuumPlayer OtherActor))
  (Variables|/Game/EatUpAll/Blueprints/Player/BP_VacuumPlayer.BP_VacuumPlayer_C|SetbIsCanInteraction _asbp_vacuum_player true)
  (Variables|/Game/EatUpAll/Blueprints/Player/BP_VacuumPlayer.BP_VacuumPlayer_C|SetInteraction%20Actor _asbp_vacuum_player self)
  (Variables|/Game/EatUpAll/Blueprints/Player/BP_VacuumPlayer.BP_VacuumPlayer_C|SetInteraction%20TimeSet _asbp_vacuum_player 2.5e+02))

(event OnComponentEndOverlap(LockBox)
  (params (OverlappedComponent :type Primitive%20Component%20Object%20Reference) (OtherActor :type Actor%20Object%20Reference) (OtherComp :type Primitive%20Component%20Object%20Reference) (OtherBodyIndex :type Integer))
  (bind _asbp_vacuum_player (Utilities|Casting|CastToBP_VacuumPlayer OtherActor))
  (Variables|/Game/EatUpAll/Blueprints/Player/BP_VacuumPlayer.BP_VacuumPlayer_C|SetbIsCanInteraction _asbp_vacuum_player false)
  (Variables|/Game/EatUpAll/Blueprints/Player/BP_VacuumPlayer.BP_VacuumPlayer_C|SetInteraction%20Actor _asbp_vacuum_player 0))

(event Custom|Close%20Door%20A
  ;[1 1 1] Close Door A
  (Utilities|FlowControl|Sequence
    (:then_0
      (Components|MoveComponentTo (Variables|Default|GetLDoorA) "180.000000,0.000000,150.000000" "90.000000,0.000000,0.000000" false false 0.3 false))
    (:then_1
      (Components|MoveComponentTo (Variables|Default|GetRDoorA) "180.000000,0.000000,150.000000" "90.000000,0.000000,0.000000" false false 0.2 false))
    (:then_2
      (Audio|PlaySoundatLocation "/Game/EatUpAll/SoundEffects/Ambient/close_door_01.close_door_01" (Transformation|GetWorldLocation (Variables|Default|GetDoorFrameA)) "0, 0, 0" 1.0 1.0 0.0 "/Game/EatUpAll/SoundEffects/SlimeSoundAttenuation.SlimeSoundAttenuation" 0 0 0)
      (Collision|SetCollisionResponsetoChannel (Variables|Default|GetDoorFrameA) "ECC_Pawn" "ECR_Block"))))

(event Custom|CloseDoorB
  ;[1 1 1] Close Door B
  (Utilities|FlowControl|Sequence
    (:then_0
      (Components|MoveComponentTo (Variables|Default|GetLDoorB) "180.000000,0.000000,150.000000" "90.000000,0.000000,0.000000" false false 0.3 false))
    (:then_1
      (Components|MoveComponentTo (Variables|Default|GetRDoorB) "180.000000,0.000000,150.000000" "90.000000,0.000000,0.000000" false false 0.2 false))
    (:then_2
      (Audio|PlaySoundatLocation "/Game/EatUpAll/SoundEffects/Ambient/close_door_01.close_door_01" (Transformation|GetWorldLocation (Variables|Default|GetDoorFrameB)) "0, 0, 0" 1.0 1.0 0.0 "/Game/EatUpAll/SoundEffects/SlimeSoundAttenuation.SlimeSoundAttenuation" 0 0 0)
      (Collision|SetCollisionResponsetoChannel (Variables|Default|GetDoorFrameB) "ECC_Pawn" "ECR_Block"))))

(event Custom|Open%20Door%20A
  ;[1 1 1] Open Door A
  (Utilities|FlowControl|Sequence
    (:then_0
      (Components|MoveComponentTo (Variables|Default|GetLDoorA) "180.000000,0.000000,70.000000" "90.000000,0.000000,0.000000" false false 0.3 false))
    (:then_1
      (Components|MoveComponentTo (Variables|Default|GetRDoorA) "180.000000,0.000000,220.000000" "90.000000,0.000000,0.000000" false false 0.2 false))
    (:then_2
      (Audio|PlaySoundatLocation "/Game/EatUpAll/SoundEffects/Ambient/open_door_01.open_door_01" (Transformation|GetWorldLocation (Variables|Default|GetDoorFrameA)) "0, 0, 0" 1.0 1.0 0.0 "/Game/EatUpAll/SoundEffects/SlimeSoundAttenuation.SlimeSoundAttenuation" 0 0 0)
      (Collision|SetCollisionResponsetoChannel (Variables|Default|GetDoorFrameA) "ECC_Pawn" "ECR_Ignore"))))

(event Custom|OpenDoorB
  ;[1 1 1] Open Door B
  (Utilities|FlowControl|Sequence
    (:then_0
      (Components|MoveComponentTo (Variables|Default|GetLDoorB) "180.000000,0.000000,70.000000" "90.000000,0.000000,0.000000" false false 0.3 false))
    (:then_1
      (Components|MoveComponentTo (Variables|Default|GetRDoorB) "180.000000,0.000000,220.000000" "90.000000,0.000000,0.000000" false false 0.2 false))
    (:then_2
      (Audio|PlaySoundatLocation "/Game/EatUpAll/SoundEffects/Ambient/open_door_01.open_door_01" (Transformation|GetWorldLocation (Variables|Default|GetDoorFrameB)) "0, 0, 0" 1.0 1.0 0.0 "/Game/EatUpAll/SoundEffects/SlimeSoundAttenuation.SlimeSoundAttenuation" 0 0 0)
      (Collision|SetCollisionResponsetoChannel (Variables|Default|GetRDoorB) "ECC_Pawn" "ECR_Ignore"))))

(event Custom|Door%20Action
  (if (Variables|Default|GetbAIsOpen)
    (Utilities|FlowControl|Sequence
      (:then_0
        (CallFunction|OpenDoorA))
      (:then_1
        (CallFunction|CloseDoorB))
      (:then_2
        (Variables|Default|SetbAIsOpen false)))
    (else
      (Utilities|FlowControl|Sequence
        (:then_0
          (CallFunction|OpenDoorB))
        (:then_1
          (CallFunction|CloseDoorA))
        (:then_2
          (Variables|Default|SetbAIsOpen true))))))

(event EventBeginPlay
  (CallFunction|DoorAction))

(event EventInteraction
  (params (Causer :type BP%20Vacuum%20Player%20Object%20Reference))
  (CallFunction|DoorAction))

(fn ConstructionScript
  (Transformation|SetRelativeLocation (Variables|Default|GetDoorFrameA) (Math|Vector|MakeVector 0.0 (.y (Variables|Default|GetDoorALocation)) 0.0) false false)
  (Transformation|SetRelativeLocation (Variables|Default|GetDoorFrameB) (Math|Vector|MakeVector 0.0 (.y (Variables|Default|GetDoorBLocation)) 0.0) false false)
  (Transformation|SetRelativeLocation (Variables|Default|GetDoorLock) (Variables|Default|GetDoorLockLocation) false false))