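; Two-panel sliding door that opens for a falling vacuum player and can be broken by red slimes.
; Entering the trigger box while falling slides both panels apart with collision ignored and plays a sound.
; Leaving the box slides them shut, restores blocking and plays a closing sound.
; A red slime hitting either panel spawns that side's door-piece actor at the impact and destroys the panel component.
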(event OnComponentHit(LDoor)
  (params (HitComponent :type Primitive%20Component%20Object%20Reference) (OtherActor :type Actor%20Object%20Reference) (OtherComp :type Primitive%20Component%20Object%20Reference) (NormalImpulse :type Vector :default "0, 0, 0") (Hit :type Hit%20Result%20Structure%20%28by%20ref%29))
  (bind _ldoor (Variables|Default|GetLDoor))
  (bind _asbp_slime_char_for_new_move_single (Utilities|Casting|CastToBP_SlimeCharForNewMove_Single OtherActor))
  (if (Variables|/Game/EatUpAll/Blueprints/Slime/BP_SlimeCharForNewMove_Single.BP_SlimeCharForNewMove_Single_C|GetbIsRedSlime _asbp_slime_char_for_new_move_single)
    (Game|SpawnActorfromClass "/Game/EatUpAll/Blueprints/Objects/BP_DoorPieceL.BP_DoorPieceL_C" (Math|Transform|MakeTransform (.Location (Collision|BreakHitResult Hit)) (.rotation (Transformation|GetWorldTransform _ldoor)) "1.000000,1.000000,1.000000") "Undefined" "MultiplyWithRoot" 0 0)
    (Components|DestroyComponent _ldoor)))

(event OnComponentBeginOverlap(Box)
  (params (OverlappedComponent :type Primitive%20Component%20Object%20Reference) (OtherActor :type Actor%20Object%20Reference) (OtherComp :type Primitive%20Component%20Object%20Reference) (OtherBodyIndex :type Integer) (bFromSweep :type Boolean) (SweepResult :type Hit%20Result%20Structure%20%28by%20ref%29))
  (bind _asbp_vacuum_player (Utilities|Casting|CastToBP_VacuumPlayer OtherActor))
  (if (AI|Components|NavMovement|IsFalling (Variables|/Script/Engine.Character|GetCharacterMovement _asbp_vacuum_player))
    (CallFunction|OpenLDoor)
    (CallFunction|OpenRdoor)
    (Audio|PlaySoundatLocation "/Game/EatUpAll/SoundEffects/Ambient/open_door_01.open_door_01" (Transformation|GetWorldLocation (Variables|Default|GetBox)) "0, 0, 0" 1.0 1.0 0.0 "/Game/EatUpAll/SoundEffects/SlimeSoundAttenuation.SlimeSoundAttenuation" 0 0 0)
    (Variables|Default|SetbIsOpen true)))

(event OnComponentEndOverlap(Box)
  (params (OverlappedComponent :type Primitive%20Component%20Object%20Reference) (OtherActor :type Actor%20Object%20Reference) (OtherComp :type Primitive%20Component%20Object%20Reference) (OtherBodyIndex :type Integer))
  (if (Variables|Default|GetbIsOpen)
    (CallFunction|CloseRDoor)
    (CallFunction|CloseLDoor)
    (Audio|PlaySoundatLocation "/Game/EatUpAll/SoundEffects/Ambient/close_door_01.close_door_01" (Transformation|GetWorldLocation (Variables|Default|GetBox)) "0, 0, 0" 1.0 1.0 0.0 "/Game/EatUpAll/SoundEffects/SlimeSoundAttenuation.SlimeSoundAttenuation" 0 0 0)
    (Variables|Default|SetbIsOpen false)))

(event OnComponentHit(RDoor)
  (params (HitComponent :type Primitive%20Component%20Object%20Reference) (OtherActor :type Actor%20Object%20Reference) (OtherComp :type Primitive%20Component%20Object%20Reference) (NormalImpulse :type Vector :default "0, 0, 0") (Hit :type Hit%20Result%20Structure%20%28by%20ref%29))
  (bind _rdoor (Variables|Default|GetRDoor))
  (bind _asbp_slime_char_for_new_move_single (Utilities|Casting|CastToBP_SlimeCharForNewMove_Single OtherActor))
  (if (Variables|/Game/EatUpAll/Blueprints/Slime/BP_SlimeCharForNewMove_Single.BP_SlimeCharForNewMove_Single_C|GetbIsRedSlime _asbp_slime_char_for_new_move_single)
    (Game|SpawnActorfromClass "/Game/EatUpAll/Blueprints/Objects/BP_DoorPieceR.BP_DoorPieceR_C" (Math|Transform|MakeTransform (.Location (Collision|BreakHitResult Hit)) (.rotation (Transformation|GetWorldTransform _rdoor)) "1.000000,1.000000,1.000000") "Undefined" "MultiplyWithRoot" 0 0)
    (Components|DestroyComponent _rdoor)))

(event Custom|Close%20RDoor
  (Collision|SetCollisionResponsetoAllChannels (Variables|Default|GetRDoor) "ECR_Block")
  (Components|MoveComponentTo (Variables|Default|GetRDoor) "0.000000,-295.000000,770.000000" "0.000000,0.000000,90.000000" false false 0.2 false))

(event Custom|Open%20LDoor
  (Collision|SetCollisionResponsetoAllChannels (Variables|Default|GetLDoor) "ECR_Ignore")
  (Components|MoveComponentTo (Variables|Default|GetLDoor) "200.000000,-295.000000,770.000000" "0.000000,0.000000,90.000000" false false 0.2 false))

(event Custom|Open%20Rdoor
  (Collision|SetCollisionResponsetoAllChannels (Variables|Default|GetRDoor) "ECR_Ignore")
  (Components|MoveComponentTo (Variables|Default|GetRDoor) "-200.000000,-295.000000,770.000000" "0.000000,0.000000,90.000000" false false 0.2 false))

(event Custom|Close%20LDoor
  (Collision|SetCollisionResponsetoAllChannels (Variables|Default|GetLDoor) "ECR_Block")
  (Components|MoveComponentTo (Variables|Default|GetLDoor) "0.000000,-295.000000,770.000000" "0.000000,0.000000,90.000000" false false 0.2 false))

(event EventBeginPlay)

(event Collision|EventActorBeginOverlap
  (params (OtherActor :type Actor%20Object%20Reference)))

(event EventTick
  (params (DeltaSeconds :type Float%20%28single-precision%29)))

(fn ConstructionScript)