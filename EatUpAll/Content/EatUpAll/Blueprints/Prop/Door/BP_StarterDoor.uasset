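; BP_StarterDoor is a sliding double door that stays locked through a start countdown, then serves BP_VacuumPlayer.
; The player controller's Phase0 event starts a 30-second text timer that reddens each second via a DelayedForloop, then unlocks the door.
; Entrance overlaps slide both panels with MoveComponentTo until Phase2 opens the door and disables that trigger logic.
; A separate sensor shows a "No" indicator to slimes, which end overlap never hides.
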(event OnComponentBeginOverlap(Enterence)
  (params (OverlappedComponent :type Primitive%20Component%20Object%20Reference) (OtherActor :type Actor%20Object%20Reference) (OtherComp :type Primitive%20Component%20Object%20Reference) (OtherBodyIndex :type Integer) (bFromSweep :type Boolean) (SweepResult :type Hit%20Result%20Structure%20%28by%20ref%29))
  (if (not (Variables|Default|GetbIsPhaze2))
    (if (Variables|Default|GetbIsUnlock)
      (Utilities|Casting|CastToBP_VacuumPlayer OtherActor)
      (if (not (Variables|Default|GetbIsOpen))
        (CallFunction|OpenDoor)))))

(event OnComponentEndOverlap(Enterence)
  (params (OverlappedComponent :type Primitive%20Component%20Object%20Reference) (OtherActor :type Actor%20Object%20Reference) (OtherComp :type Primitive%20Component%20Object%20Reference) (OtherBodyIndex :type Integer))
  (if (not (Variables|Default|GetbIsPhaze2))
    (if (Variables|Default|GetbIsUnlock)
      (Utilities|Casting|CastToBP_VacuumPlayer OtherActor)
      (if (Variables|Default|GetbIsOpen)
        (CallFunction|CloseDoor)))))

(event OnComponentBeginOverlap(SlimeSenser)
  (params (OverlappedComponent :type Primitive%20Component%20Object%20Reference) (OtherActor :type Actor%20Object%20Reference) (OtherComp :type Primitive%20Component%20Object%20Reference) (OtherBodyIndex :type Integer) (bFromSweep :type Boolean) (SweepResult :type Hit%20Result%20Structure%20%28by%20ref%29))
  ;[1 0.1491 0.8648] Detect Slime And Say that cannot Pass(should work on Client Only)
  (Utilities|Casting|CastToBP_SlimeCharForNewMove_Single OtherActor)
  (Rendering|SetVisibility (Variables|Default|GetNo) true false))

(event OnComponentEndOverlap(SlimeSenser)
  (params (OverlappedComponent :type Primitive%20Component%20Object%20Reference) (OtherActor :type Actor%20Object%20Reference) (OtherComp :type Primitive%20Component%20Object%20Reference) (OtherBodyIndex :type Integer))
  ;[1 0.1491 0.8648] Detect Slime And Say that cannot Pass(should work on Client Only)
  (Utilities|Casting|CastToBP_SlimeCharForNewMove_Single OtherActor)
  (Rendering|SetVisibility (Variables|Default|GetNo) true false))

(event Custom|SetPhaze2Bool
  ;[0.9941 0.1976 1] Detect event for phaze 2
  (Variables|Default|SetbIsPhaze2 true)
  (CallFunction|OpenDoor))

(event Custom|Close%20Door
  ;[1 1 1] Close Door
  (Utilities|FlowControl|Sequence
    (:then_0
      (Components|MoveComponentTo (Variables|Default|GetLDoor) "0.000000,-205.000000,0.000000" "0, 0, 0" false false 0.2 false))
    (:then_1
      (Components|MoveComponentTo (Variables|Default|GetRDoor) "0.000000,-205.000000,0.000000" "0, 0, 0" false false 0.3 false))
    (:then_2
      (Audio|PlaySoundatLocation "/Game/EatUpAll/SoundEffects/Ambient/open_door_01.open_door_01" (Transformation|GetWorldLocation (Variables|Default|GetDoorFrame)) "0, 0, 0" 1.0 1.0 0.0 "/Game/EatUpAll/SoundEffects/SlimeSoundAttenuation.SlimeSoundAttenuation" 0 0 0)
      (Collision|SetCollisionResponsetoChannel (Variables|Default|GetDoorFrame) "ECC_Pawn" "ECR_Ignore")
      (Variables|Default|SetbIsOpen false))))

(event Custom|Make%20Ready%20Timer
  (CallFunction|MakeReadyTimeronClient))

(event Custom|Make%20Ready%20Timer%20on%20Client
  (bind _timer (Variables|Default|GetTimer))
  (bind _timer_2 (Variables|Default|GetTimer))
  (bind _textrendercolor (Variables|/Script/Engine.TextRenderComponent|GetTextRenderColor _timer_2))
  (bind _output_get (Variables|Default|SetTime 30))
  (Rendering|Components|TextRender|SetText _timer (Utilities|Text|ToText(Integer) _output_get))
  (Rendering|SetVisibility _timer true false)
  (bind _result (Math|Integer|DecrementInt (Variables|Default|GetTime))
    (:%20%20
      (bind _index (Utilities|DelayedForloop 0 _result 1.0)
        (:loop%20Body
          (Rendering|Components|TextRender|SetText _timer_2 (Utilities|Text|ToText(Integer) (- (Variables|Default|GetTime) _index)))
          (Rendering|Components|TextRender|SetTextRenderColor _timer_2 (Math|Color|MakeColor (- (.b _textrendercolor) 8) (- (.g _textrendercolor) 8) (.r _textrendercolor) 0)))
        (:Completed
          (Rendering|SetVisibility (Variables|Default|GetTimer) false false)
          (Variables|Default|SetbIsUnlock true)
          (CallFunction|CloseDoor))))))

(event Custom|Open%20Door
  ;[1 1 1] Open Door
  (Utilities|FlowControl|Sequence
    (:then_0
      (Components|MoveComponentTo (Variables|Default|GetLDoor) "100.000000,-205.000000,0.000000" "0, 0, 0" false false 0.2 false))
    (:then_1
      (Components|MoveComponentTo (Variables|Default|GetRDoor) "-100.000000,-205.000000,0.000000" "0, 0, 0" false false 0.3 false))
    (:then_2
      (Audio|PlaySoundatLocation "/Game/EatUpAll/SoundEffects/Ambient/close_door_01.close_door_01" (Transformation|GetWorldLocation (Variables|Default|GetDoorFrame)) "0, 0, 0" 1.0 1.0 0.0 "/Game/EatUpAll/SoundEffects/SlimeSoundAttenuation.SlimeSoundAttenuation" 0 0 0)
      (Collision|SetCollisionResponsetoChannel (Variables|Default|GetDoorFrame) "ECC_Pawn" "ECR_Ignore")
      (Variables|Default|SetbIsOpen true))))

(event EventBeginPlay
  (bind _returnvalue (Game|GetPlayerController 0))
  (bind _asbp_player_contorller (Utilities|Casting|CastToBP_PlayerContorller _returnvalue))
  (EventDispatchers|BindEventtoPhase0 _asbp_player_contorller (delegate Custom|Make%20Ready%20Timer))
  (EventDispatchers|BindEventtoPhase2 _asbp_player_contorller (delegate Custom|SetPhaze2Bool)))

(fn ConstructionScript)