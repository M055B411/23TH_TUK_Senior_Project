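; Networked sliding double door that opens and closes automatically on box overlap until the linked Tower's emergency event locks it down.
; Lockdown shows two indicator planes and shuts the door; BP_Doorlock calls UnlockOpenDoor to hide them and reopen it.
; While locked, a red slime hitting either panel destroys it and spawns a debris piece.
; The server triggers open/close events that move panels, play sound and toggle the frame's Pawn collision.
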(event OnComponentHit(LDoor)
  (params (HitComponent :type Primitive%20Component%20Object%20Reference) (OtherActor :type Actor%20Object%20Reference) (OtherComp :type Primitive%20Component%20Object%20Reference) (NormalImpulse :type Vector :default "0, 0, 0") (Hit :type Hit%20Result%20Structure%20%28by%20ref%29))
  (bind _ldoor (Variables|Default|GetLDoor))
  (if (Variables|Default|GetbIsLocked)
    (bind _asbp_slime_char_for_new_move_single (Utilities|Casting|CastToBP_SlimeCharForNewMove_Single OtherActor))
    (if (Variables|/Game/EatUpAll/Blueprints/Slime/BP_SlimeCharForNewMove_Single.BP_SlimeCharForNewMove_Single_C|GetbIsRedSlime _asbp_slime_char_for_new_move_single)
      (CallFunction|SpawnPieceonServer _ldoor (.Location (Collision|BreakHitResult Hit)))
      (Components|DestroyComponent _ldoor)
      (Rendering|SetVisibility (Variables|Default|GetPlane) false false))))

(event OnComponentHit(RDoor)
  (params (HitComponent :type Primitive%20Component%20Object%20Reference) (OtherActor :type Actor%20Object%20Reference) (OtherComp :type Primitive%20Component%20Object%20Reference) (NormalImpulse :type Vector :default "0, 0, 0") (Hit :type Hit%20Result%20Structure%20%28by%20ref%29))
  (bind _rdoor (Variables|Default|GetRDoor))
  (if (Variables|Default|GetbIsLocked)
    (bind _asbp_slime_char_for_new_move_single (Utilities|Casting|CastToBP_SlimeCharForNewMove_Single OtherActor))
    (if (Variables|/Game/EatUpAll/Blueprints/Slime/BP_SlimeCharForNewMove_Single.BP_SlimeCharForNewMove_Single_C|GetbIsRedSlime _asbp_slime_char_for_new_move_single)
      (CallFunction|SpawnPieceonServer _rdoor (.Location (Collision|BreakHitResult Hit)))
      (Components|DestroyComponent _rdoor)
      (Rendering|SetVisibility (Variables|Default|GetPlane) false false))))

(event OnComponentBeginOverlap(Box)
  (params (OverlappedComponent :type Primitive%20Component%20Object%20Reference) (OtherActor :type Actor%20Object%20Reference) (OtherComp :type Primitive%20Component%20Object%20Reference) (OtherBodyIndex :type Integer) (bFromSweep :type Boolean) (SweepResult :type Hit%20Result%20Structure%20%28by%20ref%29))
  (if (not (Variables|Default|GetbIsLocked))
    (if (not (Variables|Default|GetbIsOpen))
      (if (Networking|IsServer)
        (CallFunction|OpenDooronMulti)
        (Variables|Default|SetbIsOpen true)))))

(event OnComponentEndOverlap(Box)
  (params (OverlappedComponent :type Primitive%20Component%20Object%20Reference) (OtherActor :type Actor%20Object%20Reference) (OtherComp :type Primitive%20Component%20Object%20Reference) (OtherBodyIndex :type Integer))
  (if (not (Variables|Default|GetbIsLocked))
    (if (Variables|Default|GetbIsOpen)
      (if (Networking|IsServer)
        (CallFunction|CloseDooronMulti)
        (Variables|Default|SetbIsOpen false)))))

(event Custom|UnlockOpenDoor
  ;[1 1 1] Call by BP_Doorlock
  (Rendering|SetVisibility (Variables|Default|GetPlane) false false)
  (Default|CallUpdateDoorlock)
  (if (Networking|IsServer)
    (CallFunction|OpenDooronMulti)))

(event Custom|CloseDoor%20on%20Multi
  ;[1 1 1] Close Door
  (Utilities|FlowControl|Sequence
    (:then_0
      (Components|MoveComponentTo (Variables|Default|GetRDoor) "207.500000,0.000000,160.000000" "90.000000,0.000000,0.000000" false false 0.3 false))
    (:then_1
      (Components|MoveComponentTo (Variables|Default|GetLDoor) "207.500000,0.000000,160.000000" "90.000000,0.000000,0.000000" false false 0.2 false))
    (:then_2
      (Audio|PlaySoundatLocation "/Game/EatUpAll/SoundEffects/Ambient/close_door_01.close_door_01" (Transformation|GetWorldLocation (Variables|Default|GetDoorFrame)) "0, 0, 0" 1.0 1.0 0.0 "/Game/EatUpAll/SoundEffects/SlimeSoundAttenuation.SlimeSoundAttenuation" 0 0 0)
      (Collision|SetCollisionResponsetoChannel (Variables|Default|GetDoorFrame) "ECC_Pawn" "ECR_Block"))))

(event Custom|SpawnPiece%20on%20Server
  (params (Door :type Scene%20Component%20Object%20Reference) (HitLoc :type Vector))
  (Game|SpawnActorfromClass "/Game/EatUpAll/Blueprints/Objects/BP_DoorPieceR.BP_DoorPieceR_C" (Math|Transform|MakeTransform HitLoc (.rotation (Transformation|GetWorldTransform Door)) "1.000000,1.000000,1.000000") "Undefined" "MultiplyWithRoot" 0 0))

(event Custom|OpenDoor%20on%20Multi
  ;[1 1 1] Open Door
  (Utilities|FlowControl|Sequence
    (:then_0
      (Components|MoveComponentTo (Variables|Default|GetRDoor) "207.500000,0.000000,0.000000" "90.000000,0.000000,0.000000" false false 0.3 false))
    (:then_1
      (Components|MoveComponentTo (Variables|Default|GetLDoor) "207.500000,0.000000,300.000000" "90.000000,0.000000,0.000000" false false 0.2 false))
    (:then_2
      (Audio|PlaySoundatLocation "/Game/EatUpAll/SoundEffects/Ambient/open_door_01.open_door_01" (Transformation|GetWorldLocation (Variables|Default|GetDoorFrame)) "0, 0, 0" 1.0 1.0 0.0 "/Game/EatUpAll/SoundEffects/SlimeSoundAttenuation.SlimeSoundAttenuation" 0 0 0)
      (Collision|SetCollisionResponsetoChannel (Variables|Default|GetDoorFrame) "ECC_Pawn" "ECR_Ignore"))))

(event Custom|LockDown
  (Rendering|SetVisibility (Variables|Default|GetPlane) true false)
  (Variables|Default|SetbIsLocked true)
  (if (Networking|IsServer)
    (CallFunction|CloseDooronMulti)))

(event EventBeginPlay
  (bind _tower (Variables|Default|GetTower))
  (Utilities|IsValid _tower
    (:Is%20Valid
      (EventDispatchers|BindEventtoOnEmergency _tower (delegate Custom|LockDown)))))

(fn ConstructionScript)