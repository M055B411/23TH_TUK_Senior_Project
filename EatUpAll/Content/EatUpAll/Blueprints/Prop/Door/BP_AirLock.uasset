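; Airlock prop with two door frames, toggled when the vacuum player interacts with it.
; Box1 overlap registers or clears it as the player's interaction actor, and the construction script positions frames and lock from variables.
; Interaction branches on AIsOpen to pair opening and closing events that slide panels, play sound and switch Pawn blocking.
; The door B events duplicate door A's, moving A's components and flag, so door B never moves.
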(event OnComponentBeginOverlap(Box1)
  (params (OverlappedComponent :type Primitive%20Component%20Object%20Reference) (OtherActor :type Actor%20Object%20Reference) (OtherComp :type Primitive%20Component%20Object%20Reference) (OtherBodyIndex :type Integer) (bFromSweep :type Boolean) (SweepResult :type Hit%20Result%20Structure%20%28by%20ref%29))
  (bind _asbp_vacuum_player (Utilities|Casting|CastToBP_VacuumPlayer OtherActor))
  (Variables|/Game/EatUpAll/Blueprints/Player/BP_VacuumPlayer.BP_VacuumPlayer_C|SetbIsCanInteraction _asbp_vacuum_player true)
  (Variables|/Game/EatUpAll/Blueprints/Player/BP_VacuumPlayer.BP_VacuumPlayer_C|SetInteraction%20Actor _asbp_vacuum_player self))

(event OnComponentEndOverlap(Box1)
  (params (OverlappedComponent :type Primitive%20Component%20Object%20Reference) (OtherActor :type Actor%20Object%20Reference) (OtherComp :type Primitive%20Component%20Object%20Reference) (OtherBodyIndex :type Integer))
  (bind _asbp_vacuum_player (Utilities|Casting|CastToBP_VacuumPlayer OtherActor))
  (Variables|/Game/EatUpAll/Blueprints/Player/BP_VacuumPlayer.BP_VacuumPlayer_C|SetbIsCanInteraction _asbp_vacuum_player false)
  (Variables|/Game/EatUpAll/Blueprints/Player/BP_VacuumPlayer.BP_VacuumPlayer_C|SetInteraction%20Actor _asbp_vacuum_player 0))

(event Custom|Close%20Door%20A
  ;[1 1 1] Close Door
  (Utilities|FlowControl|Sequence
    (:then_0
      (Components|MoveComponentTo (Variables|Default|GetLDoorA) "207.500000,0.000000,160.000000" "90.000000,0.000000,0.000000" false false 0.3 false))
    (:then_1
      (Components|MoveComponentTo (Variables|Default|GetRDoorA) "207.500000,0.000000,160.000000" "90.000000,0.000000,0.000000" false false 0.2 false))
    (:then_2
      (Audio|PlaySoundatLocation "/Game/EatUpAll/SoundEffects/Ambient/close_door_01.close_door_01" (Transformation|GetWorldLocation (Variables|Default|GetDoorFrameA)) "0, 0, 0" 1.0 1.0 0.0 "/Game/EatUpAll/SoundEffects/SlimeSoundAttenuation.SlimeSoundAttenuation" 0 0 0)
      (Collision|SetCollisionResponsetoChannel (Variables|Default|GetDoorFrameA) "ECC_Pawn" "ECR_Block")
      (Variables|Default|SetbAIsOpen false))))

(event Custom|CloseDoorB
  ;[1 1 1] Close Door
  (Utilities|FlowControl|Sequence
    (:then_0
      (Components|MoveComponentTo (Variables|Default|GetLDoorA) "207.500000,0.000000,160.000000" "90.000000,0.000000,0.000000" false false 0.3 false))
    (:then_1
      (Components|MoveComponentTo (Variables|Default|GetRDoorA) "207.500000,0.000000,160.000000" "90.000000,0.000000,0.000000" false false 0.2 false))
    (:then_2
      (Audio|PlaySoundatLocation "/Game/EatUpAll/SoundEffects/Ambient/close_door_01.close_door_01" (Transformation|GetWorldLocation (Variables|Default|GetDoorFrameA)) "0, 0, 0" 1.0 1.0 0.0 "/Game/EatUpAll/SoundEffects/SlimeSoundAttenuation.SlimeSoundAttenuation" 0 0 0)
      (Collision|SetCollisionResponsetoChannel (Variables|Default|GetDoorFrameA) "ECC_Pawn" "ECR_Block")
      (Variables|Default|SetbAIsOpen false))))

(event Custom|Open%20Door%20A
  ;[1 1 1] Open Door
  (Utilities|FlowControl|Sequence
    (:then_0
      (Components|MoveComponentTo (Variables|Default|GetLDoorA) "207.500000,0.000000,290.000000" "90.000000,0.000000,0.000000" false false 0.3 false))
    (:then_1
      (Components|MoveComponentTo (Variables|Default|GetRDoorA) "207.500000,0.000000,0.000000" "90.000000,0.000000,0.000000" false false 0.2 false))
    (:then_2
      (Audio|PlaySoundatLocation "/Game/EatUpAll/SoundEffects/Ambient/open_door_01.open_door_01" (Transformation|GetWorldLocation (Variables|Default|GetDoorFrameA)) "0, 0, 0" 1.0 1.0 0.0 "/Game/EatUpAll/SoundEffects/SlimeSoundAttenuation.SlimeSoundAttenuation" 0 0 0)
      (Collision|SetCollisionResponsetoChannel (Variables|Default|GetDoorFrameA) "ECC_Pawn" "ECR_Ignore")
      (Variables|Default|SetbAIsOpen true))))

(event Custom|OpenDoorB
  ;[1 1 1] Open Door
  (Utilities|FlowControl|Sequence
    (:then_0
      (Components|MoveComponentTo (Variables|Default|GetLDoorA) "207.500000,0.000000,290.000000" "90.000000,0.000000,0.000000" false false 0.3 false))
    (:then_1
      (Components|MoveComponentTo (Variables|Default|GetRDoorA) "207.500000,0.000000,0.000000" "90.000000,0.000000,0.000000" false false 0.2 false))
    (:then_2
      (Audio|PlaySoundatLocation "/Game/EatUpAll/SoundEffects/Ambient/open_door_01.open_door_01" (Transformation|GetWorldLocation (Variables|Default|GetDoorFrameA)) "0, 0, 0" 1.0 1.0 0.0 "/Game/EatUpAll/SoundEffects/SlimeSoundAttenuation.SlimeSoundAttenuation" 0 0 0)
      (Collision|SetCollisionResponsetoChannel (Variables|Default|GetDoorFrameA) "ECC_Pawn" "ECR_Ignore")
      (Variables|Default|SetbAIsOpen true))))

(event EventBeginPlay)

(event EventInteraction
  (params (Causer :type BP%20Vacuum%20Player%20Object%20Reference))
  (if (Variables|Default|GetbAIsOpen)
    (Utilities|FlowControl|Sequence
      (:then_0
        (CallFunction|OpenDoorB))
      (:then_1
        (CallFunction|CloseDoorA)))
    (else
      (Utilities|FlowControl|Sequence
        (:then_0
          (CallFunction|OpenDoorA))
        (:then_1
          (CallFunction|CloseDoorB))))))

(event EventTick
  (params (DeltaSeconds :type Float%20%28single-precision%29)))

(event Collision|EventActorBeginOverlap
  (params (OtherActor :type Actor%20Object%20Reference)))

(fn ConstructionScript
  (Transformation|SetRelativeLocation (Variables|Default|GetDoorFrameA) (Math|Vector|MakeVector 0.0 (.y (Variables|Default|GetDoorALocation)) 0.0) false false)
  (Transformation|SetRelativeLocation (Variables|Default|GetDoorFrameB) (Math|Vector|MakeVector 0.0 (.y (Variables|Default|GetDoorBLocation)) 0.0) false false)
  (Transformation|SetRelativeLocation (Variables|Default|GetDoorLock) (Variables|Default|GetDoorLockLocation) false false))