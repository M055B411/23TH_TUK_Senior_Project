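; Automatic hall door that opens when something overlaps its trigger Box and closes when an overlap ends.
; Overlap events check an IsOpen flag, then call OpenDoor or CloseDoor.
; These move the two panels in opposite directions along local Z with MoveComponentTo, play a sound at the frame and toggle the flag.
; The frame's Pawn collision response switches to Ignore when open and Block when closed.
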(event OnComponentBeginOverlap(Box)
  (params (OverlappedComponent :type Primitive%20Component%20Object%20Reference) (OtherActor :type Actor%20Object%20Reference) (OtherComp :type Primitive%20Component%20Object%20Reference) (OtherBodyIndex :type Integer) (bFromSweep :type Boolean) (SweepResult :type Hit%20Result%20Structure%20%28by%20ref%29))
  (if (not (Variables|Default|GetbIsOpen))
    (CallFunction|OpenDoor)))

(event OnComponentEndOverlap(Box)
  (params (OverlappedComponent :type Primitive%20Component%20Object%20Reference) (OtherActor :type Actor%20Object%20Reference) (OtherComp :type Primitive%20Component%20Object%20Reference) (OtherBodyIndex :type Integer))
  (if (Variables|Default|GetbIsOpen)
    (CallFunction|CloseDoor)))

(event Custom|Close%20Door
  ;[1 1 1] Close Door
  (Utilities|FlowControl|Sequence
    (:then_0
      (Components|MoveComponentTo (Variables|Default|GetLDoor) "207.500000,0.000000,160.000000" "90.000000,0.000000,0.000000" false false 0.3 false))
    (:then_1
      (Components|MoveComponentTo (Variables|Default|GetRDoor) "207.500000,0.000000,160.000000" "90.000000,0.000000,0.000000" false false 0.2 false))
    (:then_2
      (Audio|PlaySoundatLocation "/Game/EatUpAll/SoundEffects/Ambient/close_door_01.close_door_01" (Transformation|GetWorldLocation (Variables|Default|GetDoorFrame)) "0, 0, 0" 1.0 1.0 0.0 "/Game/EatUpAll/SoundEffects/SlimeSoundAttenuation.SlimeSoundAttenuation" 0 0 0)
      (Collision|SetCollisionResponsetoChannel (Variables|Default|GetDoorFrame) "ECC_Pawn" "ECR_Block")
      (Variables|Default|SetbIsOpen false))))

(event Custom|Open%20Door
  ;[1 1 1] Open Door
  (Utilities|FlowControl|Sequence
    (:then_0
      (Components|MoveComponentTo (Variables|Default|GetLDoor) "207.500000,0.000000,290.000000" "90.000000,0.000000,0.000000" false false 0.3 false))
    (:then_1
      (Components|MoveComponentTo (Variables|Default|GetRDoor) "207.500000,0.000000,0.000000" "90.000000,0.000000,0.000000" false false 0.2 false))
    (:then_2
      (Audio|PlaySoundatLocation "/Game/EatUpAll/SoundEffects/Ambient/open_door_01.open_door_01" (Transformation|GetWorldLocation (Variables|Default|GetDoorFrame)) "0, 0, 0" 1.0 1.0 0.0 "/Game/EatUpAll/SoundEffects/SlimeSoundAttenuation.SlimeSoundAttenuation" 0 0 0)
      (Collision|SetCollisionResponsetoChannel (Variables|Default|GetDoorFrame) "ECC_Pawn" "ECR_Ignore")
      (Variables|Default|SetbIsOpen true))))

(fn ConstructionScript)