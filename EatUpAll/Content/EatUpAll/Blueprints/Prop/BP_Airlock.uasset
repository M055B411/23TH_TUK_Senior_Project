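; BP_Airlock is an interactable airlock prop that triggers a linked door for the vacuum player.
; Its Box overlap registers the airlock as the player's interaction actor, enables interaction and sets an interaction time, then clears all three on exit.
; The Interaction event calls DoorAction on the referenced Door if it is valid.
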(event OnComponentBeginOverlap(Box)
  (params (OverlappedComponent :type Primitive%20Component%20Object%20Reference) (OtherActor :type Actor%20Object%20Reference) (OtherComp :type Primitive%20Component%20Object%20Reference) (OtherBodyIndex :type Integer) (bFromSweep :type Boolean) (SweepResult :type Hit%20Result%20Structure%20%28by%20ref%29))
  (bind _asbp_vacuum_player (Utilities|Casting|CastToBP_VacuumPlayer OtherActor))
  (Default|UpdateCanIA _asbp_vacuum_player true)
  (Variables|/Game/EatUpAll/Blueprints/Player/BP_VacuumPlayer.BP_VacuumPlayer_C|SetIA%20Actor _asbp_vacuum_player self)
  (Variables|/Game/EatUpAll/Blueprints/Player/BP_VacuumPlayer.BP_VacuumPlayer_C|SetIA_TimeSet _asbp_vacuum_player 2.5e+02))

(event OnComponentEndOverlap(Box)
  (params (OverlappedComponent :type Primitive%20Component%20Object%20Reference) (OtherActor :type Actor%20Object%20Reference) (OtherComp :type Primitive%20Component%20Object%20Reference) (OtherBodyIndex :type Integer))
  (bind _asbp_vacuum_player (Utilities|Casting|CastToBP_VacuumPlayer OtherActor))
  (Default|UpdateCanIA _asbp_vacuum_player false)
  (Variables|/Game/EatUpAll/Blueprints/Player/BP_VacuumPlayer.BP_VacuumPlayer_C|SetIA%20Actor _asbp_vacuum_player 0)
  (Variables|/Game/EatUpAll/Blueprints/Player/BP_VacuumPlayer.BP_VacuumPlayer_C|SetIA_TimeSet _asbp_vacuum_player 0.0))

(event EventInteraction
  (params (Causer :type BP%20Vacuum%20Player%20Object%20Reference))
  (bind _door (Variables|Default|GetDoor))
  (Utilities|IsValid _door
    (:Is%20Valid
      (Default|DoorAction _door))))

(fn ConstructionScript)