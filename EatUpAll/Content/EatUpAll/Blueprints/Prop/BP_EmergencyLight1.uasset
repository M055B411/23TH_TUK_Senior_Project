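; BP_EmergencyLight1 is an emergency light prop that turns red when a linked Tower signals an emergency.
; On BeginPlay it creates a dynamic material instance on its mesh from a square hall light material.
; If the Tower reference is valid, it binds to the Tower's EmergencyON event and sets the glow parameter to bright white.
; The bound event switches that parameter to red, with no revert in this Blueprint.
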(event Custom|E_lighton
  (Rendering|Material|SetVectorParameterValue (Variables|Default|Getglow) "B5" "(R=10.000000,G=0.000000,B=0.000000,A=10.000000)" :!class /Script/Engine.MaterialInstanceDynamic))

(event EventBeginPlay
  (bind _tower (Variables|Default|GetTower))
  (bind _returnvalue (Rendering|Material|CreateDynamicMaterialInstance (Variables|Default|GetMeshe) 0 "/Game/EatUpAll/Blueprints/Prop/Light/met/MI_Hall_Light_Square_M_Inst.MI_Hall_Light_Square_M_Inst" "None" :!class /Script/Engine.PrimitiveComponent))
  (Variables|Default|Setglow _returnvalue)
  (Utilities|IsValid _tower
    (:Is%20Valid
      (EventDispatchers|BindEventtoEmergencyON _tower (delegate Custom|E_lighton))
      (Rendering|Material|SetVectorParameterValue (Variables|Default|Getglow) "B5" "(R=10.000000,G=10.000000,B=10.000000,A=10.000000)" :!class /Script/Engine.MaterialInstanceDynamic))))

(event Collision|EventActorBeginOverlap
  (params (OtherActor :type Actor%20Object%20Reference)))

(event EventTick
  (params (DeltaSeconds :type Float%20%28single-precision%29)))

(fn ConstructionScript)