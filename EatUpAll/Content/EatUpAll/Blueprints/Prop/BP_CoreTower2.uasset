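; BP_CoreTower2 is a core tower prop that stays active until all of its linked generators, up to four, are destroyed.
; At BeginPlay it binds to each valid generator's destroyed event and counts them.
; Each destruction deactivates that generator's Niagara arc effect and decrements the count.
; When the count reaches zero, the tower stops its audio and calls TowerOff.
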(event Custom|Arc_Off%20D
  (Components|Activation|Deactivate (Variables|Default|GetNiagara3))
  (CallFunction|GeneratorDownCheck))

(event Custom|Down
  (Audio|Components|Audio|Stop (Variables|Default|GetAudio))
  (Default|CallTowerOff))

(event Custom|Arc_Off%20A
  (Components|Activation|Deactivate (Variables|Default|GetNiagara))
  (CallFunction|GeneratorDownCheck))

(event Custom|Arc_Off%20B
  (Components|Activation|Deactivate (Variables|Default|GetNiagara1))
  (CallFunction|GeneratorDownCheck))

(event Custom|Arc_Off%20C
  (Components|Activation|Deactivate (Variables|Default|GetNiagara2))
  (CallFunction|GeneratorDownCheck))

(event Custom|Generator%20DownCheck
  (bind _count (Variables|Default|Getcount))
  (Math|Integer|DecrementInt _count
    (:%20%20
      (if (<= _count 0)
        (CallFunction|Down)))))

(event EventBeginPlay
  (bind _generator_a (Variables|Default|GetGenerator%20A))
  (bind _generator_b (Variables|Default|GetGenerator%20B))
  (bind _generator_c (Variables|Default|GetGenerator%20C))
  (bind _generator_d (Variables|Default|GetGenerator%20D))
  (Utilities|FlowControl|Sequence
    (:then_0
      (Utilities|IsValid _generator_a
        (:Is%20Valid
          (EventDispatchers|BindEventtoGeneratorDestroyed _generator_a (delegate Custom|Arc_Off%20A))
          (Math|Integer|IncrementInt (Variables|Default|Getcount)))))
    (:then_1
      (Utilities|IsValid _generator_b
        (:Is%20Valid
          (EventDispatchers|BindEventtoGeneratorDestroyed _generator_b (delegate Custom|Arc_Off%20B))
          (Math|Integer|IncrementInt (Variables|Default|Getcount)))))
    (:then_2
      (Utilities|IsValid _generator_c
        (:Is%20Valid
          (EventDispatchers|BindEventtoGeneratorDestroyed _generator_c (delegate Custom|Arc_Off%20C))
          (Math|Integer|IncrementInt (Variables|Default|Getcount)))))
    (:then_3
      (Utilities|IsValid _generator_d
        (:Is%20Valid
          (EventDispatchers|BindEventtoGeneratorDestroyed _generator_d (delegate Custom|Arc_Off%20D))
          (Math|Integer|IncrementInt (Variables|Default|Getcount)))))))

(fn ConstructionScript)