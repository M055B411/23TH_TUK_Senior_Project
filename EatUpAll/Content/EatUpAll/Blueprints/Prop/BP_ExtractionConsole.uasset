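; Extraction console prop that shows a lock image and enters emergency lockdown when its linked Tower is destroyed.
; On BeginPlay it creates a dynamic material on its Plane, sets the default lock texture and, if Tower is valid, binds EmergencyLockdown to that tower's destroyed event.
; EmergencyLockdown sets the ELock flag and swaps the displayed texture to a danger image.
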(event Custom|EmergencyLockdown
  (Variables|Default|SetELock true)
  (Rendering|Material|SetTextureParameterValue (Variables|Default|GetImage) "LockImage" "/Game/EatUpAll/Blueprints/Objects/NotVacuumable/danger_ncl1_1.danger_ncl1_1"))

(event EventBeginPlay
  (bind _tower (Variables|Default|GetTower))
  (bind _returnvalue (Rendering|Material|CreateDynamicMaterialInstance (Variables|Default|GetPlane) 0 "/Game/EatUpAll/Blueprints/Objects/NotVacuumable/MI_Lock.MI_Lock" "None" :!class /Script/Engine.PrimitiveComponent))
  (Variables|Default|SetImage _returnvalue)
  (Rendering|Material|SetTextureParameterValue (Variables|Default|GetImage) "LockImage" "/Game/EatUpAll/Blueprints/Objects/Meshes/Large/Bed/l_2021091601002193600186161.l_2021091601002193600186161")
  (Utilities|IsValid _tower
    (:Is%20Valid
      (EventDispatchers|BindEventtoTowerDestroyed _tower (delegate Custom|EmergencyLockdown)))))

(fn ConstructionScript)