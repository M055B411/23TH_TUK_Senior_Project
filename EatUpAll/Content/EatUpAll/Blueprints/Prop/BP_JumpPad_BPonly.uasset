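; Jump pad actor, implemented in Blueprint, that boosts a Character upward when it leaves the pad airborne.
; On begin overlap, it stores the Character's max jump height from its movement component.
; On end overlap, if the Character is falling, LaunchCharacter applies a vertical velocity scaled from that stored height.
; The height lives in a single variable, so the most recent Character to enter sets it.
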(event EventBeginPlay)

(event Collision|EventActorBeginOverlap
  (params (OtherActor :type Actor%20Object%20Reference))
  (bind _ascharacter (Utilities|Casting|CastToCharacter OtherActor))
  (Variables|Default|SetOrignal%20Height (Class|CharacterMovementComponent|GetMaxJumpHeight (Variables|/Script/Engine.Character|GetCharacterMovement _ascharacter))))

(event EventTick
  (params (DeltaSeconds :type Float%20%28single-precision%29)))

(event Collision|EventActorEndOverlap
  (params (OtherActor :type Actor%20Object%20Reference))
  (bind _ascharacter (Utilities|Casting|CastToCharacter OtherActor))
  (if (AI|Components|NavMovement|IsFalling (Variables|/Script/Engine.Character|GetCharacterMovement _ascharacter))
    (Character|LaunchCharacter _ascharacter (Math|Vector|MakeVector 0.0 0.0 (* (Variables|Default|GetOrignal%20Height) 25.0)) false false)))

(fn ConstructionScript)