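; 3D printer prop that, when activated, spits out a random batch of objects with start, making and end sounds.
; A vacuum player inside its box can interact with it, and a slime character hitting the printer triggers the same logic.
; A Printing flag blocks re-entry while a delayed loop spawns a few random picks from SpawnActors at the sphere.
; Spawning passes through SpawnObjectOnServer to SpawnObjectOnClient.
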(event OnComponentHit(Printer)
  (params (HitComponent :type Primitive%20Component%20Object%20Reference) (OtherActor :type Actor%20Object%20Reference) (OtherComp :type Primitive%20Component%20Object%20Reference) (NormalImpulse :type Vector :default "0, 0, 0") (Hit :type Hit%20Result%20Structure%20%28by%20ref%29))
  (bind _returnvalue (Transformation|GetActorLocation))
  (Utilities|Casting|CastToBP_SlimeCharForNewMove_Single OtherActor)
  (if (not (Variables|Default|GetPrinting))
    (Variables|Default|SetPrinting true)
    (Audio|PlaySoundatLocation (Variables|Default|GetStartSound) _returnvalue "0, 0, 0" 1.0 1.0 0.0 0 0 0 0)
    (Utilities|FlowControl|Delay 1.0)
    (Utilities|DelayedForloop 0 (Math|Random|RandomIntegerinRange 3 6) (Variables|Default|GetDelay)
      (:loop%20Body
        (Audio|PlaySoundatLocation (Variables|Default|GetMakingSound) _returnvalue "0, 0, 0" 1.0 1.0 0.0 0 0 0 0)
        (CallFunction|SpawnObjectonServer))
      (:Completed
        (Variables|Default|SetPrinting false)
        (Audio|PlaySoundatLocation (Variables|Default|GetEndSound) _returnvalue "0, 0, 0" 1.0 1.0 0.0 0 0 0 0)))
    (else
      (Development|PrintString "Hello"))))

(event OnComponentBeginOverlap(Box)
  (params (OverlappedComponent :type Primitive%20Component%20Object%20Reference) (OtherActor :type Actor%20Object%20Reference) (OtherComp :type Primitive%20Component%20Object%20Reference) (OtherBodyIndex :type Integer) (bFromSweep :type Boolean) (SweepResult :type Hit%20Result%20Structure%20%28by%20ref%29))
  (bind _asbp_vacuum_player (Utilities|Casting|CastToBP_VacuumPlayer OtherActor))
  (Variables|/Game/EatUpAll/Blueprints/Player/BP_VacuumPlayer.BP_VacuumPlayer_C|SetbCanInteraction _asbp_vacuum_player true)
  (Variables|/Game/EatUpAll/Blueprints/Player/BP_VacuumPlayer.BP_VacuumPlayer_C|SetInteraction%20Actor _asbp_vacuum_player self))

(event OnComponentEndOverlap(Box)
  (params (OverlappedComponent :type Primitive%20Component%20Object%20Reference) (OtherActor :type Actor%20Object%20Reference) (OtherComp :type Primitive%20Component%20Object%20Reference) (OtherBodyIndex :type Integer))
  (bind _asbp_vacuum_player (Utilities|Casting|CastToBP_VacuumPlayer OtherActor))
  (Variables|/Game/EatUpAll/Blueprints/Player/BP_VacuumPlayer.BP_VacuumPlayer_C|SetbCanInteraction _asbp_vacuum_player false)
  (Variables|/Game/EatUpAll/Blueprints/Player/BP_VacuumPlayer.BP_VacuumPlayer_C|SetInteraction%20Actor _asbp_vacuum_player 0))

(event Custom|Spawn%20Object%20on%20Server
  (CallFunction|SpawnObjectonClient))

(event Custom|Spawn%20Object%20on%20Client
  (bind _spawnactors (Variables|Default|GetSpawnActors))
  (Game|SpawnActorfromClass (Utilities|Array|Get(acopy) _spawnactors (Math|Random|RandomIntegerinRange 0 (- (Utilities|Array|Length _spawnactors) 1))) (Math|Transform|MakeTransform (Transformation|GetWorldLocation (Variables|Default|GetSphere)) "0, 0, 0" "1.000000,1.000000,1.000000") "AdjustIfPossibleButAlwaysSpawn" "MultiplyWithRoot" 0 0))

(event EventInteraction
  (params (Causer :type BP%20Vacuum%20Player%20Object%20Reference))
  (bind _returnvalue (Transformation|GetActorLocation))
  (if (not (Variables|Default|GetPrinting))
    (Variables|Default|SetPrinting true)
    (Audio|PlaySoundatLocation (Variables|Default|GetStartSound) _returnvalue "0, 0, 0" 1.0 1.0 0.0 0 0 0 0)
    (Utilities|FlowControl|Delay 1.0)
    (Utilities|DelayedForloop 0 (Math|Random|RandomIntegerinRange 3 6) (Variables|Default|GetDelay)
      (:loop%20Body
        (Audio|PlaySoundatLocation (Variables|Default|GetMakingSound) _returnvalue "0, 0, 0" 1.0 1.0 0.0 0 0 0 0)
        (CallFunction|SpawnObjectonServer))
      (:Completed
        (Variables|Default|SetPrinting false)
        (Audio|PlaySoundatLocation (Variables|Default|GetEndSound) _returnvalue "0, 0, 0" 1.0 1.0 0.0 0 0 0 0)))
    (else
      (Development|PrintString "Hello"))))

(fn ConstructionScript)