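; BP_Siren is a siren light prop that switches on when its referenced Tower signals an emergency.
; On BeginPlay it creates a dynamic material for its sphere and, if Tower is valid, binds to the EmergencyON dispatcher and zeroes the glow.
; The event activates the rotating movement, raises both spotlights' intensity and boosts the material's glow.
; No logic here switches it back off.
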(event Custom|E_lighton
  (Components|Activation|Activate (Variables|Default|GetRotatingMovement) false)
  (Rendering|Components|Light|SetIntensity (Variables|Default|GetSpotLight2) 8e+03)
  (Rendering|Material|SetScalarParameterValue (Variables|Default|Getglow) "Glow" 3e+03 :!class /Script/Engine.MaterialInstanceDynamic))

(event EventBeginPlay
  (bind _tower (Variables|Default|GetTower))
  (bind _returnvalue (Rendering|Material|CreateDynamicMaterialInstance (Variables|Default|GetSphere) 0 0 "None" :!class /Script/Engine.PrimitiveComponent))
  (Variables|Default|Setglow _returnvalue)
  (Utilities|IsValid _tower
    (:Is%20Valid
      (EventDispatchers|BindEventtoEmergencyON _tower (delegate Custom|E_lighton))
      (Rendering|Material|SetScalarParameterValue (Variables|Default|Getglow) "Glow" 0.0 :!class /Script/Engine.MaterialInstanceDynamic))))

(event Collision|EventActorBeginOverlap
  (params (OtherActor :type Actor%20Object%20Reference)))

(event EventTick
  (params (DeltaSeconds :type Float%20%28single-precision%29)))

(fn ConstructionScript)