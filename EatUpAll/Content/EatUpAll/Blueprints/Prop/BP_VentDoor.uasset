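; BP_VentDoor is a vent door prop that lets the slime through only while its HP is below a fixed threshold.
; If it starts enterable, it listens to the game instance's slime HP change event and updates IsEnter through its own dispatcher.
; That flag switches the mesh's custom trace channel between Overlap and Block, with four Niagara effects active while blocked.
; Doors starting non-enterable stay blocked; the box overlap does nothing.
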(event OnComponentBeginOverlap(Box)
  (params (OverlappedComponent :type Primitive%20Component%20Object%20Reference) (OtherActor :type Actor%20Object%20Reference) (OtherComp :type Primitive%20Component%20Object%20Reference) (OtherBodyIndex :type Integer) (bFromSweep :type Boolean) (SweepResult :type Hit%20Result%20Structure%20%28by%20ref%29)))

(event Custom|Check%20IsEnter
  (bind _staticmesh (Variables|Default|GetStaticMesh))
  (if (Variables|Default|GetbIsEnter)
    (Collision|SetCollisionResponsetoChannel _staticmesh "ECC_GameTraceChannel1" "ECR_Overlap")
    (Components|Activation|SetActive (Variables|Default|GetNiagara1) false false)
    (else
      (Collision|SetCollisionResponsetoChannel _staticmesh "ECC_GameTraceChannel1" "ECR_Block")
      (Components|Activation|SetActive (Variables|Default|GetNiagara1) true false))))

(event Custom|Set%20IsEnter
  (params (MainSlimeHP :type Float%20%28double-precision%29))
  (if (>= MainSlimeHP 36.0)
    (Variables|Default|SetbIsEnter false)
    (Default|CallSelfEnterCheck)
    (else
      (Variables|Default|SetbIsEnter true)
      (Default|CallSelfEnterCheck))))

(event EventBeginPlay
  (if (Variables|Default|GetbIsEnter)
    (EventDispatchers|BindEventtoChangeSlimeHP (.AsBP%20Eat%20Up%20All%20Game%20Instance (Utilities|Casting|CastToBP_EatUpAllGameInstance (Game|GetGameInstance))) (delegate Custom|Set%20IsEnter))
    (EventDispatchers|BindEventtoSelfEnterCheck (delegate Custom|Check%20IsEnter))
    (else
      (Collision|SetCollisionResponsetoChannel (Variables|Default|GetStaticMesh) "ECC_GameTraceChannel1" "ECR_Block")
      (Components|Activation|SetActive (Variables|Default|GetNiagara1) true false))))

(fn ConstructionScript)