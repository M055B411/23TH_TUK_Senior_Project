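; BP_CoreTower is a destructible core tower prop that a sufficiently strong slime character damages by hitting it.
; On mesh hit, a slime with HP at or above Standard is launched away from the tower, the EmergencyON dispatcher fires and DamageCount drops.
; When DamageCount runs out, the tower spawns BP_PhaseTwoCore at its location, unbinds EmergencyON listeners and destroys itself.
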(event OnComponentHit(Mesh)
  (params (HitComponent :type Primitive%20Component%20Object%20Reference) (OtherActor :type Actor%20Object%20Reference) (OtherComp :type Primitive%20Component%20Object%20Reference) (NormalImpulse :type Vector :default "0, 0, 0") (Hit :type Hit%20Result%20Structure%20%28by%20ref%29))
  (bind _asbp_slime_char_for_new_move_done (Utilities|Casting|CastToBP_SlimeCharForNewMove_Done OtherActor))
  (Development|PrintString "Slime Hit")
  (if (>= (Variables|/Game/EatUpAll/Blueprints/Slime/BP_SlimeCharForNewMove_Done.BP_SlimeCharForNewMove_Done_C|GetHP _asbp_slime_char_for_new_move_done) (Variables|Default|GetStandard))
    (Character|LaunchCharacter _asbp_slime_char_for_new_move_done (* (Math|Vector|Normalize (- (Transformation|GetActorLocation OtherActor) (Transformation|GetActorLocation))) 1e+03) false false)
    (Default|CallEmergencyON)
    (bind _result (Math|Float|DecrementFloat (Variables|Default|GetDamageCount))
      (:%20%20
        (if (<= _result 0.0)
          (Game|SpawnActorfromClass "/Game/EatUpAll/Blueprints/Objects/BP_PhaseTwoCore.BP_PhaseTwoCore_C" (Math|Transform|MakeTransform (Transformation|GetActorLocation)) "Undefined" "MultiplyWithRoot" 0 0)
          (EventDispatchers|UnbindallEventsfromEmergencyON)
          (Actor|DestroyActor))))))

(event EventBeginPlay)

(event Collision|EventActorBeginOverlap
  (params (OtherActor :type Actor%20Object%20Reference)))

(event EventTick
  (params (DeltaSeconds :type Float%20%28single-precision%29)))

(fn ConstructionScript)