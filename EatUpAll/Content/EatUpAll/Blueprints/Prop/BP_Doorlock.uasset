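; BP_Doorlock is a door lock prop that shows its state on a screen material and broadcasts door locked and unlocked events.
; Tick reads IsUnlocked to swap the LockImage texture on a dynamic material, with two DoOnce gates resetting each other so each event fires once per change.
; If a Tower is set, its destruction triggers an emergency lockdown that shows a danger image and stops further state updates.
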(event Custom|EmergencyLockdown
  (Variables|Default|SetELock true)
  (Rendering|Material|SetTextureParameterValue (Variables|Default|GetImage) "LockImage" "/Game/EatUpAll/Blueprints/Objects/NotVacuumable/danger_ncl1_1.danger_ncl1_1"))

(event EventBeginPlay
  (bind _tower (Variables|Default|GetTower))
  (bind _returnvalue (Rendering|Material|CreateDynamicMaterialInstance (Variables|Default|GetStaticMesh) 1 0 "None" :!class /Script/Engine.PrimitiveComponent))
  (Variables|Default|SetImage _returnvalue)
  (Rendering|Material|SetTextureParameterValue (Variables|Default|GetImage) "LockImage" "/Game/EatUpAll/Blueprints/Objects/NotVacuumable/lock_off.lock_off")
  (Utilities|IsValid _tower
    (:Is%20Valid
      (EventDispatchers|BindEventtoTowerDestroyed _tower (delegate Custom|EmergencyLockdown)))))

(event Collision|EventActorBeginOverlap
  (params (OtherActor :type Actor%20Object%20Reference)))

(event EventTick
  (params (DeltaSeconds :type Float%20%28single-precision%29))
  (if (not (Variables|Default|GetELock))
    (if (Variables|Default|GetIsUnlocked)
      (Rendering|Material|SetTextureParameterValue (Variables|Default|GetImage) "LockImage" "/Game/EatUpAll/Blueprints/Objects/NotVacuumable/lock_off.lock_off")
      (Utilities|FlowControl|DoOnce false :!label _label
        (:Completed
          (Default|CallDoorUnlocked)
          (goto _label_2 Reset)))
      (else
        (Rendering|Material|SetTextureParameterValue (Variables|Default|GetImage) "LockImage" "/Game/EatUpAll/Blueprints/Objects/NotVacuumable/lock_blue.lock_blue")
        (Utilities|FlowControl|DoOnce false :!label _label_2
          (:Completed
            (Default|CallDoorLocked)
            (goto _label Reset)))))))

(fn ConstructionScript)