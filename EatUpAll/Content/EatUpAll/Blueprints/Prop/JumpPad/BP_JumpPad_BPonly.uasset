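; Jump pad prop that boosts BP_VacuumPlayer upward when the player leaves its Box trigger in midair.
; Entering the box caches the player's max jump height from the CharacterMovement component.
; Exiting while falling (airborne) calls LaunchCharacter with a multiple of that height as Z velocity, so walking off the pad gives no boost.
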(event OnComponentBeginOverlap(Box)
  (params (OverlappedComponent :type Primitive%20Component%20Object%20Reference) (OtherActor :type Actor%20Object%20Reference) (OtherComp :type Primitive%20Component%20Object%20Reference) (OtherBodyIndex :type Integer) (bFromSweep :type Boolean) (SweepResult :type Hit%20Result%20Structure%20%28by%20ref%29))
  (bind _asbp_vacuum_player (Utilities|Casting|CastToBP_VacuumPlayer OtherActor))
  (Variables|Default|SetOrignal%20Height (Class|CharacterMovementComponent|GetMaxJumpHeight (Variables|/Script/Engine.Character|GetCharacterMovement _asbp_vacuum_player))))

(event OnComponentEndOverlap(Box)
  (params (OverlappedComponent :type Primitive%20Component%20Object%20Reference) (OtherActor :type Actor%20Object%20Reference) (OtherComp :type Primitive%20Component%20Object%20Reference) (OtherBodyIndex :type Integer))
  (bind _asbp_vacuum_player (Utilities|Casting|CastToBP_VacuumPlayer OtherActor))
  (if (AI|Components|NavMovement|IsFalling (Variables|/Script/Engine.Character|GetCharacterMovement _asbp_vacuum_player))
    (Character|LaunchCharacter _asbp_vacuum_player (Math|Vector|MakeVector 0.0 0.0 (* (Variables|Default|GetOrignal%20Height) 16.0)) false false)))

(fn ConstructionScript)