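; BP_Hunter1Player is the first hunter's player character, a child class that fills in Hunter 1-specific behavior.
; Overridden events register hunter ID 1, notify the party on death and write suck and skill ammo to BP_EatUpAllGameInstance.
; Multi-suffixed events toggle BP_VacuumGun particles for client-server sync.
; When dead, SpectatorCamera input switches the view to a living BP_Hunter2Player, and Tick drives that hunter's first-person camera rotation from this character's third-person camera.
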(event Custom|Initalize%20Loc
  (Transformation|SetActorTransform (Variables|Default|GetNewVar)))

(event EventEnableAllParticleonMulti
  ;[1 1 1] Particle Sync Client-Server
  (bind _asbp_vacuum_gun (Utilities|Casting|CastToBP_VacuumGun (Variables|Default|GetVacuumGun)))
  (Default|EnableAllEffect _asbp_vacuum_gun))

(event EventDisactiveAllParticleonMuti
  ;[1 1 1] Particle Sync Client-Server
  (bind _asbp_vacuum_gun (Utilities|Casting|CastToBP_VacuumGun (Variables|Default|GetVacuumGun)))
  (Default|DisableAllEffect _asbp_vacuum_gun))

(event EventUpdateSkillAmmoonMulti
  (params (Ammo :type Float%20%28double-precision%29))
  ;[0.5876 1 0.3953] Event Override
  (Variables|/Game/EatUpAll/HUD/BP_EatUpAllGameInstance.BP_EatUpAllGameInstance_C|SetHunter1SkillAmmo (.AsBP%20Eat%20Up%20All%20Game%20Instance (Utilities|Casting|CastToBP_EatUpAllGameInstance (Game|GetGameInstance))) Ammo))

(event EventHunterIDonOwn
  (bind _returnvalue (Game|GetGameInstance))
  (bind _asbp_eat_up_all_game_instance (Utilities|Casting|CastToBP_EatUpAllGameInstance _returnvalue))
  ;[0 1 0.6655] When Possessed by player, 'Call Register Hunter' to Sync Widget
  (bind _output_get (Variables|/Game/EatUpAll/HUD/BP_EatUpAllGameInstance.BP_EatUpAllGameInstance_C|SetHunterID _asbp_eat_up_all_game_instance 1))
  (Default|CallRegisterHunter _asbp_eat_up_all_game_instance _output_get))

(event EventUpdateSuckAmmoonMulti
  (params (Ammo :type Float%20%28double-precision%29))
  ;[0.5876 1 0.3953] Event Override
  (Variables|/Game/EatUpAll/HUD/BP_EatUpAllGameInstance.BP_EatUpAllGameInstance_C|SetHunter1SuckAmmo (.AsBP%20Eat%20Up%20All%20Game%20Instance (Utilities|Casting|CastToBP_EatUpAllGameInstance (Game|GetGameInstance))) Ammo))

(event EventTick
  (params (DeltaSeconds :type Float%20%28single-precision%29))
  (bind _thirdpersoncameracomponent (Variables|Default|GetThirdPersonCameraComponent))
  (bind _returnvalue (Transformation|GetWorldRotation _thirdpersoncameracomponent))
  ;[1 0.09861 0.6047] When this actor is dead and 'X' key is Pressed,  Player can use other actor's camera
  (|CallParentFunction DeltaSeconds)
  (if (Variables|Default|GetbIsSpectator)
    (bind _returnvalue_2 (Actor|GetActorOfClass "/Game/EatUpAll/Blueprints/Player/BP_Hunter2Player.BP_Hunter2Player_C"))
    (Utilities|IsValid _returnvalue_2
      (:Is%20Valid
        (Transformation|SetWorldRotation (Variables|/Script/EatUpAll.VacuumPlayer|GetFirstPersonCameraComponent _returnvalue_2) (Math|Rotator|MakeRotator (.roll _returnvalue) (.pitch _returnvalue) (.yaw _returnvalue)) false false)))))

(event EventBeginPlay
  (|CallParentFunction)
  (EventDispatchers|BindEventtoDebugInitializeLoc (.AsBP%20Player%20Contorller (Utilities|Casting|CastToBP_PlayerContorller (Game|GetPlayerController 0))) (delegate Custom|Initalize%20Loc)))

(event Collision|EventActorBeginOverlap
  (params (OtherActor :type Actor%20Object%20Reference))
  (|CallParentFunction OtherActor) ; This node is disabled and will not be called.\nDrag off pins to build functionality.
)

(event EventEnableSuckParticleonMulti
  ;[1 1 1] Particle Sync Client-Server
  (bind _asbp_vacuum_gun (Utilities|Casting|CastToBP_VacuumGun (Variables|Default|GetVacuumGun)))
  (Default|EnableSuckEffect _asbp_vacuum_gun))

(event EventPossessed
  (params (NewController :type Controller%20Object%20Reference))
  ;[0 1 0.6655] When Possessed by player, 'Call Register Hunter' to Sync Widget
  (|CallParentFunction NewController))

(event EventIsDeath
  ;[1 0.4688 0.504] If this actor is damaged to Slime, actor is Die
  (|CallParentFunction)
  (Default|CallNotifytoParty (.AsBP%20Eat%20Up%20All%20Game%20Instance (Utilities|Casting|CastToBP_EatUpAllGameInstance (Game|GetGameInstance))) false true))

(event EventInitializeonMulti
  ;[0 1 0.6655] When Possessed by player, 'Call Register Hunter' to Sync Widget
  (|CallParentFunction)
  (bind _output_get (Variables|Default|SetSuckEnerge (Variables|Default|GetSuckEnerge_Max)))
  (Variables|/Game/EatUpAll/HUD/BP_EatUpAllGameInstance.BP_EatUpAllGameInstance_C|SetHunter1SuckAmmo (.AsBP%20Eat%20Up%20All%20Game%20Instance (Utilities|Casting|CastToBP_EatUpAllGameInstance (Game|GetGameInstance))) _output_get))

(event Input|ActionEvents|InputActionSpectatorCamera
  (params (Key :type Key%20Structure :default "None"))
  ;[1 0.09861 0.6047] When this actor is dead and 'X' key is Pressed,  Player can use other actor's camera
  (:Pressed
    (if (Variables|Default|GetbIsDead)
      (bind _returnvalue (Actor|GetActorOfClass "/Game/EatUpAll/Blueprints/Player/BP_Hunter2Player.BP_Hunter2Player_C"))
      (Utilities|IsValid _returnvalue
        (:Is%20Valid
          (if (not (Variables|/Game/EatUpAll/Blueprints/Player/BP_VacuumPlayer.BP_VacuumPlayer_C|GetbIsDead _returnvalue))
            (Default|ActiveVacuumgunPos _returnvalue)
            (Game|Player|SetViewTargetwithBlend (Game|GetPlayerController 0) _returnvalue 0.0 "VTBlend_Linear" 0.0 false)
            (Variables|Default|SetbIsSpectator true)
            (bind _asbp_eat_up_all_game_instance (Utilities|Casting|CastToBP_EatUpAllGameInstance (Game|GetGameInstance)))
            (Variables|/Game/EatUpAll/HUD/BP_EatUpAllGameInstance.BP_EatUpAllGameInstance_C|SetbIsSpectator _asbp_eat_up_all_game_instance true)))))))

(fn ConstructionScript
  (|CallParentFunction))