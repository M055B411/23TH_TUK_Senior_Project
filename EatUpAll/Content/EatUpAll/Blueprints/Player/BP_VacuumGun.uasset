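; Vacuum gun actor for the player that hosts and toggles its suction and aurora visual effects.
; On BeginPlay it moves the three effect components (NSSuck, NSAuroraSelf, NSAurora) to the muzzle location as a relative offset.
; Paired enable and disable functions switch a "self" set (suck plus self aurora) separately from an "other" set (aurora only).
; It has no Tick, overlap or suction logic of its own.
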(event EventBeginPlay
  (bind _returnvalue (Class|VacuumGun|GetMuzzleLocation))
  (Transformation|SetRelativeLocation (Variables|Default|GetNS_Aurora_self) _returnvalue false false))

(event Collision|EventActorBeginOverlap
  (params (OtherActor :type Actor%20Object%20Reference)))

(event EventTick
  (params (DeltaSeconds :type Float%20%28single-precision%29)))

(fn ConstructionScript)

(fn EnableSelfEffect
  (Components|Activation|SetActive (Variables|Default|GetNS_Suck) true false)
  (Components|Activation|SetActive (Variables|Default|GetNS_Aurora_self) true false))

(fn DisableSelfEffect
  (Components|Activation|SetActive (Variables|Default|GetNS_Suck) false false)
  (Components|Activation|SetActive (Variables|Default|GetNS_Aurora_self) false false))

(fn EnableOtherEffect
  (Components|Activation|SetActive (Variables|Default|GetNS_Aurora) true false))

(fn DisableOtherEffect
  (Components|Activation|SetActive (Variables|Default|GetNS_Aurora) false false))