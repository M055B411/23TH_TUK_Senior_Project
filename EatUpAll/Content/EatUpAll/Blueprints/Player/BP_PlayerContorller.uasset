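; Player controller for EatUpAll that lets the player switch possession between hunter and slime pawns via key presses.
; On BeginPlay it resets the hunter index and adds a development widget to the viewport.
; One Ctrl key shortcut cycles through all hunter actors, using a recursive function that skips the currently controlled pawn.
; The other possesses the first slime character found in the level.
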(event EventBeginPlay
  (Variables|Default|SetHUNTERNUM 0)
  (bind _returnvalue (UserInterface|CreateWidget "/Game/EatUpAll/Blueprints/Player/BP_WidgetForDevelop.BP_WidgetForDevelop_C"))
  (bind _output_get (Variables|Default|SetDevelopWidget _returnvalue))
  (UserInterface|Viewport|AddtoViewport _output_get 0))

(event EventTick
  (params (DeltaSeconds :type Float%20%28single-precision%29)))

(event Input|KeyboardEvents|Ctrl2
  (params (Key :type Key%20Structure :default "None"))
  (:Pressed
    (bind _outactors (Actor|GetAllActorsOfClass "/Game/EatUpAll/Blueprints/Slime/BP_SlimeCharacter.BP_SlimeCharacter_C"))
    (Pawn|Possess (Utilities|Array|Get(acopy) _outactors))))

(event Input|KeyboardEvents|Ctrl1
  (params (Key :type Key%20Structure :default "None"))
  (:Pressed
    (bind _outactors (Actor|GetAllActorsOfClass "/Game/EatUpAll/Blueprints/Player/BP_HunterPlayer.BP_HunterPlayer_C"))
    (CallFunction|ChangeHunterPawn _outactors)))

(fn ConstructionScript)

(fn ChangeHunterPawn
  (params (Array :type Array%20of%20BP%20Hunter%20Player%20Object%20References))
  (LocalVariables|SetHunterArray Array)
  (if (== (Utilities|Array|Get(acopy) Array (Variables|Default|GetHUNTERNUM)) (Pawn|GetControlledPawn))
    (Variables|Default|SetHUNTERNUM (Math|Integer|%(Integer) (+ (Variables|Default|GetHUNTERNUM) 1) (Utilities|Array|Length (LocalVariables|GetHunterArray))))
    (CallFunction|ChangeHunterPawn (LocalVariables|GetHunterArray))
    (else
      (Pawn|Possess (Utilities|Array|Get(acopy) Array (Variables|Default|GetHUNTERNUM))))))