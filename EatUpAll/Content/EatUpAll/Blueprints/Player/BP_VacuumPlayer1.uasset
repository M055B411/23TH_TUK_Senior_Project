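; Hunter player character that wields a vacuum gun to erase paint, with a HUD, death effects and a card-gated door-lock toggle.
; Holding left mouse winds up, then drains suck energy on Tick, locking out at empty until fully recharged.
; Camera sphere traces send hit UVs to actors for render-target erasing or debug painting.
; Right mouse launches a projectile; server/client event pairs relay equipping, HUD, drawing and particles, while server events set walk speed.
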(event OnAudioFinished(AudioCleanerInitiate)
  (Variables|Default|SetbIsIniSoundPlaying false))

(event Custom|Create%20WBP_Hunter%20on%20Client
  ;[1 1 1] Crosshair, Vacuum Stamina Widget and Gun Equip
  (bind _returnvalue (UserInterface|CreateWidget "/Game/EatUpAll/HUD/WBP_Hunter.WBP_Hunter_C"))
  (bind _output_get (Variables|Default|SetWBP_Hunter _returnvalue))
  (UserInterface|Viewport|AddtoPlayerScreen _output_get)
  (Utilities|IsValid _output_get
    (:Is%20Valid
      (bind _output_get_2 (Variables|Default|SetSuck%20Energe (Variables|Default|GetSuck%20Max%20Energe)))
      (Variables|/Game/EatUpAll/HUD/WBP_Hunter.WBP_Hunter_C|SetHunter%20Energe (Variables|Default|GetWBP_Hunter) _output_get_2))))

(event Custom|Create%20WBP_Hunter%20on%20Server
  ;[1 1 1] Crosshair, Vacuum Stamina Widget and Gun Equip
  (CallFunction|CreateWBPHunteronClient))

(event Custom|Equip%20Gun%20on%20Server
  ;[1 1 1] Crosshair, Vacuum Stamina Widget and Gun Equip
  (CallFunction|EquipGunonClient))

(event Custom|Active%20Vacuumgun%20pos
  (Transformation|DetachFromActor (Variables|Default|GetVacuumGun) "KeepRelative" "KeepRelative" "KeepRelative")
  (Transformation|DetachFromComponent (Variables|Default|GetMesh1P) "KeepRelative" "KeepRelative" "KeepRelative" true))

(event Custom|OnDestroyed_Event
  (params (DestroyedActor :type Actor%20Object%20Reference))
  ;[1 1 1] When Hunter is Unpossessed, Self Destroy
  (EventDispatchers|BindEventtoOnDestroyed (delegate Custom|OnDestroyed_Event))
  (Development|PrintString "HunterDestroy" false true "(R=0.000000,G=0.660000,B=1.000000,A=1.000000)" 1e+01))

(event Custom|EnableAllParticle%20on%20Server
  ;[1 1 1] Particle Sync Client-Server
  (CallFunction|EnableAllParticleonClient))

(event Custom|DisactiveAllParticle%20on%20Server
  ;[1 1 1] Particle Sync Client-Server
  (CallFunction|DisactiveAllParticleonClient))

(event Custom|RightSkill%20on%20Server
  (bind _returnvalue (Class|VacuumGun|GetMuzzleLocation (Variables|Default|GetVacuumGun)))
  (bind _returnvalue_2 (Game|SpawnActorfromClass "/Game/EatUpAll/Blueprints/Player/BP_H1Projectile.BP_H1Projectile_C" (Math|Transform|MakeTransform _returnvalue "0, 0, 0" "0.300000,0.300000,0.300000") "AlwaysSpawn" "MultiplyWithRoot" 0 0))
  (Physics|AddImpulse (Variables|/Game/EatUpAll/Blueprints/Player/BP_H1Projectile.BP_H1Projectile_C|GetStaticMesh _returnvalue_2) (* (Math|Vector|Normalize (- (Transformation|GetActorLocation _returnvalue_2) (Transformation|GetActorLocation))) 1e+03) "None" true))

(event Custom|SlowWalkSpeed%20on%20Server
  (Variables|/Script/Engine.CharacterMovementComponent|SetMaxWalkSpeed (Variables|Character|GetCharacterMovement) 3e+02))

(event Custom|EnableSuckParticle%20on%20Server
  ;[1 1 1] Particle Sync Client-Server
  (CallFunction|EnableSuckParticleonClient))

(event Custom|DisactiveAllParticle%20on%20Client
  ;[1 1 1] Particle Sync Client-Server
)

(event Custom|Paint%20Draw%20RT%20on%20Client
  ;[1 1 1] Paint Action Sync Client-Server
  (CallFunction|PaintDrawRT))

(event Custom|Erase%20Draw%20RT%20on%20Client
  ;[1 1 1] Paint Action Sync Client-Server
  (CallFunction|EraseDrawRT))

(event Custom|EnableSuckParticle%20on%20Client
  ;[1 1 1] Particle Sync Client-Server
)

(event Custom|Equip%20Gun%20on%20Client
  ;[1 1 1] Crosshair, Vacuum Stamina Widget and Gun Equip
  (Utilities|IsValid (Variables|Default|GetVacuumGun) :!label _label
    (:Is%20Valid
      (Actor|DestroyActor)
      (goto _label))
    (:Is%20Not%20Valid
      (Class|VacuumPlayer|EquipVacuumGun))))

(event Custom|Erase%20Draw%20RT%20on%20Server
  ;[1 1 1] Paint Action Sync Client-Server
  (CallFunction|EraseDrawRT))

(event Custom|EnableAllParticle%20on%20Client
  ;[1 1 1] Particle Sync Client-Server
)

(event Custom|Paint%20Draw%20RT%20on%20Server
  ;[1 1 1] Paint Action Sync Client-Server
  (CallFunction|PaintDrawRT))

(event Custom|IsDead
  ;[1 1 1] When colliding with a slime, the hunter is stunned.
  (if (Variables|Default|GetbIsStun)
    (Physics|SetSimulatePhysics (Variables|Character|GetMesh) true)
    (else
      (Physics|SetSimulatePhysics (Variables|Default|GetCapsuleComponent) false))))

(event Custom|FastWalkSpeed%20on%20Server
  (Variables|/Script/Engine.CharacterMovementComponent|SetMaxWalkSpeed (Variables|Character|GetCharacterMovement) 7e+02))

(event EventDestroyed
  (bind _vacuumgun (Variables|Default|GetVacuumGun))
  (bind _wbp_hunter (Variables|Default|GetWBP_Hunter))
  ;[1 1 1] When the Hunter is destroyed, the attached weapon and Widget are also destroyed.
  (Utilities|IsValid _vacuumgun
    (:Is%20Valid
      (Transformation|DetachFromActor _vacuumgun "KeepRelative" "KeepRelative" "KeepRelative")
      (Utilities|IsValid _wbp_hunter
        (:Is%20Valid
          (Widget|RemovefromParent _wbp_hunter)
          (Variables|Default|SetbIsDead true)
          (Camera|PlayWorldCameraShake "/Game/EatUpAll/HUD/BP_DeathShake.BP_DeathShake_C" "0, 0, 0" 0.0 6e+03)
          (bind _returnvalue (UserInterface|CreateWidget "/Game/EatUpAll/HUD/WBP_HunterDie.WBP_HunterDie_C"))
          (UserInterface|Viewport|AddtoViewport _returnvalue 0)
          (bind _newtrack_0 (Timeline|Timeline PlayFromStart)
            (:Update
              (Transformation|SetWorldRotation (Variables|Character|GetMesh) (Math|Rotator|MakeRotator 0.0 _newtrack_0 0.0) false false))))))))

(event EventBeginPlay
  ;[1 1 1] When colliding with a slime, the hunter is stunned.
  (EventDispatchers|BindEventtoDeadHunter (delegate Custom|IsDead)))

(event EventTick
  (params (DeltaSeconds :type Float%20%28single-precision%29))
  (bind _wbp_hunter (Variables|Default|GetWBP_Hunter))
  (bind _wbp_hunter_2 (Variables|Default|GetWBP_Hunter))
  (bind _crosshairspread_limit (Variables|Default|GetCrosshairSpread%20limit))
  (Utilities|FlowControl|Sequence
    (:then_0
      (if (not (Variables|Default|GetbIsSuck%20Trigger))
        (bind _output_get (Variables|Default|SetSuck%20Energe (Math|Float|Clamp(Float) (+ (Variables|Default|GetSuck%20Energe) (* 1.0 0.6)) 0.0 (Variables|Default|GetSuck%20Max%20Energe))))
        (Utilities|IsValid _wbp_hunter_2
          (:Is%20Valid
            (bind _output_get_2 (Variables|/Game/EatUpAll/HUD/WBP_Hunter.WBP_Hunter_C|SetHunter%20Energe _wbp_hunter_2 _output_get))
            (if (== (Variables|Default|GetSuck%20Max%20Energe) _output_get_2)
              (if (Variables|Default|GetbIsSuck%20Reload)
                (CallFunction|CooldownVacuumgun)
                (Variables|Default|SetbIsSuck%20Reload false)
                (Variables|/Game/EatUpAll/HUD/WBP_Hunter.WBP_Hunter_C|SetbIsReloaded (Variables|Default|GetWBP_Hunter) false)))))
        (else
          (CallFunction|EraseDrawRTonServer)
          (bind _output_get_3 (Variables|Default|SetSuck%20Energe (Math|Float|Clamp(Float) (- (Variables|Default|GetSuck%20Energe) (* 1.0 1.4)) 0.0 (Variables|Default|GetSuck%20Max%20Energe))))
          (Utilities|IsValid _wbp_hunter
            (:Is%20Valid
              (bind _output_get_4 (Variables|/Game/EatUpAll/HUD/WBP_Hunter.WBP_Hunter_C|SetHunter%20Energe _wbp_hunter _output_get_3))
              (if (== _output_get_4 0.0)
                (CallFunction|EndVacuumgun)
                (Variables|Default|SetbIsSuck%20Reload true)
                (Variables|/Game/EatUpAll/HUD/WBP_Hunter.WBP_Hunter_C|SetbIsReloaded (Variables|Default|GetWBP_Hunter) true)
                (Variables|Default|SetbIsSuck%20Trigger false)
                (Audio|PlaySoundatLocation "/Game/EatUpAll/SoundEffects/Ambient/break_08.break_08" (Transformation|GetWorldLocation (Variables|Character|GetMesh)) "0, 0, 0" 1.0 1.0 0.0 0 0 0 0)))))))
    (:then_1
      (if (Variables|Default|GetbIsPaintInput)
        (CallFunction|PaintDrawRTonServer)))
    (:then_2
      (if (Variables|Default|GetbIsEraseInput)
        (Variables|/Game/EatUpAll/HUD/WBP_Hunter.WBP_Hunter_C|SetCrosshair%20Spread (Variables|Default|GetWBP_Hunter) (Math|Float|MapRangeClamped (Variables|Default|GetCrosshairSpread) 0.0 _crosshairspread_limit 7e+01 5.0))
        (if (== (Math|Float|Clamp(Float) (Variables|Default|GetCrosshairSpread) 0.0 _crosshairspread_limit) _crosshairspread_limit)
          (Variables|Default|SetCrosshairSpread 0.0))))))

(event EventPossessed
  (params (NewController :type Controller%20Object%20Reference))
  ;[1 1 1] When colliding with a slime, the hunter is stunned.
  ;[1 1 1] Crosshair, Vacuum Stamina Widget and Gun Equip
  (CallFunction|EquipGunonServer)
  (CallFunction|CreateWBPHunteronServer))

(event EventUnpossessed
  (params (OldController :type Controller%20Object%20Reference))
  ;[1 1 1] When Hunter is Unpossessed, Self Destroy
  (CallFunction|OnDestroyedEvent OldController))

(event Input|MouseEvents|DebugKeyCtrlRightMouseButton
  (params (Key :type Key%20Structure) (ActionValue :type Input%20Action%20Value%20Structure))
  ;[1 1 1] When Left Mouse Click, Trigger Erase Action
  (:Pressed
    (Variables|Default|SetbIsPaintInput true))
  (:Released
    (Variables|Default|SetbIsPaintInput false)))

(event Input|KeyboardEvents|1
  (params (Key :type Key%20Structure))
  (:Pressed
    (if (Variables|Default|GetbHasCard)
      (bind _outactors (Actor|GetAllActorsOfClass "/Game/EatUpAll/Blueprints/Prop/BP_Doorlock.BP_Doorlock_C"))
      (Utilities|FlowControl|FlipFlop
        (:A
          (Variables|/Game/EatUpAll/Blueprints/Prop/BP_Doorlock.BP_Doorlock_C|SetIsUnlocked (Utilities|Array|Get(acopy) _outactors) true))
        (:B
          (Variables|/Game/EatUpAll/Blueprints/Prop/BP_Doorlock.BP_Doorlock_C|SetIsUnlocked (Utilities|Array|Get(acopy) _outactors) false))))))

(event Input|KeyboardEvents|Slash
  (params (Key :type Key%20Structure))
  (bind _vacuumgun (Variables|Default|GetVacuumGun))
  (bind _wbp_hunter (Variables|Default|GetWBP_Hunter))
  ;[1 1 1] When the Hunter is destroyed, the attached weapon and Widget are also destroyed.
  (:Pressed
    (Utilities|IsValid _vacuumgun
      (:Is%20Valid
        (Transformation|DetachFromActor _vacuumgun "KeepRelative" "KeepRelative" "KeepRelative")
        (Utilities|IsValid _wbp_hunter
          (:Is%20Valid
            (Widget|RemovefromParent _wbp_hunter)
            (Variables|Default|SetbIsDead true)
            (Camera|PlayWorldCameraShake "/Game/EatUpAll/HUD/BP_DeathShake.BP_DeathShake_C" "0, 0, 0" 0.0 6e+03)
            (bind _returnvalue (UserInterface|CreateWidget "/Game/EatUpAll/HUD/WBP_HunterDie.WBP_HunterDie_C"))
            (UserInterface|Viewport|AddtoViewport _returnvalue 0)
            (bind _newtrack_0 (Timeline|Timeline PlayFromStart)
              (:Update
                (Transformation|SetWorldRotation (Variables|Character|GetMesh) (Math|Rotator|MakeRotator 0.0 _newtrack_0 0.0) false false)))))))))

(event Input|MouseEvents|LeftMouseButton
  (params (Key :type Key%20Structure))
  (bind _bissuck_reload (Variables|Default|GetbIsSuck%20Reload))
  ;[1 1 1] When Left Mouse Click, Trigger Erase Action
  (:Pressed
    (Variables|Default|SetbIsEraseInput true)
    (if (Variables|Default|GetbIsSuck%20Trigger) :!label _label
      (if (Variables|Default|GetbIsEraseInput)
        (CallFunction|RunVacuumgun)
        (else
          (Variables|Default|SetbIsSuck%20Trigger false)
          (Variables|Default|SetbIsIniSoundPlaying false)
          (Variables|/Game/EatUpAll/HUD/WBP_Hunter.WBP_Hunter_C|SetbIsSuckReady (Variables|Default|GetWBP_Hunter) false)))
      (elif (not _bissuck_reload)
        (CallFunction|ReadyVacuumgun)
        (Utilities|FlowControl|Delay 1.3)
        (Variables|Default|SetbIsSuck%20Trigger true)
        (goto _label))))
  (:Released
    (Variables|Default|SetbIsEraseInput false)
    (Variables|Default|SetbIsSuck%20Trigger false)
    (if (not _bissuck_reload)
      (CallFunction|EndVacuumgun)
      (Utilities|FlowControl|Delay 1.3)
      (Variables|/Game/EatUpAll/HUD/WBP_Hunter.WBP_Hunter_C|SetbIsSuckEnd (Variables|Default|GetWBP_Hunter) false))))

(event Input|MouseEvents|RightMouseButton
  (params (Key :type Key%20Structure))
  ;[1 1 1] When Left Mouse Click, Trigger Erase Action
  (:Pressed
    (CallFunction|RightSkillonServer)))

(fn ConstructionScript)

(fn EraseDrawRT
  (bind _thirdpersoncameracomponent (Variables|Default|GetThirdPersonCameraComponent))
  (bind _returnvalue (Transformation|GetWorldLocation _thirdpersoncameracomponent))
  (bind _returnvalue_2 (Math|Vector|GetForwardVector _thirdpersoncameracomponent))
  (bind _outhits (Collision|MultiSphereTraceForObjects (+ _returnvalue (* _returnvalue_2 3.5e+02)) (+ _returnvalue (* _returnvalue_2 1.4e+03)) 128.0 (Utilities|Array|MakeArray "ObjectTypeQuery1" "ObjectTypeQuery2" "ObjectTypeQuery8" "ObjectTypeQuery10") false 0 "None" true "(R=0.000000,G=0.689303,B=1.000000,A=1.000000)" "(R=1.000000,G=0.114155,B=0.834850,A=1.000000)" 0.0))
  (for _array_element _outhits
    (if (.bBlockingHit (Collision|BreakHitResult _array_element))
      (Class|BPIPaint|OnErase(Message) (.HitActor (Collision|BreakHitResult _array_element)) (.UV (Class|GameplayStatics|FindCollisionUV _array_element))))))

(fn PaintDrawRT
  (bind _thirdpersoncameracomponent (Variables|Default|GetThirdPersonCameraComponent))
  (bind _returnvalue (Transformation|GetWorldLocation _thirdpersoncameracomponent))
  (bind _returnvalue_2 (Math|Vector|GetForwardVector _thirdpersoncameracomponent))
  (bind _outhits (Collision|MultiSphereTraceForObjects (+ _returnvalue (* _returnvalue_2 3.5e+02)) (+ _returnvalue (* _returnvalue_2 1e+03)) 42.0 (Utilities|Array|MakeArray "ObjectTypeQuery1" "ObjectTypeQuery2" "ObjectTypeQuery8" "ObjectTypeQuery10") false 0 "None" true "(R=1.000000,G=0.000000,B=0.000000,A=1.000000)" "(R=1.000000,G=0.114155,B=0.834850,A=1.000000)" 0.0))
  (for _array_element _outhits
    (if (.bBlockingHit (Collision|BreakHitResult _array_element))
      (Class|BPIPaint|OnPaint(Message) (.HitActor (Collision|BreakHitResult _array_element)) (.UV (Class|GameplayStatics|FindCollisionUV _array_element))))))

(fn ReadyVacuumgun
  (CallFunction|EnableSuckParticleonServer)
  (Variables|Default|SetbIsEndSoundPlaying false)
  (Variables|/Game/EatUpAll/HUD/WBP_Hunter.WBP_Hunter_C|SetbIsSuckEnd (Variables|Default|GetWBP_Hunter) false)
  (if (not (Variables|Default|GetbIsIniSoundPlaying))
    (Components|Activation|SetActive (Variables|Default|GetAudioCleanerInitiate) true false)
    (Variables|Default|SetbIsIniSoundPlaying true)
    (Variables|/Game/EatUpAll/HUD/WBP_Hunter.WBP_Hunter_C|SetbIsSuckReady (Variables|Default|GetWBP_Hunter) true)))

(fn RunVacuumgun
  (if (Variables|Default|GetbIsEraseInput)
    (Class|VacuumPlayer|PerformVacuum)
    (Variables|/Game/EatUpAll/HUD/WBP_Hunter.WBP_Hunter_C|SetCrosshair%20Spread (Variables|Default|GetWBP_Hunter) 5.0)
    (CallFunction|EnableAllParticleonServer)
    (Variables|Default|SetbIsIniSoundPlaying false)
    (Variables|/Game/EatUpAll/HUD/WBP_Hunter.WBP_Hunter_C|SetbIsSuckReady (Variables|Default|GetWBP_Hunter) false)
    (if (not (Variables|Default|GetbIsRunSoundPlaying))
      (Components|Activation|SetActive (Variables|Default|GetAudioCleanerRun) true false)
      (Variables|Default|SetbIsRunSoundPlaying true)
      (Variables|/Game/EatUpAll/HUD/WBP_Hunter.WBP_Hunter_C|SetbIsSuckRun (Variables|Default|GetWBP_Hunter) true)
      (CallFunction|SlowWalkSpeedonServer))))

(fn CooldownVacuumgun
  (Audio|PlaySoundatLocation "/Game/EatUpAll/SoundEffects/Ambient/break_11.break_11" (Transformation|GetWorldLocation (Variables|Character|GetMesh)) "0, 0, 0" 1.0 1.0 0.0 0 0 0 0))

(fn EndVacuumgun
  (CallFunction|DisactiveAllParticleonServer)
  (Variables|/Game/EatUpAll/HUD/WBP_Hunter.WBP_Hunter_C|SetCrosshair%20Spread (Variables|Default|GetWBP_Hunter) 7e+01)
  (Variables|Default|SetbIsRunSoundPlaying false)
  (Variables|/Game/EatUpAll/HUD/WBP_Hunter.WBP_Hunter_C|SetbIsSuckRun (Variables|Default|GetWBP_Hunter) false)
  (if (not (Variables|Default|GetbIsEndSoundPlaying))
    (Components|Activation|SetActive (Variables|Default|GetAudioCleanerEnd) true false)
    (Variables|Default|SetbIsEndSoundPlaying true)
    (Variables|/Game/EatUpAll/HUD/WBP_Hunter.WBP_Hunter_C|SetbIsSuckEnd (Variables|Default|GetWBP_Hunter) true)
    (CallFunction|FastWalkSpeedonServer)))