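; BP_H1Projectile is a player projectile that either explodes on a slime character or becomes a delayed smoke hazard.
; Until its first non-owner hit, a per-tick sphere trace triggers Explode on slimes, damaging and launching them, pushing vacuumables and destroying itself.
; That hit instead starts a countdown to repeated, delayed Smoke pulses of lighter damage, then destruction.
; Both effects use multi-sphere traces and send collision UVs through OnEraseMessage to blocking hits.
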(event OnComponentHit(StaticMesh)
  (params (HitComponent :type Primitive%20Component%20Object%20Reference) (OtherActor :type Actor%20Object%20Reference) (OtherComp :type Primitive%20Component%20Object%20Reference) (NormalImpulse :type Vector :default "0, 0, 0") (Hit :type Hit%20Result%20Structure%20%28by%20ref%29))
  (Utilities|FlowControl|DoOnce false
    (:Completed
      (if (!= OtherActor (Components|GetOwner))
        (Variables|Default|SetTime 5.0)
        (Variables|Default|SetTickle true)))))

(event Custom|Smoke
  (bind _returnvalue (Transformation|GetActorLocation))
  (bind _outhits (Collision|MultiSphereTraceForObjects _returnvalue _returnvalue 4.2e+02 (Utilities|Array|MakeArray "ObjectTypeQuery1" "ObjectTypeQuery2" "ObjectTypeQuery8" "ObjectTypeQuery10" "ObjectTypeQuery7") false 0 "ForOneFrame" true "(R=0.000000,G=0.689303,B=1.000000,A=1.000000)" "(R=1.000000,G=0.114155,B=0.834850,A=1.000000)" 1.0))
  (for _array_element _outhits
    (Utilities|FlowControl|Sequence
      (:then_0
        (if (.bBlockingHit (Collision|BreakHitResult _array_element))
          (Class|BPIPaint|OnErase(Message) (.HitActor (Collision|BreakHitResult _array_element)) (.UV (Class|GameplayStatics|FindCollisionUV _array_element)))))
      (:then_1
        (bind _asbp_slime_char_for_new_move_done (Utilities|Casting|CastToBP_SlimeCharForNewMove_Done (.HitActor (Collision|BreakHitResult _array_element))))
        (Game|Damage|ApplyDamage _asbp_slime_char_for_new_move_done 1.0 0 0))
      (:then_2
        (bind _asbp_vacuumable (Utilities|Casting|CastToBP_Vacuumable (.HitActor (Collision|BreakHitResult _array_element))))))))

(event Custom|Explode
  (bind _returnvalue (Transformation|GetActorLocation))
  (bind _outhits (Collision|MultiSphereTraceForObjects _returnvalue _returnvalue 4.2e+02 (Utilities|Array|MakeArray "ObjectTypeQuery1" "ObjectTypeQuery2" "ObjectTypeQuery8" "ObjectTypeQuery10" "ObjectTypeQuery7") false 0 "ForOneFrame" true "(R=0.000000,G=0.689303,B=1.000000,A=1.000000)" "(R=1.000000,G=0.114155,B=0.834850,A=1.000000)" 1.0))
  (for _array_element _outhits
    (Utilities|FlowControl|Sequence
      (:then_0
        (if (.bBlockingHit (Collision|BreakHitResult _array_element))
          (Class|BPIPaint|OnErase(Message) (.HitActor (Collision|BreakHitResult _array_element)) (.UV (Class|GameplayStatics|FindCollisionUV _array_element)))))
      (:then_1
        (bind _asbp_slime_char_for_new_move_done (Utilities|Casting|CastToBP_SlimeCharForNewMove_Done (.HitActor (Collision|BreakHitResult _array_element))))
        (Game|Damage|ApplyDamage _asbp_slime_char_for_new_move_done 1e+01 0 0)
        (Character|LaunchCharacter _asbp_slime_char_for_new_move_done (* (Math|Vector|Normalize (- (Transformation|GetActorLocation _asbp_slime_char_for_new_move_done) (Transformation|GetActorLocation))) 1e+03) false false))
      (:then_2
        (bind _asbp_vacuumable (Utilities|Casting|CastToBP_Vacuumable (.HitActor (Collision|BreakHitResult _array_element))))
        (Physics|AddImpulse (Variables|/Script/EatUpAll.Vacuumable|GetMesh _asbp_vacuumable) (* (Math|Vector|Normalize (- (Transformation|GetActorLocation _asbp_vacuumable) (Transformation|GetActorLocation))) 1e+03) "None" true))))
  (Actor|DestroyActor))

(event EventBeginPlay)

(event Collision|EventActorBeginOverlap
  (params (OtherActor :type Actor%20Object%20Reference)))

(event EventTick
  (params (DeltaSeconds :type Float%20%28single-precision%29))
  (bind _returnvalue (Transformation|GetActorLocation))
  (if (Variables|Default|GetTickle)
    (Variables|Default|SetTime (- (Variables|Default|GetTime) (Utilities|Time|GetWorldDeltaSeconds)))
    (if (<= (Variables|Default|GetTime) 0.0)
      (Utilities|FlowControl|DoOnce false
        (:Completed
          (bind _index (Utilities|DelayedForloop 0 5 1.0)
            (:loop%20Body
              (Development|PrintString (Utilities|String|ToString(Integer) _index))
              (CallFunction|Smoke))
            (:Completed
              (Actor|DestroyActor))))))
    (else
      (bind _outhit (Collision|SphereTraceForObjects _returnvalue _returnvalue 45.0 (Utilities|Array|MakeArray "ObjectTypeQuery7") false (Utilities|Array|MakeArray (Components|GetOwner)) "ForDuration" true "(R=1.000000,G=0.000000,B=0.000000,A=1.000000)" "(R=0.000000,G=1.000000,B=0.000000,A=1.000000)" 0.0))
      (Utilities|Casting|CastToBP_SlimeCharForNewMove_Done (.HitActor (Collision|BreakHitResult _outhit)))
      (CallFunction|Explode))))

(fn ConstructionScript)