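; Second hunter player character, adding death spectating and vacuum gun effect events on top of its parent class.
; When dead, the SpectatorCamera input switches the view to the first BP_HunterPlayer if alive; the input always removes the common play HUD.
; While dead, Tick copies its third-person camera rotation onto that hunter's first-person camera.
; Particle-sync events for clients toggle effects on its BP_VacuumGun2.
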(event EventEnableAllParticleonClient
  ;[1 1 1] Particle Sync Client-Server
  (bind _asbp_vacuum_gun_2 (Utilities|Casting|CastToBP_VacuumGun2 (Variables|Default|GetVacuumGun)))
  (Default|EnableAllEffect _asbp_vacuum_gun_2))

(event EventDisactiveAllParticleonClient
  ;[1 1 1] Particle Sync Client-Server
  (bind _asbp_vacuum_gun_2 (Utilities|Casting|CastToBP_VacuumGun2 (Variables|Default|GetVacuumGun)))
  (Default|DisableAllEffect _asbp_vacuum_gun_2))

(event EventTick
  (params (DeltaSeconds :type Float%20%28single-precision%29))
  (bind _thirdpersoncameracomponent (Variables|Default|GetThirdPersonCameraComponent))
  (bind _returnvalue (Transformation|GetWorldRotation _thirdpersoncameracomponent))
  (|CallParentFunction 0.0)
  (if (Variables|Default|GetbIsDead)
    (bind _outactors (Actor|GetAllActorsOfClass "/Game/EatUpAll/Blueprints/Player/BP_HunterPlayer.BP_HunterPlayer_C"))
    (Transformation|SetWorldRotation (Variables|/Script/EatUpAll.VacuumPlayer|GetFirstPersonCameraComponent (Utilities|Array|Get(acopy) _outactors)) (Math|Rotator|MakeRotator (.roll _returnvalue) (.pitch _returnvalue) (.yaw _returnvalue)) false false)))

(event EventBeginPlay
  (|CallParentFunction))

(event Collision|EventActorBeginOverlap
  (params (OtherActor :type Actor%20Object%20Reference))
  (|CallParentFunction OtherActor) ; This node is disabled and will not be called.\nDrag off pins to build functionality.
)

(event EventEnableSuckParticleonClient
  ;[1 1 1] Particle Sync Client-Server
  (bind _asbp_vacuum_gun_2 (Utilities|Casting|CastToBP_VacuumGun2 (Variables|Default|GetVacuumGun)))
  (Default|EnableSuckEffect _asbp_vacuum_gun_2))

(event Input|ActionEvents|InputActionSpectatorCamera
  (params (Key :type Key%20Structure))
  (:Pressed
    (Widget|RemovefromParent (Variables|/Game/EatUpAll/HUD/BP_PlayerContorller.BP_PlayerContorller_C|GetWBP_PlayCommon (.AsBP%20Player%20Contorller (Utilities|Casting|CastToBP_PlayerContorller (Game|GetPlayerController 0)))))
    (if (Variables|Default|GetbIsDead)
      (bind _outactors (Actor|GetAllActorsOfClass "/Game/EatUpAll/Blueprints/Player/BP_HunterPlayer.BP_HunterPlayer_C"))
      (if (not (Variables|/Game/EatUpAll/Blueprints/Player/BP_VacuumPlayer.BP_VacuumPlayer_C|GetbIsDead (Utilities|Array|Get(acopy) _outactors)))
        (Default|ActiveVacuumgunPos (Utilities|Array|Get(acopy) _outactors))
        (Game|Player|SetViewTargetwithBlend (Game|GetPlayerController 0) (Utilities|Array|Get(acopy) _outactors) 0.0 "VTBlend_Linear" 0.0 false)
        (Default|CallSpectatorView)))))

(fn ConstructionScript
  (|CallParentFunction))