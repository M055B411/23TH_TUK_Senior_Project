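; First-person hunter player that wields a vacuum gun and erases or paints on surfaces, apparently via render targets.
; Left and right mouse set erase and paint flags, read by a camera trace that Tick routes through server and multicast events.
; Sphere (erase) or line (paint) hits message actors with collision UVs.
; Tick also toggles gun effects by vacuuming and overload state, while left-click "Particle" RPCs sync attack montages.
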(event Custom|RPC_Multi_Disactive_Particle
  ;[1 1 1] Particle Sync Client-Server
  (Animation|PlayAnimMontage "/Game/EatUpAll/Blueprints/Player/Animations/attack_anime_2_Montage.attack_anime_2_Montage" 1.0 "None"))

(event Custom|RPC_Multi_Particle
  ;[1 1 1] Particle Sync Client-Server
  (Animation|PlayAnimMontage "/Game/EatUpAll/Blueprints/Player/Animations/attack_anime_Montage.attack_anime_Montage" 1.0 "None"))

(event Custom|Multi%20LineTrace%20RT
  (CallFunction|LineTraceRT))

(event Custom|RPC_Server_Particle
  ;[1 1 1] Particle Sync Client-Server
  (CallFunction|RPCMultiParticle))

(event Custom|RPC_Server_DisactiveParticle
  ;[1 1 1] Particle Sync Client-Server
  (CallFunction|RPCMultiDisactiveParticle))

(event Custom|Server%20LineTrace%20RT
  (CallFunction|MultiLineTraceRT))

(event EventPossessed
  (params (NewController :type Controller%20Object%20Reference))
  (bind _asplayer_controller (Utilities|Casting|CastToPlayerController NewController))
  (Utilities|IsValid (PlayerController|LocalPlayerSubsystems|GetEnhancedInputLocalPlayerSubsystem _asplayer_controller)
    (:Is%20Valid
      (Input|AddMappingContext (PlayerController|LocalPlayerSubsystems|GetEnhancedInputLocalPlayerSubsystem _asplayer_controller) "/Game/EatUpAll/VacuumPl/Input/IMC_Vacuum.IMC_Vacuum" 0 "(bIgnoreAllPressedKeysUntilRelease=True,bForceImmediately=False)"))))

(event EventTick
  (params (DeltaSeconds :type Float%20%28single-precision%29))
  (CallFunction|ServerLineTraceRT)
  (bind _asbp_vacuum_gun (Utilities|Casting|CastToBP_VacuumGun (Variables|Default|GetVacuumGun)))
  (if (and (Variables|/Script/EatUpAll.VacuumGun|GetIsVacuuming _asbp_vacuum_gun) (not (Class|VacuumGun|GetOverloaded _asbp_vacuum_gun)))
    (Default|EnableSelfEffect _asbp_vacuum_gun)
    (Default|EnableOtherEffect _asbp_vacuum_gun)
    (else
      (Default|DisableSelfEffect _asbp_vacuum_gun)
      (Default|DisableOtherEffect _asbp_vacuum_gun))))

(event EventBeginPlay
  (|CallParentFunction))

(event Collision|EventActorBeginOverlap
  (params (OtherActor :type Actor%20Object%20Reference))
  (|CallParentFunction OtherActor) ; This node is disabled and will not be called.\nDrag off pins to build functionality.
)

(event Input|MouseEvents|RightMouseButton
  (params (Key :type Key%20Structure :default "None"))
  (:Pressed
    (Variables|Default|SetCheckRT_Paint true))
  (:Released
    (Variables|Default|SetCheckRT_Paint false)))

(event Input|MouseEvents|LeftMouseButton
  (params (Key :type Key%20Structure :default "None"))
  (:Pressed
    (Variables|Default|SetCheckRT_Erase true)
    (CallFunction|RPCServerParticle))
  (:Released
    (Variables|Default|SetCheckRT_Erase false)
    (CallFunction|RPCServerDisactiveParticle)))

(fn ConstructionScript
  (|CallParentFunction))

(fn LineTraceRT
  (bind _firstpersoncameracomponent (Variables|Default|GetFirstPersonCameraComponent))
  (bind _firstpersoncameracomponent_2 (Variables|Default|GetFirstPersonCameraComponent))
  (bind _returnvalue (Transformation|GetWorldLocation _firstpersoncameracomponent_2))
  (bind _returnvalue_2 (Transformation|GetWorldLocation _firstpersoncameracomponent))
  (Utilities|FlowControl|Sequence
    (:then_0
      (if (Variables|Default|GetCheckRT_Erase)
        (bind _outhits (Collision|MultiSphereTraceForObjects _returnvalue_2 (+ _returnvalue_2 (* (Math|Vector|GetForwardVector _firstpersoncameracomponent) 1e+03)) 0.0 (Utilities|Array|MakeArray "ObjectTypeQuery1" "ObjectTypeQuery2") false 0 "None"))
        (for _array_element _outhits
          (if (.bBlockingHit (Collision|BreakHitResult _array_element))
            (Class|BPIPaint|OnErase(Message) (.HitActor (Collision|BreakHitResult _array_element)) (.UV (Class|GameplayStatics|FindCollisionUV _array_element)))))))
    (:then_1
      (if (Variables|Default|GetCheckRT_Paint)
        (bind _outhits_2 (Class|KismetSystemLibrary|LineTraceMultiforObjects _returnvalue (+ _returnvalue (* (Math|Vector|GetForwardVector _firstpersoncameracomponent_2) 1e+03)) (Utilities|Array|MakeArray "ObjectTypeQuery1" "ObjectTypeQuery2") false 0 "None" false))
        (for _array_element_2 _outhits_2
          (if (.bBlockingHit (Collision|BreakHitResult _array_element_2))
            (Class|BPIPaint|OnPaint(Message) (.HitActor (Collision|BreakHitResult _array_element_2)) (.UV (Class|GameplayStatics|FindCollisionUV _array_element_2)))))))))

(fn OnRepTest)