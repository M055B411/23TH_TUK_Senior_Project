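; BP_VacuumGun2 is a player vacuum gun Blueprint that controls two effect components, NSSuck and NSAurora.
; On BeginPlay it sets the relative location of both effects to the value returned by GetMuzzleLocation.
; Helper functions activate or deactivate both effects together, or activate the suck effect alone, without resetting them.
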(event EventBeginPlay
  (bind _returnvalue (Class|VacuumGun|GetMuzzleLocation))
  (Transformation|SetRelativeLocation (Variables|Default|GetNS_Suck) _returnvalue false false))

(fn ConstructionScript)

(fn EnableAllEffect
  (Components|Activation|SetActive (Variables|Default|GetNS_Suck) true false)
  (Components|Activation|SetActive (Variables|Default|GetNS_Aurora) true false))

(fn DisableAllEffect
  (Components|Activation|SetActive (Variables|Default|GetNS_Suck) false false)
  (Components|Activation|SetActive (Variables|Default|GetNS_Aurora) false false))

(fn EnableSuckEffect
  (Components|Activation|SetActive (Variables|Default|GetNS_Suck) true false))