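; BP_Vacuumable is a physics object, by name one that can be vacuumed, that floats on surfaces of a specific object type.
; Every tick, Buoyancy traces down from Mesh and pushes it along the hit normal with mass-scaled force that fades with distance, raising damping on contact.
; Tick also sets GenerateHit only while gravity is enabled and velocity exceeds a threshold.
; The buoyancy trace leaves debug drawing on.
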(event EventTick
  (params (DeltaSeconds :type Float%20%28single-precision%29))
  (CallFunction|Buoyancy (Variables|Character|GetMesh) 1e+02 "ObjectTypeQuery9")
  (if (and (Class|PrimitiveComponent|IsGravityEnabled (Variables|Character|GetMesh)) (> (Math|Vector|VectorLength (Transformation|GetVelocity)) 6e+02))
    (Variables|Default|SetGenerate%20Hit true)
    (else
      (Variables|Default|SetGenerate%20Hit false))))

(fn ConstructionScript)

(fn Buoyancy
  (params (Float :type Primitive%20Component%20Object%20Reference) (FloatHeight :type Float%20%28double-precision%29) (ObjectType :type EObjectTypeQuery%20Enum :default "ObjectTypeQuery1"))
  (bind _returnvalue (Transformation|GetWorldLocation Float))
  (bind _returnvalue_2 (Transformation|GetWorldScale Float))
  (bind (_outhit _returnvalue_3) (Collision|LineTraceForObjects _returnvalue (- _returnvalue (Math|Vector|MakeVector 0.0 0.0 (+ (/ (+ (.x _returnvalue_2) (.y _returnvalue_2) (.z _returnvalue_2)) 3.0) FloatHeight))) (Utilities|Array|MakeArray ObjectType) false 0 "ForDuration"))
  (if _returnvalue_3
    (Physics|AddForce Float (* (.ImpactNormal (Collision|BreakHitResult _outhit)) (Math|Float|Lerp (* (Physics|GetMass Float) 1.2e+03) 0.0 (/ (Math|Vector|VectorLength (- (.Location (Collision|BreakHitResult _outhit)) (Transformation|GetWorldLocation Float))) FloatHeight))) "None" false)
    (Class|PrimitiveComponent|SetAngularDamping Float 4.0)
    (Class|PrimitiveComponent|SetLinearDamping Float 5.0)))