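; BP_Object is a physics prop that floats above surfaces of a given object type and receives material paint values on overlap.
; Each tick, Buoyancy traces downward and pushes the mesh along the hit normal with mass-scaled force that fades with distance, raising linear and angular damping.
; On actor overlap, it writes its Color and Roughness variables to the mesh's Custom Primitive Data.
; The buoyancy trace leaves debug drawing enabled.
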(event EventBeginPlay)

(event Collision|EventActorBeginOverlap
  (params (OtherActor :type Actor%20Object%20Reference))
  (bind _color (Variables|Default|GetColor))
  (bind _staticmesh (Variables|Default|GetStaticMesh))
  (Rendering|Material|SetCustomPrimitiveDataFloat _staticmesh 4 (Variables|Default|GetRoughness))
  (Rendering|Material|SetCustomPrimitiveDataVector3 _staticmesh 0 (Math|Vector|MakeVector (.r _color) (.g _color) (.b _color))))

(event EventTick
  (params (DeltaSeconds :type Float%20%28single-precision%29))
  (CallFunction|Buoyancy (Variables|Default|GetStaticMesh) 1e+02 "ObjectTypeQuery7"))

(fn ConstructionScript)

(fn Buoyancy
  (params (PrimitiveComponent :type Primitive%20Component%20Object%20Reference) (FloatHeight1 :type Float%20%28double-precision%29) (ObjectType1 :type EObjectTypeQuery%20Enum :default "ObjectTypeQuery1"))
  (bind _returnvalue (Transformation|GetWorldLocation PrimitiveComponent))
  (bind _returnvalue_2 (Transformation|GetWorldScale PrimitiveComponent))
  (bind (_outhit _returnvalue_3) (Collision|LineTraceForObjects _returnvalue (- _returnvalue (Math|Vector|MakeVector 0.0 0.0 (+ (/ (+ (.x _returnvalue_2) (.y _returnvalue_2) (.z _returnvalue_2)) 3.0) FloatHeight1))) (Utilities|Array|MakeArray ObjectType1) false 0 "ForDuration"))
  (if _returnvalue_3
    (Physics|AddForce PrimitiveComponent (* (.ImpactNormal (Collision|BreakHitResult _outhit)) (Math|Float|Lerp (* (Physics|GetMass PrimitiveComponent) 1.1e+03) 0.0 (/ (Math|Vector|VectorLength (- (.Location (Collision|BreakHitResult _outhit)) (Transformation|GetWorldLocation PrimitiveComponent))) FloatHeight1))) "None" false)
    (Class|PrimitiveComponent|SetAngularDamping PrimitiveComponent 4.0)
    (Class|PrimitiveComponent|SetLinearDamping PrimitiveComponent 1e+01)))