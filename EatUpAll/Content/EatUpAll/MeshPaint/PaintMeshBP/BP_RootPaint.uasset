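; Base Blueprint for paintable meshes that paints and erases brush marks at a given UV on per-instance render targets.
; Construction creates runtime and persistent targets plus brush and copy materials; BeginPlay clears the targets and feeds the runtime one to the mesh's dynamic materials.
; DrawBrush stamps the runtime target through Canvas, then copies runtime to persistent and back via materials.
; Painting is throttled by DoOnce and Delay, randomizing a parameter-collection frame per stamp; erasing is unthrottled.
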(event Custom|EraseToRenderTarget
  (params (Size :type Float%20%28double-precision%29) (LocationToErase :type Vector%202D%20Structure) (TextureRenderTarget :type Texture%20Render%20Target%202D%20Object%20Reference) (TextureRenderTarget2 :type Texture%20Render%20Target%202D%20Object%20Reference))
  ;[0.3851 1 0.9801] Paint and Erase
  ;;[1 1 1] Draw RenderTarget
  (CallFunction|DrawBrush Size LocationToErase TextureRenderTarget TextureRenderTarget2 (Variables|Default|GetBrushMaterialErase)))

(event Custom|SetValues
  ;[1 1 1] Inital Setting
  (for _array_element (Variables|Default|GetDynamicMaterials)
    (Rendering|Material|SetTextureParameterValue _array_element "RT_Runtime" (Variables|Default|GetRenderTargetRuntime))))

(event Custom|DrawToRenderTarget
  (params (Size :type Float%20%28double-precision%29) (LocationToDraw :type Vector%202D%20Structure) (TextureRenderTarget :type Texture%20Render%20Target%202D%20Object%20Reference) (TextureRenderTarget2 :type Texture%20Render%20Target%202D%20Object%20Reference))
  ;[0.3851 1 0.9801] Paint and Erase
  ;;[1 1 1] Draw RenderTarget
  (Utilities|FlowControl|DoOnce false :!label _label
    (:Completed
      (Rendering|Material|SetScalarParameterValue "/Game/EatUpAll/MeshPaint/MPC_PaintFrame.MPC_PaintFrame" "Frame" (Math|Conversions|ToFloat(Integer) (Math|Random|RandomIntegerinRange 0 8)) :!class /Script/Engine.KismetMaterialLibrary)
      (CallFunction|DrawBrush Size LocationToDraw TextureRenderTarget TextureRenderTarget2 (Variables|Default|GetBrushMaterialPaint))
      (Utilities|FlowControl|Delay 0.2)
      (goto _label Reset))))

(event EventOnPaint
  (params (UV :type Vector%202D%20Structure))
  ;[0.3851 1 0.9801] Paint and Erase
  ;;[1 1 1] Input for Paint
  (CallFunction|DrawtoRenderTarget (Variables|Default|GetSize) UV (Variables|Default|GetRenderTargetRuntime) (Variables|Default|GetRenderTargetPersistant)))

(event EventOnErase
  (params (UV :type Vector%202D%20Structure))
  ;[0.3851 1 0.9801] Paint and Erase
  ;;[1 1 1] Input for Erase
  (CallFunction|ErasetoRenderTarget (Variables|Default|GetSize) UV (Variables|Default|GetRenderTargetRuntime) (Variables|Default|GetRenderTargetPersistant)))

(event EventBeginPlay
  (bind _staticmesh (Variables|Default|GetStaticMesh))
  ;[1 1 1] Inital Setting
  (for (_array_element _array_index) (Rendering|Material|GetMaterials _staticmesh)
    (bind _returnvalue (Rendering|Material|CreateDynamicMaterialInstance _staticmesh _array_index _array_element "None" :!class /Script/Engine.PrimitiveComponent))
    (Utilities|Array|SetArrayElem (Variables|Default|GetDynamicMaterials) 0 _returnvalue true)
    (Rendering|Material|SetTextureParameterValue (Variables|Default|GetDrawToPersistantMaterial) "RT_Capture" (Variables|Default|GetRenderTargetRuntime))
    (Rendering|Material|SetTextureParameterValue (Variables|Default|GetDrawToRuntimeMaterial) "RT_Persistant" (Variables|Default|GetRenderTargetPersistant))
    (Rendering|ClearRenderTarget2D (Variables|Default|GetRenderTargetRuntime))
    (Rendering|ClearRenderTarget2D (Variables|Default|GetRenderTargetPersistant)))
  (CallFunction|SetValues))

(fn ConstructionScript
  (Utilities|FlowControl|Sequence
    (:then_0
      (bind _returnvalue (Rendering|CreateRenderTarget2D 256 256 "RTF_RG16f"))
      (Variables|Default|SetRenderTargetRuntime _returnvalue))
    (:then_1
      (bind _returnvalue_2 (Rendering|CreateRenderTarget2D 256 256 "RTF_R16f"))
      (Variables|Default|SetRenderTargetPersistant _returnvalue_2))
    (:then_2
      (bind _returnvalue_3 (Rendering|Material|CreateDynamicMaterialInstance "/Game/EatUpAll/Painting/RT/M_DrawToPersistant_Inst.M_DrawToPersistant_Inst" "None" "None" :!class /Script/Engine.KismetMaterialLibrary))
      (Variables|Default|SetDrawToPersistantMaterial _returnvalue_3))
    (:then_3
      (bind _returnvalue_4 (Rendering|Material|CreateDynamicMaterialInstance "/Game/EatUpAll/Painting/RT/M_DrawToRuntime_Inst.M_DrawToRuntime_Inst" "None" "None" :!class /Script/Engine.KismetMaterialLibrary))
      (Variables|Default|SetDrawToRuntimeMaterial _returnvalue_4))
    (:then_4
      (bind _returnvalue_5 (Rendering|Material|CreateDynamicMaterialInstance "/Game/EatUpAll/MeshPaint/M_BrushPaint_Inst.M_BrushPaint_Inst" "None" "None" :!class /Script/Engine.KismetMaterialLibrary))
      (Variables|Default|SetBrushMaterialPaint _returnvalue_5))
    (:then_5
      (bind _returnvalue_6 (Rendering|Material|CreateDynamicMaterialInstance "/Game/EatUpAll/MeshPaint/M_BrushErase_Inst.M_BrushErase_Inst" "None" "None" :!class /Script/Engine.KismetMaterialLibrary))
      (Variables|Default|SetBrushMaterialErase _returnvalue_6))))

(fn DrawBrush
  (params (BrushSize :type Float%20%28double-precision%29) (DrawLocation :type Vector%202D%20Structure) (TextureRT%20Runtime :type Texture%20Render%20Target%202D%20Object%20Reference) (TextureRT%20Persistant :type Texture%20Render%20Target%202D%20Object%20Reference) (BrushMaterial :type Material%20Instance%20Object%20Reference))
  (Utilities|FlowControl|Sequence
    (:then_0
      (bind (_canvas _size _context) (Rendering|BeginDrawCanvastoRenderTarget TextureRT%20Runtime))
      (Canvas|DrawMaterial :self _canvas :RenderMaterial BrushMaterial :ScreenPosition (- (* _size DrawLocation) (/ BrushSize 2.0)) :ScreenSize (Math|Vector2D|MakeVector2D BrushSize BrushSize) :CoordinateSize "(X=1.000000,Y=1.000000)" :PivotPoint "(X=0.500000,Y=0.500000)")
      (Rendering|EndDrawCanvastoRenderTarget _context))
    (:then_1
      (Rendering|DrawMaterialtoRenderTarget TextureRT%20Persistant (Variables|Default|GetDrawToPersistantMaterial))
      (Rendering|DrawMaterialtoRenderTarget TextureRT%20Runtime (Variables|Default|GetDrawToRuntimeMaterial)))))