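; Physics object that floats over a specific surface type and carries a paintable material progress value.
; Each tick, a downward trace applies a distance-scaled hover force along the surface normal and raises damping.
; Overlaps and paint events raise progress after a short delay, while erase events lower it slightly faster.
; Progress and its maximum feed the mesh material through custom primitive data, avoiding dynamic material instances.
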(event EventBeginPlay
  (Rendering|Material|SetCustomPrimitiveDataFloat (Variables|Default|GetStaticMesh) (+ (Variables|Default|GetMaterialPrimitiveDataIndex) 1) (Variables|Default|GetProgressMax)))

(event Collision|EventActorBeginOverlap
  (params (OtherActor :type Actor%20Object%20Reference))
  (Variables|Default|SetIsOverlapped true))

(event EventOnPaint
  (params (UV :type Vector%202D%20Structure))
  (Utilities|FlowControl|Delay 0.2)
  (CallFunction|MaterialProgressUp))

(event Collision|EventActorEndOverlap
  (params (OtherActor :type Actor%20Object%20Reference))
  (Variables|Default|SetIsOverlapped false))

(event EventOnErase
  (params (UV :type Vector%202D%20Structure))
  (Utilities|FlowControl|Delay 0.2)
  (CallFunction|MaterialProgressDown))

(event EventTick
  (params (DeltaSeconds :type Float%20%28single-precision%29))
  (Utilities|FlowControl|Sequence
    (:then_0
      (CallFunction|Buoyancy (Variables|Default|GetStaticMesh) 1e+02 "ObjectTypeQuery7"))
    (:then_1
      (if (Variables|Default|GetIsOverlapped)
        (Utilities|FlowControl|Delay 0.2)
        (CallFunction|MaterialProgressUp)))
    (:then_2
      (if (>= (Variables|Default|GetMaterialProgress) 0.0)
        (CallFunction|SetMaterialProgress (Variables|Default|GetMaterialProgress))
        (else
          (Variables|Default|SetMaterialProgress 0.0))))))

(fn ConstructionScript)

(fn Buoyancy
  (params (PrimitiveComponent :type Primitive%20Component%20Object%20Reference) (FloatHeight1 :type Float%20%28double-precision%29) (ObjectType1 :type EObjectTypeQuery%20Enum :default "ObjectTypeQuery1"))
  (bind _returnvalue (Transformation|GetWorldLocation PrimitiveComponent))
  (bind _returnvalue_2 (Transformation|GetWorldScale PrimitiveComponent))
  (bind (_outhit _returnvalue_3) (Collision|LineTraceForObjects _returnvalue (- _returnvalue (Math|Vector|MakeVector 0.0 0.0 (+ (/ (+ (.x _returnvalue_2) (.y _returnvalue_2) (.z _returnvalue_2)) 3.0) FloatHeight1))) (Utilities|Array|MakeArray ObjectType1) false 0 "None"))
  (if _returnvalue_3
    (Physics|AddForce PrimitiveComponent (* (.ImpactNormal (Collision|BreakHitResult _outhit)) (Math|Float|Lerp (* (Physics|GetMass PrimitiveComponent) 1.1e+03) 0.0 (/ (Math|Vector|VectorLength (- (.Location (Collision|BreakHitResult _outhit)) (Transformation|GetWorldLocation PrimitiveComponent))) FloatHeight1))) "None" false)
    (Class|PrimitiveComponent|SetAngularDamping PrimitiveComponent 4.0)
    (Class|PrimitiveComponent|SetLinearDamping PrimitiveComponent 1e+01)))

(fn SetMaterialProgress
  (params (MaterialProgress :type Float%20%28double-precision%29))
  (bind _output_get (Variables|Default|SetMaterialProgress MaterialProgress))
  (Rendering|Material|SetCustomPrimitiveDataFloat (Variables|Default|GetStaticMesh) (Variables|Default|GetMaterialPrimitiveDataIndex) _output_get))

(fn MaterialProgressUp
  (if (< (Variables|Default|GetMaterialProgress) (Variables|Default|GetProgressMax))
    (Variables|Default|SetMaterialProgress (+ (Variables|Default|GetMaterialProgress) 0.1))))

(fn MaterialProgressDown
  (if (> (Variables|Default|GetMaterialProgress) 0.0)
    (Variables|Default|SetMaterialProgress (- (Variables|Default|GetMaterialProgress) 0.14))))