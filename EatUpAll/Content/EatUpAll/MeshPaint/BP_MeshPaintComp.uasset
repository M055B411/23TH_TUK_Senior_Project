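; Component for BP_Vacuumable actors that tracks a paint progress value and feeds it to the mesh material.
; Owner overlap or OnPaint raises progress toward ProgressMax and OnErase lowers it, each step gated by a short Delay.
; Tick writes progress into the mesh's Custom Primitive Data, resetting negatives to zero; BeginPlay stores ProgressMax in the next data slot.
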(event Custom|OwnerBeginOverlap
  (params (OtherActor :type Actor%20Object%20Reference))
  (Variables|Default|SetIsOverlapped true))

(event Custom|OwnerEndOverlap
  (params (OtherActor :type Actor%20Object%20Reference))
  (Variables|Default|SetIsOverlapped false))

(event EventOnErase
  (params (UV :type Vector%202D%20Structure))
  (Utilities|FlowControl|Delay 0.2)
  (CallFunction|MaterialProgressDown))

(event EventOnPaint
  (params (UV :type Vector%202D%20Structure))
  (Utilities|FlowControl|Delay 0.2)
  (CallFunction|MaterialProgressUp))

(event EventBeginPlay
  (bind _asbp_vacuumable (Utilities|Casting|CastToBP_Vacuumable (Components|GetOwner)))
  (Rendering|Material|SetCustomPrimitiveDataFloat (Variables|/Script/EatUpAll.Vacuumable|GetMesh _asbp_vacuumable) (+ (Variables|Default|GetMaterialPrimitiveDataIndex) 1) (Variables|Default|GetProgressMax)))

(event EventTick
  (params (DeltaSeconds :type Float%20%28single-precision%29))
  (Utilities|FlowControl|Sequence
    (:then_0
      (if (Variables|Default|GetIsOverlapped)
        (Utilities|FlowControl|Delay 0.2)
        (CallFunction|MaterialProgressUp)))
    (:then_1
      (if (>= (Variables|Default|GetMaterialProgress) 0.0)
        (CallFunction|SetMaterialProgress (Variables|Default|GetMaterialProgress))
        (else
          (Variables|Default|SetMaterialProgress 0.0))))))

(fn SetMaterialProgress
  (params (MaterialProgress :type Float%20%28double-precision%29))
  (bind _output_get (Variables|Default|SetMaterialProgress MaterialProgress))
  (bind _asbp_vacuumable (Utilities|Casting|CastToBP_Vacuumable (Components|GetOwner)))
  (Rendering|Material|SetCustomPrimitiveDataFloat (Variables|/Script/EatUpAll.Vacuumable|GetMesh _asbp_vacuumable) (Variables|Default|GetMaterialPrimitiveDataIndex) _output_get))

(fn MaterialProgressUp
  (if (< (Variables|Default|GetMaterialProgress) (Variables|Default|GetProgressMax))
    (Variables|Default|SetMaterialProgress (+ (Variables|Default|GetMaterialProgress) 0.1))))

(fn MaterialProgressDown
  (if (> (Variables|Default|GetMaterialProgress) 0.0)
    (Variables|Default|SetMaterialProgress (- (Variables|Default|GetMaterialProgress) 0.14))))