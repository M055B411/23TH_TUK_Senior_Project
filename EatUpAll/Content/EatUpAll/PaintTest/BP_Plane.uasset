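; BP_Plane is a paint-test surface whose mesh materials display splats painted into a runtime render target.
; At BeginPlay it creates dynamic instances of its materials, clears the render target and binds it to their RT parameter.
; OnPaint passes a UV to DrawToRenderTarget, which sets strength, size and position on an M_HeatSplat instance, draws it into the target and debug-prints the position.
; World-to-UV conversion math is left unconnected.
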(event Custom|DrawToRenderTarget
  (params (Location :type Vector) (Strength :type Float%20%28double-precision%29) (Size :type Float%20%28double-precision%29) (LocationToDraw :type Vector%202D%20Structure))
  (bind _returnvalue (Math|Conversions|ToVector(Vector2D) LocationToDraw))
  (bind _mid_heatsplat (Variables|Default|GetMID_Heatsplat))
  (Rendering|Material|SetScalarParameterValue _mid_heatsplat "Strength" Strength :!class /Script/Engine.MaterialInstanceDynamic)
  (Rendering|Material|SetScalarParameterValue _mid_heatsplat "Size" Size :!class /Script/Engine.MaterialInstanceDynamic)
  (Rendering|Material|SetVectorParameterValue _mid_heatsplat "Position" (Math|Conversions|ToLinearColor(Vector) _returnvalue) :!class /Script/Engine.MaterialInstanceDynamic)
  (Rendering|DrawMaterialtoRenderTarget (Variables|Default|GetRenderTargetRuntime) _mid_heatsplat)
  (Development|PrintString (Utilities|String|ToString(Vector) _returnvalue)))

(event Custom|SetValues
  (for _array_element (Variables|Default|GetDynamicMaterials)
    (Rendering|Material|SetTextureParameterValue _array_element "RT" (Variables|Default|GetRenderTargetRuntime))))

(event EventOnPaint
  (params (UV :type Vector%202D%20Structure))
  (CallFunction|DrawtoRenderTarget "0, 0, 0" (Variables|Default|GetStrength) (Variables|Default|GetSize) UV))

(event EventBeginPlay
  (bind _staticmesh (Variables|Default|GetStaticMesh))
  ;[1 1 1] you need every player search in multiplay
  (Variables|Default|SetPlayerRef (Game|GetPlayerCharacter 0))
  (for (_array_element _array_index) (Rendering|Material|GetMaterials _staticmesh)
    (bind _returnvalue (Rendering|Material|CreateDynamicMaterialInstance _staticmesh _array_index _array_element "None" :!class /Script/Engine.PrimitiveComponent))
    (Utilities|Array|SetArrayElem (Variables|Default|GetDynamicMaterials) 0 _returnvalue true)
    (Rendering|ClearRenderTarget2D (Variables|Default|GetRenderTargetRuntime)))
  (CallFunction|SetValues))

(fn ConstructionScript
  (bind _returnvalue (Rendering|Material|CreateDynamicMaterialInstance "/Game/EatUpAll/PaintTest/M_HeatSplat.M_HeatSplat" "None" "None" :!class /Script/Engine.KismetMaterialLibrary))
  (Variables|Default|SetMID_Heatsplat _returnvalue))