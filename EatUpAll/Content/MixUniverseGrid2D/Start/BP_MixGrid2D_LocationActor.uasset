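; BP_MixGrid2D_LocationActor is a sphere actor that supplies a position and radius for the MixUniverse Grid2D sample.
; On BeginPlay it caches its root world location and derives Radius from the sphere's X world scale, intended for sending to Grid2D.
; Timeline-driven movement from the cached location and random sphere scaling are present but disconnected, so neither runs.
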(event EventBeginPlay
  (Utilities|FlowControl|Sequence
    (:then_0
      ;[0.04719 0.04189 0.1458] Cache location for timeline to start from
      (Variables|Default|SetCachedLocation (Transformation|GetWorldLocation (Variables|Default|GetDefaultSceneRoot)))
      ;[0.0625 0.09326 0.125] Set Radius Value Used for Sending to Grid2D
      (Variables|Default|SetRadius (* (.X (Math|Vector|BreakVector (Transformation|GetWorldScale (Variables|Default|GetSphere)))) 1e+02)))))

(fn ConstructionScript)