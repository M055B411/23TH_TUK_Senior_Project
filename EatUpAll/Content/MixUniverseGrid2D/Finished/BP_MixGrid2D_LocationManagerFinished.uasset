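; Manager Blueprint that feeds the positions and radii of all BP_MixGrid2D_LocationActor instances to the NSMixGrid2DLocations Niagara system.
; BeginPlay gathers those actors once and sizes a Vector4 array to match.
; Every Tick packs each valid actor's location into XYZ and Radius into W, then pushes the array to User.LocationsAndSizes.
; This per-frame Blueprint loop is simple but slower than a C++ equivalent.
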(event EventBeginPlay
  ;[0.05664 0.08298 0.09375] Quick Way to get all location actors to loop through.
  (bind _outactors (Actor|GetAllActorsOfClass "/Game/MixUniverseGrid2D/Start/BP_MixGrid2D_LocationActor.BP_MixGrid2D_LocationActor_C"))
  (bind _output_get (Variables|Default|SetAllLocationActors _outactors))
  (Utilities|Array|Resize (Variables|Default|GetLocationsAndSizes) (Utilities|Array|Length _output_get)))

(event EventTick
  (params (DeltaSeconds :type Float%20%28single-precision%29))
  ;[0.04291 0.05861 0.07292] Send location data to niagara. (BP will always be slower than C++ with this method)
  (for (_array_element _array_index) (Variables|Default|GetAllLocationActors)
    (Utilities|IsValid _array_element
      (:Is%20Valid
        (Utilities|Array|SetArrayElem (Variables|Default|GetLocationsAndSizes) _array_index (Math|Vector4|MakeVector4 (.X (Math|Vector|BreakVector (Transformation|GetActorLocation _array_element))) (.Y (Math|Vector|BreakVector (Transformation|GetActorLocation _array_element))) (.Z (Math|Vector|BreakVector (Transformation|GetActorLocation _array_element))) (Variables|/Game/MixUniverseGrid2D/Start/BP_MixGrid2D_LocationActor.BP_MixGrid2D_LocationActor_C|GetRadius _array_element))))))
  (Class|NiagaraDataInterfaceArrayFunctionLibrary|SetNiagaraArrayVector4 (Variables|Default|GetNS_MixGrid2D_Locations) "User.LocationsAndSizes" (Variables|Default|GetLocationsAndSizes)))

(fn ConstructionScript)