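; Whiteboard Blueprint that lets callers paint onto the CRT_PaintBoard render target at runtime.
; On BeginPlay it creates a dynamic instance of M_PaintboardMaker as the marker and clears the target to black.
; DrawOnWhiteboard passes a 2D location to the marker's DrawLocation parameter, draws the material into the target and prints a debug message.
; DrawSize sets the marker's Size parameter for subsequent strokes.
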(event Custom|DrawOnWhiteboard
  (params (LocationToDraw :type Vector%202D%20Structure))
  (bind _whiteboardmarker (Variables|Default|GetWhiteboardMarker))
  (Rendering|Material|SetVectorParameterValue _whiteboardmarker "DrawLocation" (Math|Conversions|ToLinearColor(Vector) (Math|Conversions|ToVector(Vector2D) LocationToDraw 0.1)) :!class /Script/Engine.MaterialInstanceDynamic)
  (Rendering|DrawMaterialtoRenderTarget "/Game/RenderTarget/CRT_PaintBoard.CRT_PaintBoard" _whiteboardmarker)
  (Development|PrintString "painting"))

(event Custom|DrawSize
  (params (Draw%20size :type Float%20%28double-precision%29))
  (Rendering|Material|SetScalarParameterValue (Variables|Default|GetWhiteboardMarker) "Size" Draw%20size :!class /Script/Engine.MaterialInstanceDynamic))

(event EventBeginPlay
  (bind _returnvalue (Rendering|Material|CreateDynamicMaterialInstance "/Game/RenderTarget/M_PaintboardMaker.M_PaintboardMaker" "None" "None" :!class /Script/Engine.KismetMaterialLibrary))
  (Variables|Default|SetWhiteboardMarker _returnvalue)
  (Rendering|ClearRenderTarget2D "/Game/RenderTarget/CRT_PaintBoard.CRT_PaintBoard"))

(fn ConstructionScript)